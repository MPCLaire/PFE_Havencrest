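; Sky actor that provides day and night backdrops and periodically spawns clouds.
; A looping timer started on BeginPlay spawns a random class from CloudsList at the transform of a randomly picked spawn point component.
; SetCielJour and SetCielNuit swap the sky by toggling visibility on the CielJour and CielNuit components and all their children.
; Day is applied at start; nothing in this Blueprint calls the night switch.
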(event `self.ReceiveBeginPlay`
  (set `self.SpawnPoints_List` (`|MakeArray` (`self.SpawnPoint2`) (`self.SpawnPoint3`) (`self.SpawnPoint4`)))
  (`KismetSystemLibrary.K2_SetTimerDelegate` (delegate `SpawnClouds`) 10.0 true)
  (`self.SetCielJour`))

(event `SpawnClouds`
  (bind _outitem (`KismetArrayLibrary.Array_Random` (`self.SpawnPoints_List`)))
  (`|SpawnActorFromClass` (`KismetArrayLibrary.Array_Random` (`self.Clouds_List`)) (`KismetMathLibrary.MakeTransform` (`SceneComponent.GetSocketLocation` _outitem "None") (`SceneComponent.GetSocketRotation` _outitem "None")) "Undefined" "MultiplyWithRoot" null null))

(fn `SetCielJour`
  (bind _cielnuit (`self.CielNuit`))
  (bind _cieljour (`self.CielJour`))
  (`SceneComponent.SetVisibility` _cielnuit false false)
  (for _array_element (`SceneComponent.GetChildrenComponents` _cielnuit true)
    (`SceneComponent.SetVisibility` _array_element false false))
  (`SceneComponent.SetVisibility` _cieljour true false)
  (for _array_element_2 (`SceneComponent.GetChildrenComponents` _cieljour true)
    (`SceneComponent.SetVisibility` _array_element_2 true false)))

(fn `SetCielNuit`
  (bind _cielnuit (`self.CielNuit`))
  (bind _cieljour (`self.CielJour`))
  (`SceneComponent.SetVisibility` _cielnuit true false)
  (for _array_element (`SceneComponent.GetChildrenComponents` _cielnuit true)
    (`SceneComponent.SetVisibility` _array_element true false))
  (`SceneComponent.SetVisibility` _cieljour false false)
  (for _array_element_2 (`SceneComponent.GetChildrenComponents` _cieljour true)
    (`SceneComponent.SetVisibility` _array_element_2 false false)))

(fn `UserConstructionScript`)