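; BP_Ciel_Nuit is a night sky decor Blueprint that periodically spawns clouds.
; On BeginPlay it gathers three spawn point components into a list and starts a looping ten-second timer.
; Each tick of the timer spawns a random class from the cloud list, taking location and rotation from random picks in the spawn point list.
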(event `self.ReceiveBeginPlay`
  (set `self.SpawnPoints_List` (`|MakeArray` (`self.SpawnPoint2`) (`self.SpawnPoint3`) (`self.SpawnPoint4`)))
  (`KismetSystemLibrary.K2_SetTimerDelegate` (delegate `SpawnClouds`) 10.0 true))

(event `SpawnClouds`
  (bind _outitem (`KismetArrayLibrary.Array_Random` (`self.SpawnPoints_List`)))
  (`|SpawnActorFromClass` (`KismetArrayLibrary.Array_Random` (`self.Clouds_List`)) (`KismetMathLibrary.MakeTransform` (`SceneComponent.GetSocketLocation` _outitem "None") (`SceneComponent.GetSocketRotation` _outitem "None")) "Undefined" "MultiplyWithRoot" null null))

(fn `UserConstructionScript`)