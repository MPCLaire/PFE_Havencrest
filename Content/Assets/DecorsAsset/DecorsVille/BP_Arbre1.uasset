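; BP_Arbre1 is a town decor tree Blueprint that animates its front and back foliage layers.
; On BeginPlay it caches the initial relative locations of FeuillesDevant and FeuillesFond, then starts a timeline.
; The timeline offsets both layers along X by a small interpolated amount from those origins and restarts itself through a zero Delay when finished, producing a continuous loop.
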(event `MoveFirstLayer`
  (bind (_devantinitloc_x _devantinitloc_y _devantinitloc_z) (`KismetMathLibrary.BreakVector` (`self.DevantInitLoc`)))
  (bind (_fondinitloc_x _fondinitloc_y _fondinitloc_z) (`KismetMathLibrary.BreakVector` (`self.FondInitLoc`)))
  (bind (_direction _newtrack_0) (`Timeline|MoveTL` :!via `PlayFromStart` :!label _label)
    (:`Update`
      (bind _returnvalue (`KismetMathLibrary.Lerp` 0.0 10.0 _newtrack_0))
      (`SceneComponent.K2_SetRelativeLocation` (`self.FeuillesDevant`) (`KismetMathLibrary.MakeVector` (+ _returnvalue _devantinitloc_x) _devantinitloc_y _devantinitloc_z) false false)
      (`SceneComponent.K2_SetRelativeLocation` (`self.FeuillesFond`) (`KismetMathLibrary.MakeVector` (+ _returnvalue _fondinitloc_x) _fondinitloc_y _fondinitloc_z) false false))
    (:`Finished`
      (`KismetSystemLibrary.Delay` 0.0)
      (goto _label :!via `PlayFromStart`))))

(event `self.ReceiveBeginPlay`
  (set `self.DevantInitLoc` (`SceneComponent.RelativeLocation` (`self.FeuillesDevant`)))
  (set `self.FondInitLoc` (`SceneComponent.RelativeLocation` (`self.FeuillesFond`)))
  (`self.MoveFirstLayer`))

(fn `UserConstructionScript`)