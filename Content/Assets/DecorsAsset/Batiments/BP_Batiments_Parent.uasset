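; Parent Blueprint for buildings Ethan can enter, with optional stairs and ventilation passages.
; Overlap boxes start looping timers that poll the E key, with DoOnce gates around transitions.
; Entering or exiting spawns a fade plane, moves Ethan, and toggles facade, smoke, spotlights and walk speed.
; Occupied houses register with the game instance; ChangeDayTime swaps their main character's child actor class.
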(event `Fade`
  (params (Plane :type "StaticMeshComponent Object Reference") (`BeInvisible?` :type Boolean))
  (bind _plane (`/Game/Blueprint/BP_FadePlane.Plane` (`self.FadeRef`)))
  (bind _plane_2 (`/Game/Blueprint/BP_FadePlane.Plane` (`self.FadeRef`)))
  ;[1 1 1] fait spawn le fade plane pour transition smooth
  (bind _returnvalue (`|SpawnActorFromClass` "/Game/Blueprint/BP_FadePlane.BP_FadePlane_C" (`SceneComponent.K2_GetComponentToWorld` Plane) "Undefined" "MultiplyWithRoot" null null))
  (set `self.FadeRef` _returnvalue)
  (if `BeInvisible?`
    ;[1 1 1] Set la visibilité du plane en fonction de si on est dedans ou dehors pour pas qu'on le voit au milieu de la route
    (if (`self.IsInside`)
      (`SceneComponent.SetVisibility` _plane true false)
      (`KismetSystemLibrary.Delay` 1.0)
      (`SceneComponent.SetVisibility` _plane false false)
      (else
        (`SceneComponent.SetVisibility` _plane_2 false false)
        (`KismetSystemLibrary.Delay` 0.7)
        (`SceneComponent.SetVisibility` _plane_2 true false)))))

(event `self.ReceiveBeginPlay`
  (bind _returnvalue (`GameplayStatics.GetActorOfClass` "/Game/Blueprint/MainCharacter/Blueprints/BP_Ethan.BP_Ethan_C"))
  (set `self.EthanRef` _returnvalue)
  (set `/Game/Blueprint/MainCharacter/Blueprints/BP_Ethan.BatimentParentRef` self (`self.EthanRef`))
  (bind _asgm_ethan (cast `/Game/Blueprint/GameSystem/GM_Ethan` (`GameplayStatics.GetGameMode`)))
  ;[1 1 1] enlève les box inutiles dans les différents BP
  (set `/Game/Blueprint/GameSystem/GM_Ethan.DirectLightRef` (`self.DirectLightRef`) _asgm_ethan)
  (`|ExecutionSequence`
    (:`then_0`
      (if (not (`self.HasStairs`))
        (`ActorComponent.K2_DestroyComponent` (`self.Box_RDC`))
        (`ActorComponent.K2_DestroyComponent` (`self.Box_etage`))))
    (:`then_1`
      (if (not (`self.HasVentilation`))
        (`ActorComponent.K2_DestroyComponent` (`self.Box_Ventilation1`))
        (`ActorComponent.K2_DestroyComponent` (`self.Box_Ventilation2`))
        (`ActorComponent.K2_DestroyComponent` (`self.PointVentil1`))
        (`ActorComponent.K2_DestroyComponent` (`self.PointVentil2`))))
    (:`then_2`
      (bind _asgi_havencrest (cast `/Game/Blueprint/GameSystem/GI_Havencrest` (`GameplayStatics.GetGameInstance`)))
      (set `self.GameInstanceRef` _asgi_havencrest)
      (if (`self.thisHouseHasPeopleInIt`)
        (`KismetArrayLibrary.Array_Add` (`/Game/Blueprint/GameSystem/GI_Havencrest.BatimentsRef` _asgi_havencrest) self)))))

(event `SchoolWillDestroy`
  (if (`self.HasVentilation`)
    (`/Engine/EditorBlueprintResources/StandardMacros.DoOnce` false
      (:`Completed`
        (`KismetSystemLibrary.Delay` 3.0)
        (set `self.willDestroy?` true)
        (`KismetSystemLibrary.PrintString` "Détruit")))))

(event `CheckEnter`
  ;[1 1 1] Vérifie que le joueur clique sur E puis rend invisible la façade et envoie la ref de la caméra à BP_Ethan
  (if (and (`/Game/Blueprint/MainCharacter/Blueprints/BP_Ethan.EPressed` (`self.EthanRef`)) (`self.GameCondition`))
    (set `/Game/Blueprint/MainCharacter/Blueprints/BP_Ethan.CantMove?` true (`self.EthanRef`))
    (if (`self.IsInside`)
      ;[1 1 1] Sortir du bâtiment
      (`/Engine/EditorBlueprintResources/StandardMacros.DoOnce` false :!label _label
        (:`Completed`
          (`self.Fade` (`self.FadePlane`) true)
          (`/Game/Blueprint/MainCharacter/Blueprints/BP_Ethan.FadeEthan` (`self.EthanRef`))
          (`KismetSystemLibrary.Delay` 0.7)
          (`/Game/Blueprint/Interfaces/BPI_Batiments.SetLocationBack` (`self.EthanRef`))
          (`LightComponent.SetIntensity` (`self.SpotLight`) 0.0)
          (`LightComponent.SetIntensity` (`self.SpotLight1`) 0.0)
          (`LightComponent.SetIntensity` (`self.SpotLight2`) 0.0)
          (`SceneComponent.SetVisibility` (`self.Fond`) true true)
          (`SceneComponent.SetVisibility` (`NiagaraActor.NiagaraComponent` (`self.FumeeRef`)) true true)
          (`SceneComponent.SetVisibility` (`self.Black_Floor`) false false)
          (set `CharacterMovementComponent.MaxWalkSpeed` 600.0 (`Character.CharacterMovement` (`self.EthanRef`)))
          (`KismetSystemLibrary.Delay` 1.0)
          (set `self.IsInside` false)
          (set `/Game/Blueprint/MainCharacter/Blueprints/BP_Ethan.CantMove?` false (`self.EthanRef`))
          (goto _label_2 :!via `Reset`)))
      (else
        ;[1 1 1] Entrer dans un bâtiment
        (`/Engine/EditorBlueprintResources/StandardMacros.DoOnce` false :!label _label_2
          (:`Completed`
            (`/Game/Blueprint/MainCharacter/Blueprints/BP_Ethan.FadeEthan` (`self.EthanRef`))
            (`self.Fade` (`self.FadePlane`) true)
            (set `self.InitialIntensity` (`LightComponentBase.Intensity` (`Light.LightComponent` (`self.DirectLightRef`))))
            (`KismetSystemLibrary.Delay` 0.7)
            (set `self.IsInside` true)
            (`/Game/Blueprint/MainCharacter/Blueprints/BP_Ethan.SetNewCameraInBuilding` (`self.EthanRef`) self)
            (`/Game/Blueprint/Interfaces/BPI_Batiments.SetInsideLocation` (`self.EthanRef`) (`SceneComponent.K2_GetComponentLocation` (`self.InsidePoint`)))
            (`SceneComponent.SetVisibility` (`self.Fond`) false true)
            (`SceneComponent.SetVisibility` (`NiagaraActor.NiagaraComponent` (`self.FumeeRef`)) false true)
            (`SceneComponent.SetVisibility` (`self.Black_Floor`) true false)
            (set `CharacterMovementComponent.MaxWalkSpeed` 300.0 (`Character.CharacterMovement` (`self.EthanRef`)))
            (`LightComponent.SetIntensity` (`self.SpotLight`) 50.0)
            (`LightComponent.SetIntensity` (`self.SpotLight1`) 50.0)
            (`LightComponent.SetIntensity` (`self.SpotLight2`) 50.0)
            (`KismetSystemLibrary.Delay` 2.0)
            (set `/Game/Blueprint/MainCharacter/Blueprints/BP_Ethan.CantMove?` false (`self.EthanRef`))
            (goto _label :!via `Reset`)))))))

(event `self.Box_Entree.OnComponentBeginOverlap`
  (params (OverlappedComponent :type "PrimitiveComponent Object Reference") (OtherActor :type "Actor Object Reference") (OtherComp :type "PrimitiveComponent Object Reference") (OtherBodyIndex :type Integer) (bFromSweep :type Boolean) (SweepResult :type "HitResult Structure (by ref)"))
  ;[1 1 1] Vérifie que le joueur clique sur E puis rend invisible la façade et envoie la ref de la caméra à BP_Ethan
  (if (== OtherActor (`GameplayStatics.GetPlayerPawn` 0))
    (`SceneComponent.SetVisibility` (`self.E`) true false)
    (bind _returnvalue (`KismetSystemLibrary.K2_SetTimerDelegate` (delegate `CheckEnter`) 0.2 true))))

(event `self.Box_Entree.OnComponentEndOverlap`
  (params (OverlappedComponent :type "PrimitiveComponent Object Reference") (OtherActor :type "Actor Object Reference") (OtherComp :type "PrimitiveComponent Object Reference") (OtherBodyIndex :type Integer))
  ;[1 1 1] Vérifie que le joueur clique sur E puis rend invisible la façade et envoie la ref de la caméra à BP_Ethan
  (if (== OtherActor (`self.EthanRef`))
    (`KismetSystemLibrary.K2_ClearAndInvalidateTimerHandle` (stale `self.Box_Entree.OnComponentBeginOverlap` _returnvalue))
    (`SceneComponent.SetVisibility` (`self.E`) false false)))

(event `self.Box_RDC.OnComponentEndOverlap`
  (params (OverlappedComponent :type "PrimitiveComponent Object Reference") (OtherActor :type "Actor Object Reference") (OtherComp :type "PrimitiveComponent Object Reference") (OtherBodyIndex :type Integer))
  ;[1 1 1] Fais aller à l'étage
  (`KismetSystemLibrary.K2_ClearAndInvalidateTimerHandle` (stale `self.Box_RDC.OnComponentBeginOverlap` _returnvalue))
  (`KismetSystemLibrary.Delay` 1.0)
  (goto _label_3 :!via `Reset`))

(event `self.Box_RDC.OnComponentBeginOverlap`
  (params (OverlappedComponent :type "PrimitiveComponent Object Reference") (OtherActor :type "Actor Object Reference") (OtherComp :type "PrimitiveComponent Object Reference") (OtherBodyIndex :type Integer) (bFromSweep :type Boolean) (SweepResult :type "HitResult Structure (by ref)"))
  ;[1 1 1] Fais aller à l'étage
  (if (== OtherActor (`self.EthanRef`))
    (`/Engine/EditorBlueprintResources/StandardMacros.DoOnce` false :!label _label_3
      (:`Completed`
        (bind _returnvalue (`KismetSystemLibrary.K2_SetTimerDelegate` (delegate `GoUpstairs`) 0.2 true))))))

(event `GoUpstairs`
  (bind _ethanref (`self.EthanRef`))
  ;[1 1 1] Fais aller à l'étage
  (if (and (`self.CanChangeFloor`) (`/Game/Blueprint/MainCharacter/Blueprints/BP_Ethan.EPressed` _ethanref))
    (set `self.CanChangeFloor` false)
    (`/Game/Blueprint/Interfaces/BPI_Batiments.SwitchFloor` _ethanref (`SceneComponent.K2_GetComponentLocation` (`self.Box_etage`)))
    (`KismetSystemLibrary.Delay` 1.0)
    (set `self.CanChangeFloor` true)
    (goto _label_4 :!via `Reset`)))

(event `self.Box_etage.OnComponentEndOverlap`
  (params (OverlappedComponent :type "PrimitiveComponent Object Reference") (OtherActor :type "Actor Object Reference") (OtherComp :type "PrimitiveComponent Object Reference") (OtherBodyIndex :type Integer))
  ;[1 1 1] Fais descendre
  (`KismetSystemLibrary.K2_ClearAndInvalidateTimerHandle` (stale `self.Box_etage.OnComponentBeginOverlap` _returnvalue))
  (`KismetSystemLibrary.Delay` 1.0)
  (goto _label_4 :!via `Reset`))

(event `self.Box_etage.OnComponentBeginOverlap`
  (params (OverlappedComponent :type "PrimitiveComponent Object Reference") (OtherActor :type "Actor Object Reference") (OtherComp :type "PrimitiveComponent Object Reference") (OtherBodyIndex :type Integer) (bFromSweep :type Boolean) (SweepResult :type "HitResult Structure (by ref)"))
  ;[1 1 1] Fais descendre
  (if (== OtherActor (`self.EthanRef`))
    (`/Engine/EditorBlueprintResources/StandardMacros.DoOnce` true :!label _label_4
      (:`Completed`
        (bind _returnvalue (`KismetSystemLibrary.K2_SetTimerDelegate` (delegate `DoDownstairs`) 0.2 true))))))

(event `DoDownstairs`
  (bind _ethanref (`self.EthanRef`))
  ;[1 1 1] Fais descendre
  (if (and (`self.CanChangeFloor`) (`/Game/Blueprint/MainCharacter/Blueprints/BP_Ethan.EPressed` _ethanref))
    (set `self.CanChangeFloor` false)
    (`/Game/Blueprint/Interfaces/BPI_Batiments.SwitchFloor` _ethanref (`SceneComponent.K2_GetComponentLocation` (`self.Box_RDC`)))
    (`KismetSystemLibrary.Delay` 1.0)
    (set `self.CanChangeFloor` true)
    (goto _label_3 :!via `Reset`)))

(event `self.Box_Ventilation1.OnComponentEndOverlap`
  (params (OverlappedComponent :type "PrimitiveComponent Object Reference") (OtherActor :type "Actor Object Reference") (OtherComp :type "PrimitiveComponent Object Reference") (OtherBodyIndex :type Integer))
  ;[1 1 1] Passer d'un côté à l'autre de la ventilation
  (`KismetSystemLibrary.K2_ClearAndInvalidateTimerHandle` (stale `self.Box_Ventilation1.OnComponentBeginOverlap` _returnvalue))
  (`KismetSystemLibrary.Delay` 1.0)
  (goto _label_5 :!via `Reset`))

(event `self.Box_Ventilation1.OnComponentBeginOverlap`
  (params (OverlappedComponent :type "PrimitiveComponent Object Reference") (OtherActor :type "Actor Object Reference") (OtherComp :type "PrimitiveComponent Object Reference") (OtherBodyIndex :type Integer) (bFromSweep :type Boolean) (SweepResult :type "HitResult Structure (by ref)"))
  ;[1 1 1] Passer d'un côté à l'autre de la ventilation
  (if (== OtherActor (`self.EthanRef`))
    (`/Engine/EditorBlueprintResources/StandardMacros.DoOnce` false :!label _label_5
      (:`Completed`
        (bind _returnvalue (`KismetSystemLibrary.K2_SetTimerDelegate` (delegate `GoToOtherSide`) 0.2 true))))))

(event `GoToOtherSide`
  (bind _ethanref (`self.EthanRef`))
  ;[1 1 1] Passer d'un côté à l'autre de la ventilation
  (if (and (`self.CanChangeFloor`) (`/Game/Blueprint/MainCharacter/Blueprints/BP_Ethan.EPressed` _ethanref) (`self.willDestroy?`))
    (set `self.CanChangeFloor` false)
    (if (`self.IsInVentilation`)
      (`/Game/Blueprint/Interfaces/BPI_Batiments.SwitchFloor` _ethanref (`SceneComponent.K2_GetComponentLocation` (`self.PointVentil1_1`)))
      (set `self.IsInVentilation` false)
      (else
        (`/Game/Blueprint/Interfaces/BPI_Batiments.SwitchFloor` _ethanref (`SceneComponent.K2_GetComponentLocation` (`self.PointVentil1`)))
        (set `self.IsInVentilation` true)))
    (`KismetSystemLibrary.Delay` 1.0)
    (set `self.CanChangeFloor` true)
    (goto _label_6 :!via `Reset`)))

(event `self.Box_Ventilation2.OnComponentEndOverlap`
  (params (OverlappedComponent :type "PrimitiveComponent Object Reference") (OtherActor :type "Actor Object Reference") (OtherComp :type "PrimitiveComponent Object Reference") (OtherBodyIndex :type Integer))
  ;[1 1 1] Passer d'un côté à l'autre de la ventilation
  (`KismetSystemLibrary.K2_ClearAndInvalidateTimerHandle` (stale `self.Box_Ventilation2.OnComponentBeginOverlap` _returnvalue))
  (`KismetSystemLibrary.Delay` 1.0)
  (goto _label_6 :!via `Reset`))

(event `self.Box_Ventilation2.OnComponentBeginOverlap`
  (params (OverlappedComponent :type "PrimitiveComponent Object Reference") (OtherActor :type "Actor Object Reference") (OtherComp :type "PrimitiveComponent Object Reference") (OtherBodyIndex :type Integer) (bFromSweep :type Boolean) (SweepResult :type "HitResult Structure (by ref)"))
  ;[1 1 1] Passer d'un côté à l'autre de la ventilation
  (if (== OtherActor (`self.EthanRef`))
    (`/Engine/EditorBlueprintResources/StandardMacros.DoOnce` true :!label _label_6
      (:`Completed`
        (bind _returnvalue (`KismetSystemLibrary.K2_SetTimerDelegate` (delegate `GoBack`) 0.2 true))))))

(event `GoBack`
  ;[1 1 1] Passer d'un côté à l'autre de la ventilation
  (if (and (`self.CanChangeFloor`) (`/Game/Blueprint/MainCharacter/Blueprints/BP_Ethan.EPressed` (`self.EthanRef`)))
    (set `self.CanChangeFloor` false)
    (if (`self.IsInVentilation`)
      (`/Game/Blueprint/Interfaces/BPI_Batiments.SwitchFloor` (`self.EthanRef`) (`SceneComponent.K2_GetComponentLocation` (`self.PointVentil2_1`)))
      (set `self.IsInVentilation` false)
      (else
        (`/Game/Blueprint/Interfaces/BPI_Batiments.SwitchFloor` (`self.EthanRef`) (`SceneComponent.K2_GetComponentLocation` (`self.PointVentil2`)))
        (set `self.IsInVentilation` true)))
    (`KismetSystemLibrary.Delay` 1.0)
    (set `self.CanChangeFloor` true)
    (goto _label_5 :!via `Reset`)))

(event `/Game/Blueprint/Interfaces/BPI_DayTime.ChangeDayTime`
  (params (DayTime :type Integer))
  (bind _listcharabat (`self.ListCharaBat`))
  (bind _persoprincipal (`self.PersoPrincipal`))
  (`KismetSystemLibrary.PrintString` "Hellooooooo")
  (`KismetSystemLibrary.PrintString` (`KismetStringLibrary.Conv_IntToString` DayTime))
  (switch `int` DayTime
    (:`1`
      (`ChildActorComponent.SetChildActorClass` _persoprincipal (`|GetArrayItem` _listcharabat)))
    (:`2`
      (`ChildActorComponent.SetChildActorClass` _persoprincipal (`|GetArrayItem` _listcharabat 1)))
    (:`3`
      (`ChildActorComponent.SetChildActorClass` _persoprincipal (`|GetArrayItem` _listcharabat 2)))))

(fn `UserConstructionScript`)