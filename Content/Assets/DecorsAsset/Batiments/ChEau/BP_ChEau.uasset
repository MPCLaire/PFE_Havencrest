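; ChEau building Blueprint with a ladder, hosting a serpent character who leads into the Snake minigame level.
; Overlapping SnakeBox starts a looping timer polling Ethan's E press, which either advances the serpent's dialogue to its question or, once asked, saves state and opens the level.
; A quest box validates an objective message on the widget.
; Leaving the entrance box clears or restores the serpent's boing sound depending on IsInside.
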(event `self.ReceiveBeginPlay`
  (`parent.ReceiveBeginPlay`)
  (set `self.hasLadder` true)
  (set `self.isChEau` true)
  (bind _asbp_serpent_dialogue (cast `/Game/Blueprint/Characters/BP_SerpentDialogue` (`ActorComponent.GetOwner` (`Actor.RootComponent` (`|GetArrayItem` (`self.GetAllChildActors` (`self.SerpentChara`) true))))))
  (set `self.SerpentDialogueRef` _asbp_serpent_dialogue))

(event `self.ValidateQuestBox.OnComponentBeginOverlap`
  (params (OverlappedComponent :type "PrimitiveComponent Object Reference") (OtherActor :type "Actor Object Reference") (OtherComp :type "PrimitiveComponent Object Reference") (OtherBodyIndex :type Integer) (bFromSweep :type Boolean) (SweepResult :type "HitResult Structure (by ref)"))
  (if (== OtherActor (`self.EthanRef`))
    (bind _foundwidgets (`WidgetBlueprintLibrary.GetAllWidgetsOfClass` null))
    (message `/Game/Blueprint/Interfaces/BPI_Objectifs.ValidateObjectif` (`|GetArrayItem` _foundwidgets) (`self.QuestIndex`))))

(event `self.SnakeBox.OnComponentBeginOverlap`
  (params (OverlappedComponent :type "PrimitiveComponent Object Reference") (OtherActor :type "Actor Object Reference") (OtherComp :type "PrimitiveComponent Object Reference") (OtherBodyIndex :type Integer) (bFromSweep :type Boolean) (SweepResult :type "HitResult Structure (by ref)"))
  (if (and (== OtherActor (`self.EthanRef`)) (not (`self.SnakeIsStarted`)))
    (bind _returnvalue (`KismetSystemLibrary.K2_SetTimerDelegate` (delegate `CheckE`) 0.1 true))))

(event `CheckE`
  (bind _ethanref (`self.EthanRef`))
  (bind _serpentdialogueref (`self.SerpentDialogueRef`))
  (bind _as_gi_havencrest (`/Game/Blueprint/MainCharacter/Blueprints/BP_Ethan.As GI Havencrest` _ethanref))
  (if (`/Game/Blueprint/MainCharacter/Blueprints/BP_Ethan.EPressed` (`self.EthanRef`))
    (`KismetSystemLibrary.K2_ClearAndInvalidateTimerHandle` (stale `self.SnakeBox.OnComponentBeginOverlap` _returnvalue))
    (if (`/Game/Blueprint/Characters/BP_SerpentDialogue.HasAsked?` _serpentdialogueref)
      (set `/Game/Blueprint/GameSystem/GI_Havencrest.GameState` "NewEnumerator1" _as_gi_havencrest)
      (`/Game/Blueprint/GameSystem/GI_Havencrest.Set Save Before MG` _as_gi_havencrest "BP_ChEau_C" (`self.K2_GetActorLocation` _ethanref))
      (`GameplayStatics.OpenLevelBySoftObjectPtr` "/Game/Maps/Snake_Level.Snake_Level")
      (else
        (`/Engine/EditorBlueprintResources/StandardMacros.DoOnce` false
          (:`Completed`
            (`/Game/Blueprint/Characters/BP_SerpentDialogue.ChangeToNextDialogue` _serpentdialogueref)
            (set `/Game/Blueprint/Characters/BP_SerpentDialogue.CanShowQuestion` true _serpentdialogueref)
            (`KismetSystemLibrary.PrintString` "change")))))))

(event `self.Box_Entree.OnComponentEndOverlap`
  (params (OverlappedComponent :type "PrimitiveComponent Object Reference") (OtherActor :type "Actor Object Reference") (OtherComp :type "PrimitiveComponent Object Reference") (OtherBodyIndex :type Integer))
  (bind _boing (`/Game/Blueprint/Characters/BP_Serpent.Boing` (`self.SerpentChara`)))
  (if (== OtherActor (`self.EthanRef`))
    (if (`self.IsInside`)
      (`AudioComponent.SetSound` _boing null)
      (else
        (`AudioComponent.SetSound` _boing "/Game/Sounds/Serpent/SC_SnakeBoing.SC_SnakeBoing")))))

(fn `UserConstructionScript`)