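; Pierre's house building Blueprint, which validates a journal objective when Ethan enters it.
; Two seconds after BeginPlay, it prints each GameInstance building and appends three Pierre day/night references to ListCharaBat on every iteration.
; Entrance box overlaps toggle InsidePierre, and the first starts a looping timer.
; Once InsidePierre and IsInside are both true, the timer stops and WB_Journal validates the objective; the Objectif1 setter is unreachable.
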(event `self.ReceiveBeginPlay`
  (bind _listcharabat (`self.ListCharaBat`))
  (`parent.ReceiveBeginPlay`)
  (`KismetSystemLibrary.Delay` 2.0)
  (for _array_element (`/Game/Blueprint/GameSystem/GI_Havencrest.BatimentsRef` (`self.GameInstanceRef`))
    (`KismetSystemLibrary.PrintString` (`KismetSystemLibrary.GetObjectName` _array_element))
    (`KismetArrayLibrary.Array_Add` _listcharabat "/Game/Blueprint/Characters/BP_PierreNuit1.BP_PierreNuit1_C")
    (`KismetArrayLibrary.Array_Add` _listcharabat "/Game/Blueprint/Characters/BP_PierreJour2.BP_PierreJour2_C")
    (`KismetArrayLibrary.Array_Add` _listcharabat "/Game/Blueprint/Characters/PersosSecondaires/Bp_PierreNuit2.Bp_PierreNuit2_C")))

(event `self.Box_Entree.OnComponentBeginOverlap`
  (params (OverlappedComponent :type "PrimitiveComponent Object Reference") (OtherActor :type "Actor Object Reference") (OtherComp :type "PrimitiveComponent Object Reference") (OtherBodyIndex :type Integer) (bFromSweep :type Boolean) (SweepResult :type "HitResult Structure (by ref)"))
  (cast `/Game/Blueprint/MainCharacter/Blueprints/BP_Ethan` OtherActor)
  (set `self.InsidePierre` true)
  (`/Engine/EditorBlueprintResources/StandardMacros.DoOnce` false
    (:`Completed`
      (bind _returnvalue (`KismetSystemLibrary.K2_SetTimerDelegate` (delegate `CheckIfInside`) 0.2 true)))))

(event `self.Box_Entree.OnComponentEndOverlap`
  (params (OverlappedComponent :type "PrimitiveComponent Object Reference") (OtherActor :type "Actor Object Reference") (OtherComp :type "PrimitiveComponent Object Reference") (OtherBodyIndex :type Integer))
  (cast `/Game/Blueprint/MainCharacter/Blueprints/BP_Ethan` OtherActor)
  (set `self.InsidePierre` false))

(event `CheckIfInside`
  (if (and (`self.InsidePierre`) (`self.IsInside`))
    (`KismetSystemLibrary.K2_ClearAndInvalidateTimerHandle` (stale `self.Box_Entree.OnComponentBeginOverlap` _returnvalue))
    (bind _foundwidgets (`WidgetBlueprintLibrary.GetAllWidgetsOfClass` "/Game/Blueprint/Widget/WB_Journal.WB_Journal_C"))
    (message `/Game/Blueprint/Interfaces/BPI_Objectifs.ValidateObjectif` _foundwidgets (`self.Index`))))

(fn `UserConstructionScript`)