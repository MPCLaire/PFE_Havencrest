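; Garage building actor that hosts the day/night switch, the garage "MJ" sequence and a bowling-ball reaction.
; Player entry, while allowed, swaps day and night sky actors, clears clouds for night, shows the time widget and notifies buildings; leaving removes the widget and permission.
; A second box starts a looping timer that polls Ethan's E press to launch the MJ sequence.
; A bowling ball hitting that box breaks the shelf material and ends bowling.
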(event `self.ReceiveBeginPlay`
  (`parent.ReceiveBeginPlay`)
  (`/Game/Blueprint/MainCharacter/Blueprints/BP_Ethan.GetGarageRef` (`self.EthanRef`) (`self.FadePlane`) self)
  (bind _returnvalue (`GameplayStatics.GetActorOfClass` "/Game/Assets/DecorsAsset/Ciel/BP_Ciel.BP_Ciel_C"))
  (set `self.CielTransform` (`self.GetTransform` _returnvalue))
  (set `self.CielRef` _returnvalue))

(event `self.Box_Entree.OnComponentBeginOverlap`
  (params (OverlappedComponent :type "PrimitiveComponent Object Reference") (OtherActor :type "Actor Object Reference") (OtherComp :type "PrimitiveComponent Object Reference") (OtherBodyIndex :type Integer) (bFromSweep :type Boolean) (SweepResult :type "HitResult Structure (by ref)"))
  (if (== OtherActor (`GameplayStatics.GetPlayerCharacter` 0))
    (`/Engine/EditorBlueprintResources/StandardMacros.DoOnce` false :!label _label
      (:`Completed`
        (`KismetSystemLibrary.PrintString` "je renter")
        (`self.SetDayOrNight`)
        (`KismetSystemLibrary.Delay` 1.0)
        (goto _label :!via `Reset`)))))

(event `self.Box_Entree.OnComponentEndOverlap`
  (params (OverlappedComponent :type "PrimitiveComponent Object Reference") (OtherActor :type "Actor Object Reference") (OtherComp :type "PrimitiveComponent Object Reference") (OtherBodyIndex :type Integer))
  (bind _returnvalue (`GameplayStatics.GetPlayerController` 0))
  (bind _gameinstanceref (`self.GameInstanceRef`))
  (if (== OtherActor (`GameplayStatics.GetPlayerCharacter` 0))
    (if (`/Game/Blueprint/GameSystem/GI_Havencrest.canChangeDayTime` _gameinstanceref)
      (set `/Game/Blueprint/GameSystem/GI_Havencrest.canChangeDayTime` false _gameinstanceref)
      (`Widget.RemoveFromParent` (`self.TimeWidgetRef`))
      (set `PlayerController.bShowMouseCursor` false _returnvalue)
      (`WidgetBlueprintLibrary.SetInputMode_GameOnly` _returnvalue))))

(event `self.Box.OnComponentBeginOverlap`
  (params (OverlappedComponent :type "PrimitiveComponent Object Reference") (OtherActor :type "Actor Object Reference") (OtherComp :type "PrimitiveComponent Object Reference") (OtherBodyIndex :type Integer) (bFromSweep :type Boolean) (SweepResult :type "HitResult Structure (by ref)"))
  (if (== OtherActor (`self.EthanRef`))
    (`/Engine/EditorBlueprintResources/StandardMacros.DoOnce` false
      (:`Completed`
        (bind _returnvalue (`KismetSystemLibrary.K2_SetTimerDelegate` (delegate `CheckE`) 0.1 true))))
    (else
      (cast `/Game/Blueprint/Mini_Jeux/Bowling/BP_BowlingBall` OtherActor)
      (`GameplayStatics.PlaySound2D` "/Game/Sounds/BowlingSounds/CasierQuiCase2.CasierQuiCase2" 1.0 1.0 0.0 null null)
      (`PrimitiveComponent.SetMaterial` (`self.Etagere`) 0 "/Game/Assets/DecorsAsset/Batiments/Garage/M_Etagere_Cassee.M_Etagere_Cassee")
      (`/Game/Blueprint/MainCharacter/Blueprints/BP_Ethan.EndBowling` (`self.EthanRef`)))))

(event `CheckE`
  (if (`/Game/Blueprint/MainCharacter/Blueprints/BP_Ethan.EPressed` (`self.EthanRef`))
    (`KismetSystemLibrary.K2_ClearAndInvalidateTimerHandle` (stale `self.Box.OnComponentBeginOverlap` _returnvalue))
    (`/Game/Blueprint/MainCharacter/Blueprints/BP_Ethan.StartGarageMJ` (`self.EthanRef`) (`SceneComponent.K2_GetComponentLocation` (`self.MJLocation`)))))

(fn `SetDayOrNight`
  (bind _cieltransform (`self.CielTransform`))
  (if (`/Game/Blueprint/GameSystem/GI_Havencrest.canChangeDayTime` (`self.GameInstanceRef`))
    (if (`self.IsDay?`)
      (set `self.IsDay?` false)
      (`self.K2_DestroyActor` (`self.CielRef`))
      (bind _returnvalue (`|SpawnActorFromClass` "/Game/Assets/DecorsAsset/Ciel/BP_Ciel_Nuit.BP_Ciel_Nuit_C" _cieltransform "AlwaysSpawn" "MultiplyWithRoot" null null))
      (set `self.CielNuitRef` _returnvalue)
      (bind _outactors (`GameplayStatics.GetAllActorsOfClass` "/Game/Assets/DecorsAsset/Ciel/BP_Clouds_Parent.BP_Clouds_Parent_C"))
      (for _array_element _outactors
        (`self.K2_DestroyActor` _array_element))
      (else
        (set `self.IsDay?` true)
        (`self.K2_DestroyActor` (`self.CielNuitRef`))
        (bind _returnvalue_2 (`|SpawnActorFromClass` "/Game/Assets/DecorsAsset/Ciel/BP_Ciel.BP_Ciel_C" _cieltransform "AlwaysSpawn" "MultiplyWithRoot" null null))
        (set `self.CielRef` _returnvalue_2)))
    (bind _returnvalue_3 (`|CreateWidget` "/Game/Blueprint/Widget/WB_JourNuit.WB_JourNuit_C"))
    (bind _output_get (set `self.TimeWidgetRef` _returnvalue_3))
    (`UserWidget.AddToViewport` _output_get 0)
    (bind _result (`/Engine/EditorBlueprintResources/StandardMacros.IncrementInt` (`self.RealDayTime`))
      (:`  `
        (for _array_element_2 (`/Game/Blueprint/GameSystem/GI_Havencrest.BatimentsRef` (`self.GameInstanceRef`))
          (message `/Game/Blueprint/Interfaces/BPI_DayTime.ChangeDayTime` _array_element_2 _result))))))

(fn `UserConstructionScript`)