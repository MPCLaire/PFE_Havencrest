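; BP_Boulangerie is the bakery building Blueprint, a child that extends its parent's BeginPlay.
; After the parent call, it registers its two black planes in BlackPlanes and three entries, including BP_Chou, in ListCharaBat.
; It only fills these arrays; the file contains no logic that uses them, and its construction script is empty.
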(event `self.ReceiveBeginPlay`
  (bind _listcharabat (`self.ListCharaBat`))
  (`parent.ReceiveBeginPlay`)
  (`KismetArrayLibrary.Array_Add` (`self.BlackPlanes`) (`self.BlackPlane`))
  (`KismetArrayLibrary.Array_Add` (`self.BlackPlanes`) (`self.BlackPlane1`))
  (`KismetArrayLibrary.Array_Add` _listcharabat)
  (`KismetArrayLibrary.Array_Add` _listcharabat)
  (`KismetArrayLibrary.Array_Add` _listcharabat "/Game/Blueprint/Items/Collectable/BP_Chou.BP_Chou_C"))

(fn `UserConstructionScript`)