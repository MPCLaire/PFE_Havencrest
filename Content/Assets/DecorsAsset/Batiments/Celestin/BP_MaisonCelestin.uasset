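; Celestin's house Blueprint, a building with trigger boxes that react to Ethan and host the entry point to Celestin's minigame.
; One box re-enables Ethan's movement once, while the upstairs box saves Ethan's location, calls SetLocationBack and reveals the Fond component.
; The minigame box activates and deactivates the game on overlap begin and end.
; An unwired broken-floor sequence with cracking sound and camera switch never runs.
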(event `self.ReceiveBeginPlay`
  (`PrimitiveComponent.SetCastShadow` (`self.E`) false)
  (`parent.ReceiveBeginPlay`))

(event `self.Box_0.OnComponentBeginOverlap`
  (params (OverlappedComponent :type "PrimitiveComponent Object Reference") (OtherActor :type "Actor Object Reference") (OtherComp :type "PrimitiveComponent Object Reference") (OtherBodyIndex :type Integer) (bFromSweep :type Boolean) (SweepResult :type "HitResult Structure (by ref)"))
  (if (== OtherActor (`self.EthanRef`))
    (`/Engine/EditorBlueprintResources/StandardMacros.DoOnce` false
      (:`Completed`
        (set `/Game/Blueprint/MainCharacter/Blueprints/BP_Ethan.CantMove?` false (`self.EthanRef`))))))

(event `self.Box_etage.OnComponentBeginOverlap`
  (params (OverlappedComponent :type "PrimitiveComponent Object Reference") (OtherActor :type "Actor Object Reference") (OtherComp :type "PrimitiveComponent Object Reference") (OtherBodyIndex :type Integer) (bFromSweep :type Boolean) (SweepResult :type "HitResult Structure (by ref)"))
  (bind _ethanref (`self.EthanRef`))
  (if (== OtherActor _ethanref)
    (set `/Game/Blueprint/MainCharacter/Blueprints/BP_Ethan.InitialLocation` (`SceneComponent.K2_GetComponentLocation` (`Character.CapsuleComponent` _ethanref)) _ethanref)
    (`/Game/Blueprint/Interfaces/BPI_Batiments.SetLocationBack` _ethanref)
    (`SceneComponent.SetVisibility` (`self.Fond`) true true)))

(event `self.BoxMiniGame.OnComponentBeginOverlap`
  (params (OverlappedComponent :type "PrimitiveComponent Object Reference") (OtherActor :type "Actor Object Reference") (OtherComp :type "PrimitiveComponent Object Reference") (OtherBodyIndex :type Integer) (bFromSweep :type Boolean) (SweepResult :type "HitResult Structure (by ref)"))
  (bind _ethanref (`self.EthanRef`))
  (if (== OtherActor _ethanref)
    (`/Game/Blueprint/MainCharacter/Blueprints/BP_Ethan.ActivateGameCelestin` _ethanref)))

(event `self.BoxMiniGame.OnComponentEndOverlap`
  (params (OverlappedComponent :type "PrimitiveComponent Object Reference") (OtherActor :type "Actor Object Reference") (OtherComp :type "PrimitiveComponent Object Reference") (OtherBodyIndex :type Integer))
  (bind _ethanref (`self.EthanRef`))
  (if (== OtherActor _ethanref)
    (`/Game/Blueprint/MainCharacter/Blueprints/BP_Ethan.DeactivateGameCelestin` _ethanref)))

(fn `UserConstructionScript`
  (`parent.UserConstructionScript`))