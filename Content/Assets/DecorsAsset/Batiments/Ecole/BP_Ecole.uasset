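; School building actor, derived from a parent building Blueprint, that adapts the school to story progress and time of day.
; BeginPlay registers characters and black planes, then uses GameState to set the prop list or, in later states, destroy props, explosion and vent grille components.
; A non-zero day time, rechecked on ChangeDayTime, swaps classroom door components.
; Two ventilation overlap boxes show prompts to Ethan; the first also toggles his vent-destroy ability.
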(event `self.ReceiveBeginPlay`
  (bind _porteclasse4 (`self.PorteClasse4`))
  (bind _listcharabat (`self.ListCharaBat`))
  (bind _array (`|MakeArray` (`self.Chaise3`) (`self.Table1`) (`self.Chaise8`) (`self.Table3`) (`self.Chaise6`) (`self.Table8`)))
  (set `self.isSchool` true)
  (`parent.ReceiveBeginPlay`)
  (`KismetArrayLibrary.Array_Add` _listcharabat "/Game/Blueprint/Characters/BP_AlbertNuit1.BP_AlbertNuit1_C")
  (`KismetArrayLibrary.Array_Add` _listcharabat)
  (`KismetArrayLibrary.Array_Add` _listcharabat "/Game/Blueprint/Characters/PersosSecondaires/BP_AlbertNuit2.BP_AlbertNuit2_C")
  (set `self.EcoleRef` self)
  (`KismetArrayLibrary.Array_Add` (`self.BlackPlanes`) (`self.BlackPlane`))
  (`KismetArrayLibrary.Array_Add` (`self.BlackPlanes`) (`self.BlackPlane1`))
  (`KismetArrayLibrary.Array_Add` (`self.BlackPlanes`) (`self.BlackPlane3`))
  (`PrimitiveComponent.SetCastShadow` (`self.E_Etage`) false)
  (`PrimitiveComponent.SetCastShadow` (`self.E`) false)
  (`PrimitiveComponent.SetCastShadow` (`self.E_RDC`) false)
  (`|ExecutionSequence`
    (:`then_0`
      (switch `/Game/Blueprint/GameSystem/E_Instance` (`/Game/Blueprint/GameSystem/GI_Havencrest.GameState` (`self.GameInstanceRef`))
        (:`NewEnumerator0`
          (set `self.SchoolProps` _array :!label _label))
        (:`NewEnumerator1`
          (goto _label))
        (:`NewEnumerator3`
          (goto _label))
        (:`NewEnumerator4`
          (bind _output_get (set `self.SchoolProps` _array :!label _label_2))
          (for _array_element _output_get
            (`ActorComponent.K2_DestroyComponent` _array_element))
          (`ActorComponent.K2_DestroyComponent` (`self.Explosion`))
          (`ActorComponent.K2_DestroyComponent` (`self.Mw`))
          (`ActorComponent.K2_DestroyComponent` (`self.VentilGrille`))
          (set `self.willDestroy?` true))
        (:`NewEnumerator5`
          (goto _label_2))
        (:`NewEnumerator6`
          (goto _label_2))
        (:`NewEnumerator2`
          (goto _label_2))))
    (:`then_1`
      (if (> (`/Game/Blueprint/GameSystem/GI_Havencrest.InstanceDayTime` (`self.GameInstanceRef`)) 0) :!label _label_3
        (if (and (`KismetSystemLibrary.IsValid` _porteclasse4) (`KismetSystemLibrary.IsValid` (`self.PorteClasse5`)) (`KismetSystemLibrary.IsValid` (`self.PorteClasse6`)) (`KismetSystemLibrary.IsValid` (`self.PorteClasse7`)))
          (`ActorComponent.K2_DestroyComponent` _porteclasse4)
          (`ActorComponent.K2_DestroyComponent` (`self.PorteClasse5`))
          (`ActorComponent.K2_DestroyComponent` (`self.PorteClasse6`))
          (`ActorComponent.K2_DestroyComponent` (`self.PorteClasse7`))
          (`SceneComponent.SetVisibility` (`self.PorteClasse2`) true false)
          (`SceneComponent.SetVisibility` (`self.PorteClasse`) true false))))))

(event `self.Box_Ventilation1.OnComponentBeginOverlap`
  (params (OverlappedComponent :type "PrimitiveComponent Object Reference") (OtherActor :type "Actor Object Reference") (OtherComp :type "PrimitiveComponent Object Reference") (OtherBodyIndex :type Integer) (bFromSweep :type Boolean) (SweepResult :type "HitResult Structure (by ref)"))
  (bind _ethanref (`self.EthanRef`))
  (if (== OtherActor _ethanref)
    (`/Game/Blueprint/MainCharacter/Blueprints/BP_Ethan.uCanDestroyVent` _ethanref)
    (`SceneComponent.SetVisibility` (`self.EgrilleEnter`) true false)))

(event `self.Box_Ventilation1.OnComponentEndOverlap`
  (params (OverlappedComponent :type "PrimitiveComponent Object Reference") (OtherActor :type "Actor Object Reference") (OtherComp :type "PrimitiveComponent Object Reference") (OtherBodyIndex :type Integer))
  (bind _ethanref (`self.EthanRef`))
  (if (== OtherActor _ethanref)
    (`/Game/Blueprint/MainCharacter/Blueprints/BP_Ethan.uCantDetroyVent` _ethanref)
    (`SceneComponent.SetVisibility` (`self.EgrilleEnter`) false false)))

(event `/Game/Blueprint/Interfaces/BPI_DayTime.ChangeDayTime`
  (params (DayTime :type Integer))
  (`parent.ChangeDayTime` (`/Game/Blueprint/GameSystem/GI_Havencrest.InstanceDayTime` (`self.GameInstanceRef`)))
  (goto _label_3))

(event `self.Box_Ventilation2.OnComponentBeginOverlap`
  (params (OverlappedComponent :type "PrimitiveComponent Object Reference") (OtherActor :type "Actor Object Reference") (OtherComp :type "PrimitiveComponent Object Reference") (OtherBodyIndex :type Integer) (bFromSweep :type Boolean) (SweepResult :type "HitResult Structure (by ref)"))
  (if (== OtherActor (`self.EthanRef`))
    (`SceneComponent.SetVisibility` (`self.EsortieGrille`) true false)))

(event `self.Box_Ventilation2.OnComponentEndOverlap`
  (params (OverlappedComponent :type "PrimitiveComponent Object Reference") (OtherActor :type "Actor Object Reference") (OtherComp :type "PrimitiveComponent Object Reference") (OtherBodyIndex :type Integer))
  (if (== OtherActor (`self.EthanRef`))
    (`SceneComponent.SetVisibility` (`self.EsortieGrille`) false false)))

(fn `UserConstructionScript`)