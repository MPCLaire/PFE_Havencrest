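; BP_CabMed is a medical cabinet building Blueprint derived from a parent building class.
; On BeginPlay it fills its building character list with MarieNuit entries, starts locked and publishes itself as CabMedRef.
; On ChangeDayTime it calls the parent, then for day time 1 swaps the secondary character child actor to BP_LaetriciaAttente.
; Tick prints the unlock state as debug output.
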(event `self.ReceiveBeginPlay`
  (bind _listcharabat (`self.ListCharaBat`))
  (`parent.ReceiveBeginPlay`)
  (`KismetArrayLibrary.Array_Add` _listcharabat "/Game/Blueprint/Characters/BP_MarieNuit1.BP_MarieNuit1_C")
  (`KismetArrayLibrary.Array_Add` _listcharabat)
  (`KismetArrayLibrary.Array_Add` _listcharabat "/Game/Blueprint/Characters/PersosSecondaires/BP_MarieNuit2.BP_MarieNuit2_C")
  (set `self.isUnlocked` false)
  (set `self.CabMedRef` self))

(event `/Game/Blueprint/Interfaces/BPI_DayTime.ChangeDayTime`
  (params (DayTime :type Integer))
  (`parent.ChangeDayTime` DayTime)
  (if (== DayTime 1)
    (`ChildActorComponent.SetChildActorClass` (`self.PersoSecondaire`) "/Game/Blueprint/Characters/BP_LaetriciaAttente.BP_LaetriciaAttente_C")))

(event `self.ReceiveTick`
  (params (DeltaSeconds :type "Float (single-precision)"))
  (`KismetSystemLibrary.PrintString` (`KismetStringLibrary.Conv_BoolToString` (`self.isUnlocked`)) true true (struct :`R` 1.0 :`G` 0.859999 :`A` 1.0)))

(fn `UserConstructionScript`)