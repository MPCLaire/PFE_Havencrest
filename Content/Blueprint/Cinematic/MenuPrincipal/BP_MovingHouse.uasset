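; Main menu cinematic house actor built to pulse a rectangle mesh along its Y scale, currently inert because BeginPlay is empty.
; ScaleHouse loops a timeline after a random integer delay, lerping Y from InitialScale to three units above it.
; SetScaleFirst and SetScaleSecond are opposite-phase alternatives that recursively step Y up and down each second.
; The logic that caches InitialScale, starts ScaleHouse or picks a phase via MoveFirst is disconnected.
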(event `ScaleHouse`
  (bind (_initialscale_x _initialscale_y) (`KismetMathLibrary.BreakVector` (`self.InitialScale`)))
  (bind (_returnvalue_x _returnvalue_y _returnvalue_z) (`KismetMathLibrary.BreakVector` (`SceneComponent.K2_GetComponentScale` (`self.House_Rectangle`))))
  (`KismetSystemLibrary.RetriggerableDelay` (`KismetMathLibrary.Conv_IntToDouble` (`KismetMathLibrary.RandomIntegerInRange` 0 2)) :!label _label)
  (bind (_direction _newtrack_0) (`Timeline|SclaeTL` :!via `PlayFromStart`)
    (:`Update`
      (`SceneComponent.SetWorldScale3D` (`self.House_Rectangle`) (`KismetMathLibrary.MakeVector` _returnvalue_x (`KismetMathLibrary.Lerp` _initialscale_y (+ _initialscale_y 3.0) _newtrack_0) _returnvalue_z)))
    (:`Finished`
      (`KismetSystemLibrary.Delay` 0.0)
      (goto _label))))

(event `self.ReceiveBeginPlay`)

(event `SetScaleFirst`
  (bind _house_rectangle (`self.House_Rectangle`))
  (bind (_returnvalue_x _returnvalue_y _returnvalue_z) (`KismetMathLibrary.BreakVector` (`SceneComponent.K2_GetComponentScale` (`self.House_Rectangle`))))
  (bind (_returnvalue_x_2 _returnvalue_y_2 _returnvalue_z_2) (`KismetMathLibrary.BreakVector` (`SceneComponent.K2_GetComponentScale` (`self.House_Rectangle`))))
  (`KismetSystemLibrary.Delay` 1.0)
  (`SceneComponent.SetWorldScale3D` _house_rectangle (`KismetMathLibrary.MakeVector` _returnvalue_x (+ _returnvalue_y 3.0) _returnvalue_z))
  (`KismetSystemLibrary.Delay` 1.0)
  (`SceneComponent.SetWorldScale3D` _house_rectangle (`KismetMathLibrary.MakeVector` _returnvalue_x_2 (- _returnvalue_y_2 3.0) _returnvalue_z_2))
  (`self.SetScaleFirst`))

(event `SetScaleSecond`
  (bind _house_rectangle (`self.House_Rectangle`))
  (bind (_returnvalue_x _returnvalue_y _returnvalue_z) (`KismetMathLibrary.BreakVector` (`SceneComponent.K2_GetComponentScale` (`self.House_Rectangle`))))
  (bind (_returnvalue_x_2 _returnvalue_y_2 _returnvalue_z_2) (`KismetMathLibrary.BreakVector` (`SceneComponent.K2_GetComponentScale` (`self.House_Rectangle`))))
  (`KismetSystemLibrary.Delay` 1.0)
  (`SceneComponent.SetWorldScale3D` _house_rectangle (`KismetMathLibrary.MakeVector` _returnvalue_x (- _returnvalue_y 3.0) _returnvalue_z))
  (`KismetSystemLibrary.Delay` 1.0)
  (`SceneComponent.SetWorldScale3D` _house_rectangle (`KismetMathLibrary.MakeVector` _returnvalue_x_2 (+ _returnvalue_y_2 3.0) _returnvalue_z_2))
  (`self.SetScaleSecond`))

(fn `UserConstructionScript`)