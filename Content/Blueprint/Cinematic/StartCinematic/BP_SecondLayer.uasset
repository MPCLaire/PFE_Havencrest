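; BP_SecondLayer is an actor, filed under the start cinematic, that slides along the world Y axis.
; On BeginPlay it stores its root's world location and calls Move, which plays a Timeline from the start.
; Each Timeline update lerps a Y offset from zero toward negative Y and adds it to the stored location, keeping X and Z fixed.
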(event `Move`
  (bind (_initlocation_x _initlocation_y _initlocation_z) (`KismetMathLibrary.BreakVector` (`self.InitLocation`)))
  (bind (_direction _newtrack_0) (`Timeline|Timeline` :!via `PlayFromStart`)
    (:`Update`
      (`SceneComponent.K2_SetWorldLocation` (`self.DefaultSceneRoot`) (`KismetMathLibrary.MakeVector` _initlocation_x (+ (`KismetMathLibrary.Lerp` 0.0 -1600.0 _newtrack_0) _initlocation_y) _initlocation_z) false false))))

(event `self.ReceiveBeginPlay`
  (set `self.InitLocation` (`SceneComponent.K2_GetComponentLocation` (`self.DefaultSceneRoot`)))
  (`self.Move`))

(fn `UserConstructionScript`)