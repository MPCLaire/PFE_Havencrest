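; Player Blueprint for the game's endings, showing either the good (BonneFin) or bad (MauvaiseFin) ending as a paged widget.
; Two spawn events create the matching widget, add it to the viewport, hide the cursor and set Game and UI input.
; Q/Left and D/Right turn pages back and forward on the good-ending widget if valid, otherwise on the bad-ending one without a validity check.
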(event `self.ReceiveBeginPlay`)

(event `SpawnBonneFin`
  (bind _returnvalue (`GameplayStatics.GetPlayerController` 0))
  (bind _returnvalue_2 (`|CreateWidget` "/Game/Blueprint/Widget/WB_BonneFin.WB_BonneFin_C"))
  (bind _output_get (set `self.BonneFinRef` _returnvalue_2))
  (`UserWidget.AddToViewport` _output_get 0)
  (set `PlayerController.bShowMouseCursor` false _returnvalue)
  (`WidgetBlueprintLibrary.SetInputMode_GameAndUIEx` _returnvalue null))

(event `SpawnMauvaiseFin`
  (bind _returnvalue (`GameplayStatics.GetPlayerController` 0))
  (bind _returnvalue_2 (`|CreateWidget` "/Game/Blueprint/Widget/WB_MauvaiseFin2.WB_MauvaiseFin2_C"))
  (bind _output_get (set `self.MauvaiseFinRef` _returnvalue_2))
  (`UserWidget.AddToViewport` _output_get 0)
  (set `PlayerController.bShowMouseCursor` false _returnvalue)
  (`WidgetBlueprintLibrary.SetInputMode_GameAndUIEx` _returnvalue null))

(event `Key|Q`
  (params (Key :type "Key Structure"))
  (bind _bonnefinref (`self.BonneFinRef`))
  (:`Pressed`
    (if (`KismetSystemLibrary.IsValid` _bonnefinref) :!label _label
      (`/Game/Blueprint/Widget/WB_BonneFin.PageBack` _bonnefinref)
      (else
        (`/Game/Blueprint/Widget/WB_MauvaiseFin2.PageBack` (`self.MauvaiseFinRef`))))))

(event `Key|Left`
  (params (Key :type "Key Structure"))
  (:`Pressed`
    (goto _label)))

(event `Key|D`
  (params (Key :type "Key Structure"))
  (bind _bonnefinref (`self.BonneFinRef`))
  (:`Pressed`
    (if (`KismetSystemLibrary.IsValid` _bonnefinref) :!label _label_2
      (`/Game/Blueprint/Widget/WB_BonneFin.PageForward` _bonnefinref)
      (else
        (`/Game/Blueprint/Widget/WB_MauvaiseFin2.PageForward` (`self.MauvaiseFinRef`))))))

(event `Key|Right`
  (params (Key :type "Key Structure"))
  (:`Pressed`
    (goto _label_2)))

(fn `UserConstructionScript`)