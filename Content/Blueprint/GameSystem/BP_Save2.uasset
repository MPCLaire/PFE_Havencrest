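; BP_Save2 is a save game object that records a state for each saved actor.
; It keeps two parallel arrays, ActorSaved and States, matched by index.
; AddAnObject uses the linear search in CheckActorIsInArray to overwrite an existing actor's state, or appends a new pair.
; Every call then immediately writes the object itself to the fixed "Save1" slot.
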(fn `AddAnObject`
  (params (ActorSaved :type "Actor Object Reference") (State :type "EDataLayerState Enum" :default "Unloaded"))
  (bind _actorsaved (`self.ActorSaved`))
  (bind _states (`self.States`))
  (if (`KismetArrayLibrary.Array_IsEmpty` _actorsaved)
    (`KismetArrayLibrary.Array_Add` _actorsaved ActorSaved)
    (`KismetArrayLibrary.Array_Add` _states State)
    (else
      (bind (_isinarray _array_index) (`self.CheckActorIsInArray` ActorSaved))
      (if _isinarray
        (`KismetArrayLibrary.Array_Set` _states _array_index State)
        (else
          (`KismetArrayLibrary.Array_Add` _actorsaved ActorSaved)
          (`KismetArrayLibrary.Array_Add` _states State)))))
  (`GameplayStatics.SaveGameToSlot` self "Save1"))

(fn `CheckActorIsInArray`
  (params (Actor :type "Actor Object Reference"))
  (returns (IsInArray :type Boolean) (`Array Index` :type Integer))
  (for (_array_element _array_index) (`self.ActorSaved`)
    (if (== Actor _array_element)
      (return true _array_index))))