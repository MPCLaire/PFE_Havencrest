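; GM_Ethan, apparently the game mode, handles day and night lighting for the Havencrest level.
; On BeginPlay it caches the Havencrest game instance and, only in that level, the BP_Ethan actor and every BP_Lampadaire street lamp.
; Setnight and SetDay change directional light intensity and switch the lamps, though DirectLightRef is never assigned here.
; Save and SavePlayerLoc are empty, and the BP_Save slot logic is disconnected.
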(event `self.ReceiveBeginPlay`
  (bind _asgi_havencrest (cast `/Game/Blueprint/GameSystem/GI_Havencrest` (`GameplayStatics.GetGameInstance`)))
  (set `self.As GI Havencrest` _asgi_havencrest)
  (bind _returnvalue (`GameplayStatics.GetCurrentLevelName` true))
  (if (`KismetStringLibrary.EqualEqual_StrStr` _returnvalue "Havencrest")
    (bind _returnvalue_2 (`GameplayStatics.GetActorOfClass` "/Game/Blueprint/MainCharacter/Blueprints/BP_Ethan.BP_Ethan_C"))
    (set `self.EthanRef` _returnvalue_2)
    (bind _outactors (`GameplayStatics.GetAllActorsOfClass` "/Game/Assets/DecorsAsset/DecorsVille/BP_Lampadaire.BP_Lampadaire_C"))
    (for _array_element _outactors
      (`KismetArrayLibrary.Array_Add` (`self.LampadairesRef`) _array_element))))

(event `Save`)

(event `Set night`
  (`LightComponent.SetIntensity` (`Light.LightComponent` (`self.DirectLightRef`)) 1.0)
  (for _array_element (`self.LampadairesRef`)
    (`/Game/Assets/DecorsAsset/DecorsVille/BP_Lampadaire.TurnLightsOn` _array_element)))

(event `SetDay`
  (`LightComponent.SetIntensity` (`Light.LightComponent` (`self.DirectLightRef`)) 2.5)
  (for _array_element (`self.LampadairesRef`)
    (`/Game/Assets/DecorsAsset/DecorsVille/BP_Lampadaire.TurnLightsOff` _array_element)))

(event `self.ReceiveTick`
  (params (DeltaSeconds :type "Float (single-precision)")))

(fn `SavePlayerLoc`)

(fn `UserConstructionScript`)