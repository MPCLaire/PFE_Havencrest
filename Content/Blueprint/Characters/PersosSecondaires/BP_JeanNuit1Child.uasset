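; Child Blueprint for the secondary character Jean on night 1 ("Nuit1"), supplying this variant's dialogue and player choices.
; On BeginPlay it copies its own dialogue, choice and line variables into the inherited ones before calling the parent, which holds the base logic.
; Choices 1 and 3 extend the parent handlers to raise or lower the GameInstance's QuotientSocial score, with the penalty outweighing the gain.
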(event `self.ReceiveBeginPlay`
  (set `self.DialogueJeanNuit1` (`self.DialogueJeanNuit1Child`))
  (set `self.DialogueChoice1JeanNuit1` (`self.DialogueChoice1JeanNuit1Child`))
  (set `self.DialogueChoice2JeanNuit1` (`self.DialogueChoice2JeanNuit1Child`))
  (set `self.DialogueChoice3JeanNuit1` (`self.DialogueChoice3JeanNuit1Child`))
  (set `self.DialogueChoiceEndJeanNuit1` (`self.DialogueChoiceEndJeanNuit1Child`))
  (set `self.LineChoice1JeanNuit1` (`self.LineChoice1JeanNuit1Child`))
  (set `self.LineChoice2JeanNuit1` (`self.LineChoice2JeanNuit1Child`))
  (set `self.LineChoice3JeanNuit1` (`self.LineChoice3JeanNuit1Child`))
  (`parent.ReceiveBeginPlay`))

(event `/Game/Blueprint/Interfaces/BPI_DialogueChoice.Choice1`
  (`parent.Choice1`)
  (`/Engine/EditorBlueprintResources/StandardMacros.IncrementInt` (`/Game/Blueprint/GameSystem/GI_Havencrest.QuotientSocial` (`self.GameInstanceRef`))))

(event `/Game/Blueprint/Interfaces/BPI_DialogueChoice.Choice3`
  (bind _quotientsocial (`/Game/Blueprint/GameSystem/GI_Havencrest.QuotientSocial` (`self.GameInstanceRef`)))
  (`parent.Choice3`)
  (`/Engine/EditorBlueprintResources/StandardMacros.DecrementInt` _quotientsocial
    (:`  `
      (`/Engine/EditorBlueprintResources/StandardMacros.DecrementInt` _quotientsocial))))

(fn `UserConstructionScript`
  (`parent.UserConstructionScript`))