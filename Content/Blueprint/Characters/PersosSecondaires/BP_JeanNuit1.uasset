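; Dialogue NPC Blueprint for Jean, a secondary character, in his "Nuit1" (night 1) version.
; BeginPlay loads his dialogue, choice lines and name into inherited variables before running the parent logic.
; ShowChoices hides the end button and, when IsChoiceChara is false, alternates between two secondary dialogues via FlipFlop.
; Choice overrides lower or raise the GameInstance's QuotientSocial score, and ChoiceEnd clears IsChoiceChara.
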(event `self.ReceiveBeginPlay`
  (set `self.BaseDialogue` (`self.DialogueJeanNuit1`))
  (set `self.DialogueChoice1` (`self.DialogueChoice1JeanNuit1`))
  (set `self.DialogueChoice2` (`self.DialogueChoice2JeanNuit1`))
  (set `self.DialogueChoice3` (`self.DialogueChoice3JeanNuit1`))
  (set `self.DialogueChoiceEnd` (`self.DialogueChoiceEndJeanNuit1`))
  (set `self.LineChoice1` (`self.LineChoice1JeanNuit1`))
  (set `self.LineChoice2` (`self.LineChoice2JeanNuit1`))
  (set `self.LineChoice3` (`self.LineChoice3JeanNuit1`))
  (set `self.CharaName` "Jean")
  (set `self.NumberOfChoices` 1)
  (`parent.ReceiveBeginPlay`))

(event `self.ShowChoices`
  (`parent.ShowChoices`)
  (`Widget.SetVisibility` (`/Game/Blueprint/Widget/Dialogue/WB_Choice.BTN_ChoiceEnd` (`self.UIchoice`)) "Hidden")
  (if (not (`self.isChoiceChara`))
    (`/Engine/EditorBlueprintResources/StandardMacros.FlipFlop`
      (:`A`
        (set `self.BaseDialogue` (`self.DialogueSecondaryJeanNuit1`)))
      (:`B`
        (set `self.BaseDialogue` (`self.DialogueSecondary2JeanNuit1`))))))

(event `/Game/Blueprint/Interfaces/BPI_DialogueChoice.Choice1`
  (`parent.Choice1`)
  (`/Engine/EditorBlueprintResources/StandardMacros.DecrementInt` (`/Game/Blueprint/GameSystem/GI_Havencrest.QuotientSocial` (`self.GameInstanceRef`))))

(event `/Game/Blueprint/Interfaces/BPI_DialogueChoice.Choice2`
  (`parent.Choice2`)
  (`/Engine/EditorBlueprintResources/StandardMacros.IncrementInt` (`/Game/Blueprint/GameSystem/GI_Havencrest.QuotientSocial` (`self.GameInstanceRef`))))

(event `/Game/Blueprint/Interfaces/BPI_DialogueChoice.Choice3`
  (`parent.Choice3`)
  (`/Engine/EditorBlueprintResources/StandardMacros.IncrementInt` (`/Game/Blueprint/GameSystem/GI_Havencrest.QuotientSocial` (`self.GameInstanceRef`))))

(event `/Game/Blueprint/Interfaces/BPI_DialogueChoice.ChoiceEnd`
  (`parent.ChoiceEnd`)
  (set `self.isChoiceChara` false))

(fn `UserConstructionScript`
  (`parent.UserConstructionScript`))