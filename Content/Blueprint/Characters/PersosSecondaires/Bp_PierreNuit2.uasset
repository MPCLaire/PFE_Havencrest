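; Blueprint for the secondary character Pierre on night 2 (PierreNuit2), supplying his dialogue to a parent character class.
; BeginPlay sets the first dialogue as BaseDialogue and clears IsChoiceChara before running the parent logic.
; Each ShowChoices call runs the parent, then uses the WhatText counter to advance BaseDialogue through three dialogues, looping back to the first.
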(event `self.ReceiveBeginPlay`
  (set `self.BaseDialogue` (`self.Dialogue1PierreNuit2`))
  (set `self.isChoiceChara` false)
  (`parent.ReceiveBeginPlay`))

(event `self.ShowChoices`
  (bind _whattext (`self.WhatText`))
  (`parent.ShowChoices`)
  (switch `int` (`self.WhatText`)
    (:`0`
      (set `self.BaseDialogue` (`self.Dialogue2PierreNuit2`))
      (`/Engine/EditorBlueprintResources/StandardMacros.IncrementInt` _whattext))
    (:`1`
      (set `self.BaseDialogue` (`self.Dialogue3PierreNuit2`))
      (`/Engine/EditorBlueprintResources/StandardMacros.IncrementInt` _whattext))
    (:`2`
      (set `self.BaseDialogue` (`self.Dialogue1PierreNuit2`))
      (set `self.WhatText` 0))))

(fn `UserConstructionScript`
  (`parent.UserConstructionScript`))