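; Child Blueprint for the secondary character Jean-Driss on night 1, an NPC with a choice-based dialogue.
; BeginPlay loads his dialogue, choice texts and name into inherited variables before calling the parent logic.
; ShowChoices hides the third and end choice buttons, leaving the other options to the parent.
; Both choices switch him to secondary dialogue and disable further choices, but only the first lowers the Game Instance's QuotientSocial.
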(event `self.ReceiveBeginPlay`
  (set `self.BaseDialogue` (`self.DialogueJean-DrissNuit1`))
  (set `self.DialogueChoice1` (`self.DialogueChoice1Jean-DrissNuit1`))
  (set `self.DialogueChoice2` (`self.DialogueChoice2Jean-DrissNuit1`))
  (set `self.LineChoice1` (`self.LineChoice1Jean-DrissNuit1`))
  (set `self.LineChoice2` (`self.LineChoice2Jean-DrissNuit1`))
  (set `self.CharaName` "Jean-Driss")
  (set `self.NumberOfChoices` 1)
  (`parent.ReceiveBeginPlay`))

(event `self.ShowChoices`
  (`parent.ShowChoices`)
  (`Widget.SetVisibility` (`/Game/Blueprint/Widget/Dialogue/WB_Choice.BTN_ChoiceEnd` (`self.UIchoice`)) "Hidden")
  (`Widget.SetVisibility` (`/Game/Blueprint/Widget/Dialogue/WB_Choice.BTN_Choice3` (`self.UIchoice`)) "Hidden"))

(event `/Game/Blueprint/Interfaces/BPI_DialogueChoice.Choice1`
  (`parent.Choice1`)
  (`/Engine/EditorBlueprintResources/StandardMacros.DecrementInt` (`/Game/Blueprint/GameSystem/GI_Havencrest.QuotientSocial` (`self.GameInstanceRef`))
    (:`  `
      (set `self.BaseDialogue` (`self.DialogueSecondaryJean-DrissNuit1`) :!label _label)
      (set `self.isChoiceChara` false)
      (set `self.HasChoice` false))))

(event `/Game/Blueprint/Interfaces/BPI_DialogueChoice.Choice2`
  (`parent.Choice2`)
  (goto _label))

(fn `UserConstructionScript`
  (`parent.UserConstructionScript`))