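; Secondary character Blueprint for Jeanne-Claude on the second night ("Nuit2"), a dialogue NPC built on a parent choice-dialogue class.
; BeginPlay fills the inherited dialogue, choice and name variables before calling the parent, and ShowChoices hides the third and end choice buttons.
; Choice 1 raises and choice 2 lowers the GameInstance's QuotientSocial.
; ChoiceEnd switches to secondary dialogue and clears the choice-character flag.
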(event `self.ReceiveBeginPlay`
  (set `self.BaseDialogue` (`self.DialogueJeanne-ClaudeNuit2`))
  (set `self.DialogueChoice1` (`self.DialogueChoice1Jeanne-ClaudeNuit2`))
  (set `self.DialogueChoice2` (`self.DialogueChoice2Jeanne-ClaudeNuit2`))
  (set `self.DialogueChoiceEnd` (`self.DialogueChoiceEndJeanne-ClaudeNuit2`))
  (set `self.LineChoice1` (`self.LineChoice1Jeanne-ClaudeNuit2`))
  (set `self.LineChoice2` (`self.LineChoice2Jeanne-ClaudeNuit2`))
  (set `self.CharaName` "Jeanne-Claude")
  (set `self.NumberOfChoices` 1)
  (`parent.ReceiveBeginPlay`))

(event `self.ShowChoices`
  (bind _uichoice (`self.UIchoice`))
  (`parent.ShowChoices`)
  (`Widget.SetVisibility` (`/Game/Blueprint/Widget/Dialogue/WB_Choice.BTN_ChoiceEnd` _uichoice) "Hidden")
  (`Widget.SetVisibility` (`/Game/Blueprint/Widget/Dialogue/WB_Choice.BTN_Choice3` _uichoice) "Hidden"))

(event `/Game/Blueprint/Interfaces/BPI_DialogueChoice.Choice1`
  (`parent.Choice1`)
  (`/Engine/EditorBlueprintResources/StandardMacros.IncrementInt` (`/Game/Blueprint/GameSystem/GI_Havencrest.QuotientSocial` (`self.GameInstanceRef`))))

(event `/Game/Blueprint/Interfaces/BPI_DialogueChoice.Choice2`
  (`parent.Choice2`)
  (`/Engine/EditorBlueprintResources/StandardMacros.DecrementInt` (`/Game/Blueprint/GameSystem/GI_Havencrest.QuotientSocial` (`self.GameInstanceRef`))))

(event `/Game/Blueprint/Interfaces/BPI_DialogueChoice.ChoiceEnd`
  (`parent.ChoiceEnd`)
  (set `self.BaseDialogue` (`self.DialogueSecondaryJeanne-ClaudeNuit2`))
  (set `self.isChoiceChara` false))

(fn `UserConstructionScript`
  (`parent.UserConstructionScript`))