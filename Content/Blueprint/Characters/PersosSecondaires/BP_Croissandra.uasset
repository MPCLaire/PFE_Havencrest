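; BP_Croissandra is the secondary character Croissandra, a child Blueprint that feeds her dialogue and choice content into a parent dialogue system.
; BeginPlay loads the "Nuit2" lines and a single choice before calling the parent.
; Any choice closes the choice phase, with the first also raising QuotientSocial on the GameInstance.
; Afterwards, ShowChoices alternates secondary dialogues through FlipFlops, with the pair depending on IsNight1.
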(event `self.ReceiveBeginPlay`
  (set `self.BaseDialogue` (`self.DialogueCroissandraNuit2`))
  (set `self.DialogueChoice1` (`self.DialogueChoice1CroissandraNuit2`))
  (set `self.DialogueChoice2` (`self.DialogueChoice2CroissandraNuit2`))
  (set `self.DialogueChoice3` (`self.DialogueChoice3CroissandraNuit2`))
  (set `self.LineChoice1` (`self.LineChoice1CroissandraNuit2`))
  (set `self.LineChoice2` (`self.LineChoice2CroissandraNuit2`))
  (set `self.LineChoice3` (`self.LineChoice3CroissandraNuit2`))
  (set `self.CharaName` "Croissandra")
  (set `self.NumberOfChoices` 1)
  (`parent.ReceiveBeginPlay`))

(event `self.ShowChoices`
  (`parent.ShowChoices`)
  (`Widget.SetVisibility` (`/Game/Blueprint/Widget/Dialogue/WB_Choice.BTN_ChoiceEnd` (`self.UIchoice`)) "Hidden")
  (if (`self.isChoiceChara`)
    _
    (elif (`/Game/Blueprint/GameSystem/GI_Havencrest.isNight1` (`self.GameInstanceRef`))
      (`/Engine/EditorBlueprintResources/StandardMacros.FlipFlop`
        (:`A`
          (set `self.BaseDialogue` (`self.DialogueSecondaryCroissandraNuit2`) :!label _label))
        (:`B`
          (set `self.BaseDialogue` (`self.DialogueSecondary2CroissandraNuit2`))))
      (else
        (`/Engine/EditorBlueprintResources/StandardMacros.FlipFlop`
          (:`A`
            (goto _label))
          (:`B`
            (set `self.BaseDialogue` (`self.DialogueSecondary3CroissandraNuit2`))))))))

(event `/Game/Blueprint/Interfaces/BPI_DialogueChoice.Choice1`
  (`parent.Choice1`)
  (`/Engine/EditorBlueprintResources/StandardMacros.IncrementInt` (`/Game/Blueprint/GameSystem/GI_Havencrest.QuotientSocial` (`self.GameInstanceRef`))
    (:`  `
      (set `self.isChoiceChara` false :!label _label_2)
      (set `self.HasChoice` false))))

(event `/Game/Blueprint/Interfaces/BPI_DialogueChoice.Choice2`
  (`parent.Choice2`)
  (goto _label_2))

(event `/Game/Blueprint/Interfaces/BPI_DialogueChoice.Choice3`
  (`parent.Choice3`)
  (goto _label_2))

(fn `UserConstructionScript`
  (`parent.UserConstructionScript`))