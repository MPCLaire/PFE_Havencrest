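; Secondary character Emma, a child dialogue Blueprint that fills the parent's dialogue, choice and name variables with her own content.
; The first choice display sets a persistent GameInstance flag and switches to her choice dialogue.
; Later displays hide the end-choice button and, outside choice mode, alternate two secondary dialogues via FlipFlop.
; Picking any choice exits choice mode, with the first raising and the third lowering the GameInstance social quotient.
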(event `self.ReceiveBeginPlay`
  (set `self.BaseDialogue` (`self.DialogueSecondaryEmma`))
  (set `self.DialogueChoice1` (`self.DialogueChoice1Emma`))
  (set `self.DialogueChoice2` (`self.DialogueChoice2Emma`))
  (set `self.DialogueChoice3` (`self.DialogueChoice3Emma`))
  (set `self.LineChoice1` (`self.LineChoice1Emma`))
  (set `self.LineChoice2` (`self.LineChoice2Emma`))
  (set `self.LineChoice3` (`self.LineChoice3Emma`))
  (set `self.CharaName` "Emma")
  (set `self.NumberOfChoices` 1)
  (set `self.isChoiceChara` false)
  (`parent.ReceiveBeginPlay`))

(event `self.ShowChoices`
  (bind _gameinstanceref (`self.GameInstanceRef`))
  (`parent.ShowChoices`)
  (if (`/Game/Blueprint/GameSystem/GI_Havencrest.hasEmmaSayFirstLine` _gameinstanceref)
    (`Widget.SetVisibility` (`/Game/Blueprint/Widget/Dialogue/WB_Choice.BTN_ChoiceEnd` (`self.UIchoice`)) "Hidden")
    (if (not (`self.isChoiceChara`))
      (`/Engine/EditorBlueprintResources/StandardMacros.FlipFlop`
        (:`A`
          (set `self.BaseDialogue` (`self.DialogueSecondary2Emma`)))
        (:`B`
          (set `self.BaseDialogue` (`self.DialogueSecondary3Emma`)))))
    (else
      (set `self.isChoiceChara` true)
      (set `/Game/Blueprint/GameSystem/GI_Havencrest.hasEmmaSayFirstLine` true _gameinstanceref)
      (set `self.BaseDialogue` (`self.DialogueEmma`)))))

(event `/Game/Blueprint/Interfaces/BPI_DialogueChoice.Choice1`
  (`parent.Choice1`)
  (`/Engine/EditorBlueprintResources/StandardMacros.IncrementInt` (`/Game/Blueprint/GameSystem/GI_Havencrest.QuotientSocial` (`self.GameInstanceRef`))
    (:`  `
      (set `self.isChoiceChara` false :!label _label)
      (set `self.HasChoice` false))))

(event `/Game/Blueprint/Interfaces/BPI_DialogueChoice.Choice2`
  (`parent.Choice2`)
  (goto _label))

(event `/Game/Blueprint/Interfaces/BPI_DialogueChoice.Choice3`
  (`parent.Choice3`)
  (`/Engine/EditorBlueprintResources/StandardMacros.DecrementInt` (`/Game/Blueprint/GameSystem/GI_Havencrest.QuotientSocial` (`self.GameInstanceRef`))
    (:`  `
      (goto _label))))

(fn `UserConstructionScript`
  (`parent.UserConstructionScript`))