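; BP_LaetriciaNuit1 is the secondary character Laetricia for night 1, a dialogue character with a player choice.
; BeginPlay fills the parent's dialogue, choice and name variables, and ShowChoices hides the third and end choice buttons.
; Either choice runs parent logic, switches to secondary dialogue and disables further choices.
; The second choice also increments QuotientSocial on the GameInstance.
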(event `self.ReceiveBeginPlay`
  (set `self.BaseDialogue` (`self.DialogueLaetriciaNuit1`))
  (set `self.DialogueChoice1` (`self.DialogueChoice1LaetriciaNuit1`))
  (set `self.DialogueChoice2` (`self.DialogueChoice2LaetriciaNuit1`))
  (set `self.LineChoice1` (`self.LineChoice1LaetriciaNuit1`))
  (set `self.LineChoice2` (`self.LineChoice2LaetriciaNuit1`))
  (set `self.CharaName` "Laetricia")
  (set `self.NumberOfChoices` 1)
  (`parent.ReceiveBeginPlay`))

(event `self.ShowChoices`
  (`parent.ShowChoices`)
  (`Widget.SetVisibility` (`/Game/Blueprint/Widget/Dialogue/WB_Choice.BTN_ChoiceEnd` (`self.UIchoice`)) "Hidden")
  (`Widget.SetVisibility` (`/Game/Blueprint/Widget/Dialogue/WB_Choice.BTN_Choice3` (`self.UIchoice`)) "Hidden"))

(event `/Game/Blueprint/Interfaces/BPI_DialogueChoice.Choice1`
  (`parent.Choice1`)
  (set `self.BaseDialogue` (`self.DialogueSecondaryLaetriciaNuit1`) :!label _label)
  (set `self.isChoiceChara` false)
  (set `self.HasChoice` false))

(event `/Game/Blueprint/Interfaces/BPI_DialogueChoice.Choice2`
  (`parent.Choice2`)
  (`/Engine/EditorBlueprintResources/StandardMacros.IncrementInt` (`/Game/Blueprint/GameSystem/GI_Havencrest.QuotientSocial` (`self.GameInstanceRef`))
    (:`  `
      (goto _label))))

(fn `UserConstructionScript`
  (`parent.UserConstructionScript`))