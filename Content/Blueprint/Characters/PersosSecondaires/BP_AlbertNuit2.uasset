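; Dialogue Blueprint for Albert, a secondary character on night 2, built on a parent character class that provides the choice logic.
; BeginPlay loads his dialogue, choice responses and name into inherited variables before calling the parent.
; Choices 1 and 3 raise and lower the GameInstance's social quotient, and any choice clears the choice flags.
; ShowChoices hides the end button and, without an active choice, alternates between two secondary dialogues through a FlipFlop.
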(event `self.ReceiveBeginPlay`
  (set `self.BaseDialogue` (`self.DialogueAlbertNuit2`))
  (set `self.DialogueChoice1` (`self.DialogueChoice1AlbertNuit2`))
  (set `self.DialogueChoice2` (`self.DialogueChoice2AlbertNuit2`))
  (set `self.DialogueChoice3` (`self.DialogueChoice3AlbertNuit2`))
  (set `self.LineChoice1` (`self.LineChoice1AlbertNuit2`))
  (set `self.LineChoice2` (`self.LineChoice2AlbertNuit2`))
  (set `self.LineChoice3` (`self.LineChoice3AlbertNuit2`))
  (set `self.CharaName` "Albert")
  (set `self.NumberOfChoices` 1)
  (`parent.ReceiveBeginPlay`))

(event `self.ShowChoices`
  (`parent.ShowChoices`)
  (`Widget.SetVisibility` (`/Game/Blueprint/Widget/Dialogue/WB_Choice.BTN_ChoiceEnd` (`self.UIchoice`)) "Hidden")
  (if (not (`self.isChoiceChara`))
    (`/Engine/EditorBlueprintResources/StandardMacros.FlipFlop`
      (:`A`
        (set `self.BaseDialogue` (`self.DialogueSecondaryAlbertNuit2`)))
      (:`B`
        (set `self.BaseDialogue` (`self.DialogueSecondary2AlbertNuit2`))))))

(event `/Game/Blueprint/Interfaces/BPI_DialogueChoice.Choice1`
  (`parent.Choice1`)
  (`/Engine/EditorBlueprintResources/StandardMacros.IncrementInt` (`/Game/Blueprint/GameSystem/GI_Havencrest.QuotientSocial` (`self.GameInstanceRef`))
    (:`  `
      (set `self.isChoiceChara` false :!label _label)
      (set `self.HasChoice` false))))

(event `/Game/Blueprint/Interfaces/BPI_DialogueChoice.Choice2`
  (`parent.Choice2`)
  (goto _label))

(event `/Game/Blueprint/Interfaces/BPI_DialogueChoice.Choice3`
  (`parent.Choice3`)
  (`/Engine/EditorBlueprintResources/StandardMacros.DecrementInt` (`/Game/Blueprint/GameSystem/GI_Havencrest.QuotientSocial` (`self.GameInstanceRef`))
    (:`  `
      (goto _label))))

(fn `UserConstructionScript`
  (`parent.UserConstructionScript`))