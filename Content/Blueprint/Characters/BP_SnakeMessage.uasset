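; BP_SnakeMessage is a dialogue character for the snake sequence that gates the win on the snake having a key.
; On BeginPlay it sets its dialogue and display name, then defers to its parent.
; When a BP_Snake overlaps its capsule, it calls SnakeWin if the snake has the key.
; Otherwise it starts dialogue as "Serpent", clears the snake's Snaking flag and calls StartSnake on PlayerSnakeRef.
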(event `self.ReceiveBeginPlay`
  (set `self.BaseDialogue` (`self.MessageSnake`))
  (set `self.CharaName` "Snake")
  (`parent.ReceiveBeginPlay`))

(event `self.Capsule.OnComponentBeginOverlap`
  (params (OverlappedComponent :type "PrimitiveComponent Object Reference") (OtherActor :type "Actor Object Reference") (OtherComp :type "PrimitiveComponent Object Reference") (OtherBodyIndex :type Integer) (bFromSweep :type Boolean) (SweepResult :type "HitResult Structure (by ref)"))
  (bind _asbp_snake (cast `/Game/Blueprint/Mini_Jeux/Snake/BP_Snake` OtherActor))
  (set `self.SnakeRef` _asbp_snake)
  (if (`/Game/Blueprint/Mini_Jeux/Snake/BP_Snake.HasKey` _asbp_snake)
    (`/Game/Blueprint/Mini_Jeux/Snake/BP_Snake.SnakeWin` (`self.SnakeRef`))
    (else
      (set `self.CharaName` "Serpent")
      (`self.StartTalkingToChara`)
      (set `/Game/Blueprint/Mini_Jeux/Snake/BP_Snake.Snaking?` false (`self.SnakeRef`))
      (`/Game/Blueprint/Mini_Jeux/Snake/BP_PlayerSnake.StartSnake` (`self.PlayerSnakeRef`)))))

(fn `UserConstructionScript`
  (`parent.UserConstructionScript`))