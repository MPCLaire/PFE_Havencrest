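; BP_JeanNuit2 is a dialogue character blueprint for Jean, likely on the second night, that leads into the game's ending.
; It sets Jean's base dialogue at BeginPlay, then swaps it once on capsule overlap to the Pierre-arrest dialogue if the game instance's CanArrestPierre is set.
; ShowChoices extends the parent, calls Fade on BP_Police's plane, waits briefly, then opens the good or bad ending level based on the same flag.
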(event `self.ReceiveBeginPlay`
  (set `self.BaseDialogue` (`self.DialogueJeanNuit2`))
  (set `self.CharaName` "Jean")
  (`parent.ReceiveBeginPlay`))

(event `self.Capsule.OnComponentBeginOverlap`
  (params (OverlappedComponent :type "PrimitiveComponent Object Reference") (OtherActor :type "Actor Object Reference") (OtherComp :type "PrimitiveComponent Object Reference") (OtherBodyIndex :type Integer) (bFromSweep :type Boolean) (SweepResult :type "HitResult Structure (by ref)"))
  (if (`/Game/Blueprint/GameSystem/GI_Havencrest.CanArrestPierre` (`self.GameInstanceRef`))
    (`/Engine/EditorBlueprintResources/StandardMacros.DoOnce` false
      (:`Completed`
        (set `self.Dialogue` (`self.DialogueJeanNuit2PierreArrest`))
        (`KismetSystemLibrary.PrintString` "Hello")))))

(event `self.ShowChoices`
  (`parent.ShowChoices`)
  (bind _returnvalue (`GameplayStatics.GetActorOfClass` "/Game/Assets/DecorsAsset/Batiments/Police/BP_Police.BP_Police_C"))
  (`/Game/Assets/DecorsAsset/Batiments/BP_Batiments_Parent.Fade` _returnvalue (`/Game/Assets/DecorsAsset/Batiments/BP_Batiments_Parent.FadePlane` _returnvalue) false)
  (`KismetSystemLibrary.Delay` 1.0)
  (if (`/Game/Blueprint/GameSystem/GI_Havencrest.CanArrestPierre` (`self.GameInstanceRef`))
    (`GameplayStatics.OpenLevelBySoftObjectPtr` "/Game/Maps/BonneFin.BonneFin")
    (else
      (`GameplayStatics.OpenLevelBySoftObjectPtr` "/Game/Maps/MauvaiseFin.MauvaiseFin"))))

(fn `UserConstructionScript`
  (`parent.UserConstructionScript`))