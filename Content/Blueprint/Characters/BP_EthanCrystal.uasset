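; BP_EthanCrystal is a dialogue character Blueprint tied to Ethan's crystal, built on a parent class that supplies the dialogue and choice logic.
; On BeginPlay it selects the normal dialogue, marks itself as a non-choice character with a placeholder name, then runs the parent setup.
; Its ShowChoices override calls the parent, then clears the crystal possession flag on the referenced Ethan.
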(event `self.ReceiveBeginPlay`
  (set `self.BaseDialogue` (`self.DialogueNormal`))
  (set `self.isChoiceChara` false)
  (set `self.CharaName` "Nochara")
  (`parent.ReceiveBeginPlay`))

(event `self.ShowChoices`
  (`parent.ShowChoices`)
  (set `/Game/Blueprint/MainCharacter/Blueprints/BP_Ethan.hasCristal` false (`self.EthanRef`)))

(fn `UserConstructionScript`
  (`parent.UserConstructionScript`))