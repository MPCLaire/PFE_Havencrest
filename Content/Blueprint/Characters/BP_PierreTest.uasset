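; BP_PierreTest is a dialogue character named Pierre, built as a child Blueprint that supplies his text to a parent class.
; BeginPlay fills the inherited base dialogue, choices, choice lines and name before calling the parent's BeginPlay.
; Overriding Choice1 runs the parent logic, flags an important first choice as made and swaps the three choices for follow-up dialogue.
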(event `self.ReceiveBeginPlay`
  (set `self.BaseDialogue` (`self.DialoguePierre1`))
  (set `self.DialogueChoice1` (`self.DialogueChoixPierre1`))
  (set `self.DialogueChoice2` (`self.DialogueChoixPierre2`))
  (set `self.DialogueChoice3` (`self.DialogueChoixPierre3`))
  (set `self.DialogueChoiceEnd` (`self.DialogueChoixPierreEnd`))
  (set `self.LineChoice1` (`self.LineChoicePierre1`))
  (set `self.LineChoice2` (`self.LineChoicePierre2`))
  (set `self.LineChoice3` (`self.LineChoicePierre3`))
  (set `self.CharaName` "Pierre")
  (`parent.ReceiveBeginPlay`))

(event `/Game/Blueprint/Interfaces/BPI_DialogueChoice.Choice1`
  (`parent.Choice1`)
  (set `self.HasMadeImportantChoice1` true)
  (set `self.DialogueChoice1` (`self.DialogueChoicePierre1-1`))
  (set `self.DialogueChoice2` (`self.DialogueChoicePierre1-2`))
  (set `self.DialogueChoice3` (`self.DialogueChoicePierre1-3`)))

(fn `UserConstructionScript`
  (`parent.UserConstructionScript`))