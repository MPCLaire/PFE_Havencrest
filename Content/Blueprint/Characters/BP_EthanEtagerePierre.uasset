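; Character Blueprint for EthanEtagerePierre, a dialogue actor that is removed at a specific story state.
; On BeginPlay it sets BaseDialogue to DialogueNormal, clears the choice-character flag and names itself "Nochara" before calling the parent BeginPlay.
; It then destroys itself if the game instance's GameState is "Sortie Pierre MJ".
; All other behavior comes from the parent class.
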(event `self.ReceiveBeginPlay`
  (set `self.BaseDialogue` (`self.DialogueNormal`))
  (set `self.isChoiceChara` false)
  (set `self.CharaName` "Nochara")
  (`parent.ReceiveBeginPlay`)
  (switch `/Game/Blueprint/GameSystem/E_Instance` (`/Game/Blueprint/GameSystem/GI_Havencrest.GameState` (`self.GameInstanceRef`))
    (:`NewEnumerator2`
      (`self.K2_DestroyActor`))))

(event `self.ReceiveTick`
  (params (DeltaSeconds :type "Float (single-precision)")))

(fn `UserConstructionScript`
  (`parent.UserConstructionScript`))