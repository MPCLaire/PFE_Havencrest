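; Parent Blueprint for dialogue characters with a nested second level of choices, extending a choice-character parent and naming the character "Pierre".
; BeginPlay loads the three base choices, their lines and the end dialogue.
; Picking the first choice saves the current choice state and swaps in a sub-set of choices.
; Once all sub-choices are made, it restores the saved state and base dialogues.
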(event `self.ReceiveBeginPlay`
  (`self.SetDialoguesForChoiceChara`)
  (set `self.CharaName` "Pierre")
  (`parent.ReceiveBeginPlay`))

(event `/Game/Blueprint/Interfaces/BPI_DialogueChoice.Choice1`
  (`parent.Choice1`)
  (if (`self.HasMadeImportantChoice1`)
    ;[1 1 1] Set quelques variables lorsqu'on a fini de sélectionner les nouveaux choix
    (if (== (`self.ChoicesMade`) (`self.NumberOfChoices`)) :!label _label
      (set `self.ChoicesMade` (`self.OldChoicesMade`))
      (set `self.isChoice1Made` (`self.isOldChoice1Made`))
      (set `self.isChoice2Made` (`self.isOldChoice2Made`))
      (set `self.isChoice3Made` (`self.isOldChoice3Made`))
      (set `self.HasMadeImportantChoice1` false)
      (`self.SetDialoguesForChoiceChara`))
    (else
      ;[1 1 1] Une fois que l'on a fait le choix qui amène sur d'autres choix, on set les variables de dialogues pour les nouveaux choix et on conserve les variables liées au premier dialogue
      (set `self.OldChoicesMade` (`self.ChoicesMade`))
      (set `self.isOldChoice1Made` (`self.isChoice1Made`))
      (set `self.isOldChoice2Made` (`self.isChoice2Made`))
      (set `self.isOldChoice3Made` (`self.isChoice3Made`))
      (set `self.HasMadeImportantChoice1` true)
      (set `self.ChoicesMade` 0)
      (set `self.isChoice1Made` false)
      (set `self.isChoice2Made` false)
      (set `self.isChoice3Made` false)
      (set `self.DialogueChoice1` (`self.DialogueChoiceChara1-1`))
      (set `self.DialogueChoice2` (`self.DialogueChoiceChara1-2`))
      (set `self.DialogueChoice3` (`self.DialogueChoiceChara1-3`))
      (set `self.LineChoice1` (`self.LineChoiceChara1-1`))
      (set `self.LineChoice2` (`self.LineChoiceChara1-2`))
      (set `self.LineChoice3` (`self.LineChoiceChara1-3`)))))

(event `/Game/Blueprint/Interfaces/BPI_DialogueChoice.Choice2`
  (`parent.Choice2`)
  (if (`self.HasMadeImportantChoice1`) :!label _label_2
    (goto _label)))

(event `/Game/Blueprint/Interfaces/BPI_DialogueChoice.Choice3`
  (`parent.Choice3`)
  (goto _label_2))

(fn `UserConstructionScript`
  (`parent.UserConstructionScript`))