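; BP_EthanTrouRat is a non-choice dialogue interactable, apparently a rat hole, that can lead into the PierreMiniJeu level.
; It extends a parent dialogue character and picks DialogueNormal or Dialogue2 based on the GameInstance CanGoToCafard flag when conversation starts.
; When the event ends with that flag set, it triggers PierreMaisonRef's FadeEtage, waits briefly, zeroes the saved EthanSpawn and opens the mini-game level.
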(event `self.ReceiveBeginPlay`
  (set `self.BaseDialogue` (`self.DialogueNormal`))
  (set `self.isChoiceChara` false)
  (set `self.CharaName` "Nochara")
  (`parent.ReceiveBeginPlay`))

(event `self.ShowChoices`
  (`parent.ShowChoices`))

(event `self.EndEvent`
  (if (`/Game/Blueprint/GameSystem/GI_Havencrest.CanGoToCafard` (`self.GameInstanceRef`))
    (`/Game/Assets/DecorsAsset/Batiments/Pierre/BP_Pierre_Maison.FadeEtage` (`self.PierreMaisonRef`))
    (`KismetSystemLibrary.Delay` 0.7)
    (set `/Game/Blueprint/GameSystem/GI_Havencrest.EthanSpawn` (0.0 0.0 0.0) (`self.GameInstanceRef`))
    (`GameplayStatics.OpenLevelBySoftObjectPtr` "/Game/Maps/PierreMiniJeu_Level.PierreMiniJeu_Level")))

(event `/Game/Blueprint/Interfaces/BPI_TalkToChara.StartTalkingToChara`
  (bind _dialoguenormal (`self.DialogueNormal`))
  (bind _dialogue2 (`self.Dialogue2`))
  (if (`/Game/Blueprint/GameSystem/GI_Havencrest.CanGoToCafard` (`self.GameInstanceRef`))
    (set `self.BaseDialogue` _dialoguenormal)
    (set `self.Dialogue` _dialoguenormal)
    (else
      (set `self.BaseDialogue` _dialogue2)
      (set `self.Dialogue` _dialogue2)))
  (`parent.StartTalkingToChara`))

(fn `UserConstructionScript`
  (`parent.UserConstructionScript`))