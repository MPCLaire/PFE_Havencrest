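; Dialogue character Blueprint for EthanMineNo, set up on BeginPlay as a non-choice character named "Nochara" that uses its normal dialogue.
; Capsule overlap events track whether Ethan is within range.
; The ShowChoices override runs the parent logic, then, if Ethan is absent, hides EPerso and hides it again after a short delay, with debug prints along the way.
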(event `self.ReceiveBeginPlay`
  (set `self.BaseDialogue` (`self.DialogueNormal`))
  (set `self.isChoiceChara` false)
  (set `self.CharaName` "Nochara")
  (`parent.ReceiveBeginPlay`))

(event `self.Capsule.OnComponentBeginOverlap`
  (params (OverlappedComponent :type "PrimitiveComponent Object Reference") (OtherActor :type "Actor Object Reference") (OtherComp :type "PrimitiveComponent Object Reference") (OtherBodyIndex :type Integer) (bFromSweep :type Boolean) (SweepResult :type "HitResult Structure (by ref)"))
  (if (== OtherActor (`self.EthanRef`))
    (set `self.isWithEthan` true)))

(event `self.ShowChoices`
  (`parent.ShowChoices`)
  (if (not (`self.isWithEthan`))
    (`KismetSystemLibrary.PrintString` "Hello" true true (struct :`R` 1.0 :`G` 1.0 :`B` 1.0 :`A` 1.0))
    (`SceneComponent.SetVisibility` (`self.E_perso`) false false)
    (`KismetSystemLibrary.PrintString` "Hello2" true true (struct :`R` 1.0 :`G` 1.0 :`B` 1.0 :`A` 1.0))
    (`KismetSystemLibrary.Delay` 0.2)
    (`SceneComponent.SetVisibility` (`self.E_perso`) false false)))

(event `self.Capsule.OnComponentEndOverlap`
  (params (OverlappedComponent :type "PrimitiveComponent Object Reference") (OtherActor :type "Actor Object Reference") (OtherComp :type "PrimitiveComponent Object Reference") (OtherBodyIndex :type Integer))
  (if (== OtherActor (`self.EthanRef`))
    (set `self.isWithEthan` false)))

(fn `UserConstructionScript`
  (`parent.UserConstructionScript`))