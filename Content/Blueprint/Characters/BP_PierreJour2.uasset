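; Dialogue character Blueprint for Pierre on "Jour2" (day 2), built on a parent class that supplies the dialogue and choice behavior.
; BeginPlay assigns his name, dialogues and choice lines before calling the parent, then sets the choice count to three.
; The first prompt hides the third button; picking either option swaps the first two choices to second-stage content, so the next prompt shows all three.
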(event `self.ReceiveBeginPlay`
  (set `self.BaseDialogue` (`self.DialoguePierreJour2`))
  (set `self.DialogueChoice1` (`self.DialogueChoice1-1PierreJour2`))
  (set `self.DialogueChoice2` (`self.DialogueChoice1-2PierreJour2`))
  (set `self.DialogueChoice3` (`self.DialogueChoice2-3PierreJour2`))
  (set `self.DialogueChoiceEnd` (`self.DialogueChoiceEndPierreJour2`))
  (set `self.LineChoice1` (`self.LineChoice1-1PierreJour2`))
  (set `self.LineChoice2` (`self.LineChoice1-2PierreJour2`))
  (set `self.LineChoice3` (`self.LineChoice2-3PierreJour2`))
  (set `self.CharaName` "Pierre")
  (`parent.ReceiveBeginPlay`)
  (set `self.NumberOfChoices` 3))

(event `self.ShowChoices`
  (bind _btn_choice3 (`/Game/Blueprint/Widget/Dialogue/WB_Choice.BTN_Choice3` (`self.UIchoice`)))
  (`parent.ShowChoices`)
  (if (`self.IsAtFirstChoice`)
    (`Widget.SetVisibility` _btn_choice3 "Hidden")
    (else
      (`Widget.SetVisibility` _btn_choice3 "Visible"))))

(event `/Game/Blueprint/Interfaces/BPI_DialogueChoice.Choice1`
  (`parent.Choice1`)
  (if (`self.IsAtFirstChoice`) :!label _label
    (set `self.IsAtFirstChoice` false)
    (set `self.DialogueChoice1` (`self.DialogueChoice2-1PierreJour2`))
    (set `self.DialogueChoice2` (`self.DialogueChoice2-2PierreJour2`))
    (set `self.LineChoice1` (`self.LineChoice2-1PierreJour2`))
    (set `self.LineChoice2` (`self.LineChoice2-2PierreJour2`))))

(event `/Game/Blueprint/Interfaces/BPI_DialogueChoice.Choice2`
  (`parent.Choice2`)
  (goto _label))

(fn `UserConstructionScript`
  (`parent.UserConstructionScript`))