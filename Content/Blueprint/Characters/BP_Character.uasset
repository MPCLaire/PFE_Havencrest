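; BP_Character is a talkable NPC that plays branching dialogue with BP_Ethan.
; While Ethan overlaps its capsule, a looping timer polls his E press to start each line, which a second timer types letter by letter into WB_DialogueTest.
; After the last line, it either opens WB_Choice, whose options swap in another dialogue array through the Choice events, or closes the dialogue.
; The end choice clears HasChoice so its dialogue can finish.
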(event `self.ReceiveBeginPlay`)

(event `Talk`
  ;[1 1 1] Ajoute le texte lettre par lettre
  (`self.UI`
    (:`then`
      _)
    (:`else`
      (bind _returnvalue (`|CreateWidget` "/Game/Blueprint/Widget/Dialogue/WB_DialogueTest.WB_DialogueTest_C" (`GameplayStatics.GetPlayerController` 0)))
      (bind _output_get (set `self.UI` _returnvalue))
      (`UserWidget.AddToViewport` _output_get 0)))
  (bind _output_get_2 (set `self.Letters` (`KismetStringLibrary.Concat_StrStr` (`self.Letters`) (`|GetArrayItem` (`KismetStringLibrary.GetCharacterArrayFromString` (`|GetArrayItem` (`self.Dialogue`) (`self.dialogueIndex`))) (`self.CharaIndex`)))))
  (`TextBlock.SetText` (`/Game/Blueprint/Widget/Dialogue/WB_DialogueTest.TalkText` (`self.UI`)) (`KismetTextLibrary.Conv_StringToText` _output_get_2))
  (bind _result (`/Engine/EditorBlueprintResources/StandardMacros.IncrementInt` (`self.CharaIndex`))
    (:`  `
      ;[1 1 1] Reset pour le prochain dialogue
      (if (== _result (`KismetArrayLibrary.Array_Length` (`KismetStringLibrary.GetCharacterArrayFromString` (`|GetArrayItem` (`self.Dialogue`) (`self.dialogueIndex`)))))
        (`/Engine/EditorBlueprintResources/StandardMacros.IncrementInt` (`self.dialogueIndex`)
          (:`  `
            (set `self.CharaIndex` 0)
            (set `self.Letters` "")
            (`KismetSystemLibrary.K2_ClearAndInvalidateTimerHandle` (stale `StartTalking` _returnvalue))))))))

(event `StartTalking`
  (bind _ethanref (`self.EthanRef`))
  ;[1 1 1] Quand on appuie sur E, ça démarre le dialogue
  ;[1 1 1] Choisi la ligne de dialogue s'il y en a une.
  (if (`/Game/Blueprint/MainCharacter/Blueprints/BP_Ethan.EPressed` (stale `self.Capsule.OnComponentBeginOverlap` _output_get))
    (if (< (`self.dialogueIndex`) (`KismetArrayLibrary.Array_Length` (`self.Dialogue`)))
      (set `/Game/Blueprint/MainCharacter/Blueprints/BP_Ethan.isTalking` true _ethanref)
      (bind _returnvalue (`KismetSystemLibrary.K2_SetTimerDelegate` (delegate `Talk`) (`self.TextTime`) true))
      (else
        ;[1 1 1] Affiche les choix
        (if (`self.HasChoice`)
          (bind _returnvalue_2 (`|CreateWidget` "/Game/Blueprint/Widget/Dialogue/WB_Choice.WB_Choice_C"))
          (bind _output_get (set `self.UIchoice` _returnvalue_2))
          (`UserWidget.AddToViewport` _output_get 0)
          (set `/Game/Blueprint/Widget/Dialogue/WB_Choice.CharaRef` self _output_get)
          (set `self.Letters` "")
          (else
            ;[1 1 1] Met fin au dialogue
            (set `/Game/Blueprint/MainCharacter/Blueprints/BP_Ethan.isTalking` false _ethanref)
            (`Widget.RemoveFromParent` (`self.UI`))
            (set `self.dialogueIndex` 0)
            (set `self.UI` null)))))))

(event `self.Capsule.OnComponentBeginOverlap`
  (params (OverlappedComponent :type "PrimitiveComponent Object Reference") (OtherActor :type "Actor Object Reference") (OtherComp :type "PrimitiveComponent Object Reference") (OtherBodyIndex :type Integer) (bFromSweep :type Boolean) (SweepResult :type "HitResult Structure (by ref)"))
  ;[1 1 1] Quand on appuie sur E, ça démarre le dialogue
  (bind _asbp_ethan (cast `/Game/Blueprint/MainCharacter/Blueprints/BP_Ethan` OtherActor))
  (bind _output_get (set `self.EthanRef` _asbp_ethan))
  (bind _returnvalue (`KismetSystemLibrary.K2_SetTimerDelegate` (delegate `StartTalking`) 0.4 true)))

(event `self.Capsule.OnComponentEndOverlap`
  (params (OverlappedComponent :type "PrimitiveComponent Object Reference") (OtherActor :type "Actor Object Reference") (OtherComp :type "PrimitiveComponent Object Reference") (OtherBodyIndex :type Integer))
  ;[1 1 1] Faire en sorte que le dialogue ne se lance pas si on quitte la capsule collision
  (if (== OtherActor (`self.EthanRef`))
    (`KismetSystemLibrary.K2_ClearAndInvalidateTimerHandle` (stale `self.Capsule.OnComponentBeginOverlap` _returnvalue))))

(event `/Game/Blueprint/Interfaces/BPI_DialogueChoice.Choice1`
  ;[0 0.2549 1] Si on appuie sur le premier choix
  (`Widget.RemoveFromParent` (`self.UIchoice`))
  (set `self.Dialogue` (`self.DialogueChoice1`))
  (set `self.dialogueIndex` 0)
  (set `self.CharaIndex` 0)
  (`self.Talk`))

(event `/Game/Blueprint/Interfaces/BPI_DialogueChoice.Choice2`
  ;[0 0.2549 1] Si on appuie sur le deuxième choix
  (`Widget.RemoveFromParent` (`self.UIchoice`))
  (set `self.Dialogue` (`self.DialogueChoice2`))
  (set `self.dialogueIndex` 0)
  (set `self.CharaIndex` 0)
  (`self.Talk`))

(event `/Game/Blueprint/Interfaces/BPI_DialogueChoice.Choice3`
  ;[0 0.2549 1] Si on appuie sur le troisième choix
  (`Widget.RemoveFromParent` (`self.UIchoice`))
  (set `self.Dialogue` (`self.DialogueChoice3`))
  (set `self.dialogueIndex` 0)
  (set `self.CharaIndex` 0)
  (`self.Talk`))

(event `/Game/Blueprint/Interfaces/BPI_DialogueChoice.ChoiceEnd`
  ;[0 0.2549 1] Si on met fin au choix
  (`Widget.RemoveFromParent` (`self.UIchoice`))
  (set `self.Dialogue` (`self.DialogueChoiceEnd`))
  (set `self.dialogueIndex` 0)
  (set `self.CharaIndex` 0)
  (`self.Talk`)
  (set `self.HasChoice` false))

(fn `UserConstructionScript`)