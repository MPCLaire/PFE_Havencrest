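; Blueprint for the Day 1 Pierre character, extending a parent dialogue class with story-specific choice handling.
; The end-dialogue button stays hidden until CanPassDialogue is true.
; With HasMadeImportantChoice1 set, Choice1 unlocks that button and advances the objective message once, while Choice3 records in the Game Instance that Ethan knows of the bakery theft.
; Overridden choice events still call the parent logic.
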(event `self.ReceiveBeginPlay`
  (`parent.ReceiveBeginPlay`))

(event `self.ShowChoices`
  (`parent.ShowChoices`)
  (if (not (`self.canPassDialogue`))
    (`Widget.SetVisibility` (`/Game/Blueprint/Widget/Dialogue/WB_Choice.BTN_ChoiceEnd` (`self.UIchoice`)) "Hidden")))

(event `/Game/Blueprint/Interfaces/BPI_DialogueChoice.Choice1`
  (if (`self.HasMadeImportantChoice1`)
    (`|ExecutionSequence`
      (:`then_0`
        (`/Engine/EditorBlueprintResources/StandardMacros.DoOnce` false
          (:`Completed`
            (`Widget.SetVisibility` (`/Game/Blueprint/Widget/Dialogue/WB_Choice.BTN_ChoiceEnd` (`self.UIchoice`)) "Visible")
            (set `self.canPassDialogue` true)
            (bind _foundwidgets (`WidgetBlueprintLibrary.GetAllWidgetsOfClass` null))
            (message `/Game/Blueprint/Interfaces/BPI_Objectifs.NextObjectif` (`|GetArrayItem` _foundwidgets) (`self.Index`)))))
      (:`then_1`
        (`parent.Choice1` :!label _label)))
    (else
      (goto _label))))

(event `/Game/Blueprint/Interfaces/BPI_DialogueChoice.Choice3`
  (if (`self.HasMadeImportantChoice1`)
    (set `/Game/Blueprint/GameSystem/GI_Havencrest.EthanKnowsBakeryTheft` true (`self.GameInstanceRef`)))
  (`parent.Choice3`))

(fn `UserConstructionScript`
  (`parent.UserConstructionScript`))