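; Dialogue Blueprint for Albert on night 1, filling the parent character's lines and branching choices at BeginPlay.
; Choice overrides gate later options and set GameInstance knowledge flags, with Choice1 and Choice2 deliberately calling each other's parent logic.
; The first choice display unlocks the medical office and resets the post office and police main characters' child actor classes.
; Talking advances journal objectives, and one branch displays a garage photo.
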(event `/Game/Blueprint/Interfaces/BPI_TalkToChara.StartTalkingToChara`
  (`parent.StartTalkingToChara`)
  (`/Engine/EditorBlueprintResources/StandardMacros.DoOnce` false
    (:`Completed`
      (`/Game/Blueprint/Widget/WB_Journal.ValidateObjectif` (`self.JournalRef`) 6))))

(event `self.ReceiveBeginPlay`
  (set `self.DialogueChara1` (`self.DialogueAlbert1`))
  (set `self.DialogueChoiceChara1` (`self.DialogueChoiceAlbert1`))
  (set `self.DialogueChoiceChara2` (`self.DialogueChoiceAlbert2`))
  (set `self.DialogueChoiceChara3` (`self.DialogueChoiceAlbert3`))
  (set `self.DialogueChoiceCharaEnd` (`self.DialogueChoiceAlbertEnd`))
  (set `self.LineChoiceChara1` (`self.LineChoiceAlbert1`))
  (set `self.LineChoiceChara2` (`self.LineChoiceAlbert2`))
  (set `self.LineChoiceChara3` (`self.LineChoiceAlbert3`))
  (set `self.DialogueChoiceChara1-1` (`self.DialogueChoiceAlbert1-1`))
  (set `self.DialogueChoiceChara1-2` (`self.DialogueChoiceAlbert1-2`))
  (set `self.DialogueChoiceChara1-3` (`self.DialogueChoiceAlbert1-3`))
  (set `self.LineChoiceChara1-1` (`self.DialogueIndisponible`))
  (set `self.LineChoiceChara1-2` (`self.LineChoiceAlbert1-2`))
  (set `self.LineChoiceChara1-3` (`self.LineChoiceAlbert1-3`))
  (`parent.ReceiveBeginPlay`)
  (set `self.CharaName` "Albert")
  (if (not (or (`self.isChoice3Available`) (`self.isChoice1-3Available`)))
    (set `self.NumberOfChoices` 2)))

(event `self.ShowChoices`
  (bind _imagedialogue (`/Game/Blueprint/Widget/Dialogue/WB_DialogueTest.ImageDialogue` (`self.UI`)))
  (`parent.ShowChoices`)
  (`|ExecutionSequence`
    (:`then_0`
      (`/Engine/EditorBlueprintResources/StandardMacros.DoOnce` false
        (:`Completed`
          (for _array_element (`/Game/Blueprint/GameSystem/GI_Havencrest.BatimentsRef` (`self.GameInstanceRef`))
            (if (`/Game/Assets/DecorsAsset/Batiments/BP_Batiments_Parent.isCabMed` _array_element)
              (set `/Game/Assets/DecorsAsset/Batiments/BP_Batiments_Parent.isUnlocked` true _array_element)
              (elif (`/Game/Assets/DecorsAsset/Batiments/BP_Batiments_Parent.isLaPoste` _array_element)
                (`ChildActorComponent.SetChildActorClass` (`/Game/Assets/DecorsAsset/Batiments/BP_Batiments_Parent.PersoPrincipal` _array_element) null :!label _label)
                (elif (`/Game/Assets/DecorsAsset/Batiments/BP_Batiments_Parent.isPolice` _array_element)
                  (goto _label))))))))
    (:`then_1`
      (if (not (`self.canPassDialogue`))
        (`Widget.SetVisibility` (`/Game/Blueprint/Widget/Dialogue/WB_Choice.BTN_ChoiceEnd` (`self.UIchoice`)) "Hidden"))
      (if (`self.HasMadeImportantChoice1`)
        (if (not (`self.isChoice1-2Available`))
          (`Widget.SetIsEnabled` (`/Game/Blueprint/Widget/Dialogue/WB_Choice.BTN_Choice1` (`self.UIchoice`)) false)
          (set `self.NumberOfChoices` 2))
        (if (`self.isChoice1-3Available`)
          (`Widget.SetVisibility` (`/Game/Blueprint/Widget/Dialogue/WB_Choice.BTN_Choice3` (`self.UIchoice`)) "Visible"))
        (elif (not (`self.isChoice3Available`))
          (`Widget.SetVisibility` (`/Game/Blueprint/Widget/Dialogue/WB_Choice.BTN_Choice3` (`self.UIchoice`)) "Hidden")
          (set `self.NumberOfChoices` 2))))
    (:`then_2`
      (if (`Widget.IsVisible` _imagedialogue)
        (`Widget.SetVisibility` _imagedialogue "Hidden")))))

(event `self.EndEvent`
  (`/Game/Blueprint/Widget/WB_Journal.NextObjectif` (`self.JournalRef`) 7))

(event `/Game/Blueprint/Interfaces/BPI_DialogueChoice.Choice2`
  (bind _imagedialogue (`/Game/Blueprint/Widget/Dialogue/WB_DialogueTest.ImageDialogue` (`self.UI`)))
  ;[1 1 1] C'est volontaire que les choix 1 et 2 récupèrent le code de leur parent de l'autre choix (en gros le choix 1 a le code du choix 2 du père et inversement
  (if (`self.HasMadeImportantChoice1`)
    (`Widget.SetVisibility` (`/Game/Blueprint/Widget/Dialogue/WB_Choice.BTN_ChoiceEnd` (`self.UIchoice`)) "Visible")
    (set `self.canPassDialogue` true)
    (else
      (`Image.SetBrushFromTexture` _imagedialogue "/Game/Assets/DecorsAsset/Batiments/Garage/Garage_Photo.Garage_Photo" false)
      (`Widget.SetVisibility` _imagedialogue "Visible")
      (set `/Game/Blueprint/GameSystem/GI_Havencrest.EthanKnowsPierre` true (`self.GameInstanceRef`))))
  (`parent.Choice1`))

(event `/Game/Blueprint/Interfaces/BPI_DialogueChoice.Choice1`
  ;[1 1 1] C'est volontaire que les choix 1 et 2 récupèrent le code de leur parent de l'autre choix (en gros le choix 1 a le code du choix 2 du père et inversement
  (`parent.Choice2`)
  (if (not (`self.HasMadeImportantChoice1`))
    (set `self.LineChoiceChara1-1` (`self.LineChoiceAlbert1-1`))
    (set `self.isChoice1-2Available` true)))

(event `/Game/Blueprint/Interfaces/BPI_DialogueChoice.Choice3`
  (if (`self.HasMadeImportantChoice1`)
    (set `self.isChoice3Available` false)
    (set `/Game/Blueprint/GameSystem/GI_Havencrest.EthanKnowsCroissandra` true (`self.GameInstanceRef`)))
  (`parent.Choice3`))

(event `/Game/Blueprint/Interfaces/BPI_DialogueChoice.ChoiceEnd`
  (`parent.ChoiceEnd`)
  (set `/Game/Blueprint/GameSystem/GI_Havencrest.HasTalkToAlbert` true (`self.GameInstanceRef`)))

(fn `UserConstructionScript`
  (`parent.UserConstructionScript`))