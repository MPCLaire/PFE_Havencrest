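; Dialogue NPC Laetricia ("Attente" variant), a child Blueprint that loads her lines and three choices into the parent's dialogue system.
; ActivateLongDialogue switches to the long choice dialogue, which hides the end-choice button.
; Choices 1 and 2 load second-stage lines, while choice 3 changes BP_MarieNuit1's dialogue and disables box enlargement.
; Tick enlarges the dialogue box at a set line index after a delay and countdown, and the following line restores it.
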(event `self.ReceiveBeginPlay`
  (set `self.BaseDialogue` (`self.DialogueLaetriciaAttenteStart`))
  (set `self.DialogueChoice1` (`self.DialogueChoice1LaetriciaAttente`))
  (set `self.DialogueChoice2` (`self.DialogueChoice2LaetriciaAttente`))
  (set `self.DialogueChoice3` (`self.DialogueChoice3LaetriciaAttente`))
  (set `self.DialogueChoiceEnd` (`self.DialogueChoiceEndLaetriciaAttente`))
  (set `self.LineChoice1` (`self.LineChoice1LaetriciaAttente`))
  (set `self.LineChoice2` (`self.LineChoice2LaetriciaAttente`))
  (set `self.LineChoice3` (`self.LineChoice3LaetriciaAttente`))
  (set `self.CharaName` "Laetricia")
  (set `self.NumberOfChoices` 3)
  (set `self.isChoiceChara` false)
  (`parent.ReceiveBeginPlay`))

(event `/Game/Blueprint/Interfaces/BPI_DialogueChoice.Choice1`
  (`parent.Choice1`)
  (set `self.LineChoice1` (`self.SecondLineChoice1LaetriciaAttente`) :!label _label)
  (set `self.LineChoice2` (`self.SecondLineChoice2LaetriciaAttente`))
  (set `self.LineChoice3` (`self.SecondLineChoice3LaetriciaAttente`))
  (set `self.StartAgrandissement` 3))

(event `/Game/Blueprint/Interfaces/BPI_DialogueChoice.Choice2`
  (`parent.Choice2`)
  (goto _label))

(event `/Game/Blueprint/Interfaces/BPI_DialogueChoice.Choice3`
  (bind _returnvalue (`GameplayStatics.GetActorOfClass` "/Game/Blueprint/Characters/BP_MarieNuit1.BP_MarieNuit1_C"))
  (`self.ChangeDialogue` _returnvalue)
  (`parent.Choice3`)
  (set `self.NumberOfChoices` (`self.ChoicesMade`))
  (set `self.willGetBigger` false))

(event `self.ShowChoices`
  (`parent.ShowChoices`)
  (if (`self.isChoiceChara`)
    (`Widget.SetVisibility` (`/Game/Blueprint/Widget/Dialogue/WB_Choice.BTN_ChoiceEnd` (`self.UIchoice`)) "Hidden")))

(event `self.ReceiveTick`
  (params (DeltaSeconds :type "Float (single-precision)"))
  (bind _waitingtimer (`self.WaitingTimer`))
  ;[1 1 1] Lance l'agrandissement de la box
  (if (and (== (`self.dialogueIndex`) (`self.StartAgrandissement`)) (`self.isNpcTalking`) (`self.willGetBigger`))
    (`KismetSystemLibrary.Delay` 0.74)
    (if (<= _waitingtimer 0)
      (`|ExecutionSequence`
        (:`then_0`
          (set `self.WaitingTimer` (- _waitingtimer 1) :!label _label_2))
        (:`then_1`
          (if (not (== (`self.WaitingTimer`) -17))
            (`/Game/Blueprint/Widget/Dialogue/WB_DialogueTest.ResizeBox` (`self.UI`)))))
      (else
        (goto _label_2)))))

(event `/Game/Blueprint/Interfaces/BPI_TalkToChara.StartTalkingToChara`
  (`parent.StartTalkingToChara`)
  (if (== (`self.dialogueIndex`) (+ (`self.StartAgrandissement`) 1))
    (`/Game/Blueprint/Widget/Dialogue/WB_DialogueTest.ResizeToOrigin` (`self.UI`))
    (set `self.WaitingTimer` 3)))

(event `ActivateLongDialogue`
  (set `self.Dialogue` (`self.DialogueLaetriciaAttente`))
  (set `self.isChoiceChara` true)
  (set `self.HasChoice` true))

(fn `UserConstructionScript`
  (`parent.UserConstructionScript`))