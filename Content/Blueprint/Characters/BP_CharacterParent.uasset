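; Parent Blueprint for talkable NPCs, running their dialogue with the player, Ethan, who gets an E prompt inside the capsule.
; A looping timer types out Dialogue map keys (values name speakers), appending rich-text tags whole; talking again speeds it up.
; Speakers set the name, portrait dimming and voice sound.
; Choice characters offer three branches via WB_Choice, switching to an ending dialogue once ChoicesMade reaches NumberOfChoices; finishing resets the conversation.
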(event `self.ReceiveBeginPlay`
  (set `self.Dialogue` (`self.BaseDialogue`))
  (if (not (`self.isChoiceChara`))
    (set `self.HasChoice` false))
  (bind _asgi_havencrest (cast `/Game/Blueprint/GameSystem/GI_Havencrest` (`GameplayStatics.GetGameInstance`)))
  (set `self.GameInstanceRef` _asgi_havencrest)
  (bind _asbp_ethan (cast `/Game/Blueprint/MainCharacter/Blueprints/BP_Ethan` (`GameplayStatics.GetPlayerCharacter` 0)))
  (set `self.EthanRef` _asbp_ethan)
  (set `self.TextTime` 0.01)
  (`PrimitiveComponent.SetCastShadow` (`self.E_perso`) false)
  (`KismetSystemLibrary.Delay` 0.5)
  (bind _foundwidgets (`WidgetBlueprintLibrary.GetAllWidgetsOfClass` "/Game/Blueprint/Widget/WB_Journal.WB_Journal_C"))
  (set `self.JournalRef` (`|GetArrayItem` _foundwidgets)))

(event `Talk`
  (`|ExecutionSequence`
    (:`then_0`
      ;[1 1 1] Code pour que les dialogues spéciaux s'affichent normalement
      (`/Engine/EditorBlueprintResources/StandardMacros.DoOnce` false :!label _label
        (:`Completed`
          (`self.MakeTalkSounds`))))
    (:`then_1`
      (bind _keys (`BlueprintMapLibrary.Map_Keys` (`self.Dialogue`)))
      (bind _returnvalue (`KismetStringLibrary.GetCharacterArrayFromString` (`|GetArrayItem` _keys (`self.dialogueIndex`))))
      (bind _output (`|GetArrayItem` _returnvalue (`self.CharaIndex`)))
      (if (`KismetStringLibrary.EqualEqual_StrStr` _output "<")
        (while (`KismetStringLibrary.NotEqual_StrStr` _output ">") :!label _label_2
          (bind _returnvalue_2 (`KismetStringLibrary.Concat_StrStr` (`self.Letters`) _output))
          (set `self.Letters` _returnvalue_2)
          (`/Engine/EditorBlueprintResources/StandardMacros.IncrementInt` (`self.CharaIndex`)))
        (set `self.Letters` _returnvalue_2)
        (`/Engine/EditorBlueprintResources/StandardMacros.IncrementInt` (`self.CharaIndex`)
          (:`  `
            (if (`KismetStringLibrary.EqualEqual_StrStr` (`|GetArrayItem` _returnvalue (- (`self.CharaIndex`) 2)) "/")
              _
              (else
                (goto _label_2))))))
      ;[1 1 1] Ajoute le texte lettre par lettre
      (`self.UI`
        (:`then`
          _)
        (:`else`
          (bind _returnvalue_3 (`|CreateWidget` "/Game/Blueprint/Widget/Dialogue/WB_DialogueTest.WB_DialogueTest_C" (`GameplayStatics.GetPlayerController` 0)))
          (bind _output_get (set `self.UI` _returnvalue_3))
          (`UserWidget.AddToViewport` _output_get 0)
          (`self.ChooseName`)))
      (bind _line (`self.SelectLine`))
      (`RichTextBlock.SetText` (`/Game/Blueprint/Widget/Dialogue/WB_DialogueTest.RichTextBlock_0` (`self.UI`)) _line)
      ;[1 1 1] Reset pour le prochain dialogue
      (bind _islineended (`self.VerifyEndOfLine`))
      (if _islineended
        (`/Engine/EditorBlueprintResources/StandardMacros.IncrementInt` (`self.dialogueIndex`)
          (:`  `
            (set `self.CharaIndex` 0)
            (set `self.isNpcTalking` false)
            (set `self.Letters` "")
            (`KismetSystemLibrary.K2_ClearAndInvalidateTimerHandle` (stale `/Game/Blueprint/Interfaces/BPI_TalkToChara.StartDialogueAfterChoice` _returnvalue))
            (`KismetSystemLibrary.PrintString` "fini" true true (struct :`R` 0.149375 :`G` 1.0 :`A` 1.0))
            (set `self.TextTime` 0.01)
            (set `self.hasAlreadyDeactivate` false)
            (`|ExecutionSequence`
              (:`then_0`
                (goto _label :!via `Reset`))
              (:`then_1`
                (`KismetSystemLibrary.Delay` 1.0)
                (if (not (`self.hasAlreadyDeactivate`))
                  (`ActorComponent.Deactivate` (`self.Voice`))
                  (set `self.hasAlreadyDeactivate` true))))))))))

(event `/Game/Blueprint/Interfaces/BPI_TalkToChara.StartDialogueAfterChoice`
  ;[1 1 1] Lance le premier dialogue après un choix
  (if (`self.justMadeAChoice`)
    (set `self.justMadeAChoice` false)
    ;[1 1 1] Choisi la ligne de dialogue s'il y en a une.
    (bind _returnvalue (`KismetSystemLibrary.K2_SetTimerDelegate` (delegate `Talk`) (/ (`self.TextTime`) 1.0) true :!label _label_3))))

(event `StartTalking`
  ;[1 1 1] Quand on appuie sur E, ça démarre le dialogue
)

(event `/Game/Blueprint/Interfaces/BPI_TalkToChara.StartTalkingToChara`
  (bind _uichoice (`self.UIchoice`))
  ;[1 1 1] Quand on appuie sur E, ça démarre le dialogue
  (`SceneComponent.SetVisibility` (`self.PaperFlipbook`) false false)
  (`SceneComponent.SetVisibility` (`PaperCharacter.Sprite` (`self.EthanRef`)) false false)
  (`SceneComponent.SetVisibility` (`self.E_perso`) false false)
  ;[1 1 1] Choisi la ligne de dialogue s'il y en a une.
  (if (`self.isNpcTalking`)
    ;[1 1 1] Skip dialogue
    (if (not (== (`GameplayStatics.GetObjectClass` self) "/Game/Blueprint/Characters/BP_LaetriciaAttente.BP_LaetriciaAttente_C"))
      (`/Engine/EditorBlueprintResources/StandardMacros.IsValid` _uichoice
        (:`Is Valid`
          (if (not (`Widget.IsInViewport` _uichoice))
            (set `self.TextTime` 0.0001 :!label _label_4)
            (`self.SkipDialogue`)))
        (:`Is Not Valid`
          (goto _label_4))))
    (else
      (`|ExecutionSequence`
        (:`then_0`
          (if (not (`self.hasAlreadyDeactivate`))
            (`ActorComponent.Deactivate` (`self.Voice`))
            (set `self.hasAlreadyDeactivate` true)))
        (:`then_1`
          (set `self.isNpcTalking` true)
          (if (< (`self.dialogueIndex`) (`BlueprintMapLibrary.Map_Length` (`self.Dialogue`)))
            (set `/Game/Blueprint/MainCharacter/Blueprints/BP_Ethan.CantMove?` true (`self.EthanRef`))
            (`self.ChooseName`)
            (goto _label_3)
            (else
              (`self.ShowChoices`))))))))

(event `self.Capsule.OnComponentBeginOverlap`
  (params (OverlappedComponent :type "PrimitiveComponent Object Reference") (OtherActor :type "Actor Object Reference") (OtherComp :type "PrimitiveComponent Object Reference") (OtherBodyIndex :type Integer) (bFromSweep :type Boolean) (SweepResult :type "HitResult Structure (by ref)"))
  ;[1 1 1] Quand on appuie sur E, ça démarre le dialogue
  (if (== OtherActor (`self.EthanRef`))
    (message `/Game/Blueprint/Interfaces/BPI_TalkToChara.CanTalk` OtherActor self)
    (`SceneComponent.SetVisibility` (`self.E_perso`) true false)))

(event `SkipDialogue`
  ;[1 1 1] Choisi la ligne de dialogue s'il y en a une.
  (goto _label_3))

(event `self.Capsule.OnComponentEndOverlap`
  (params (OverlappedComponent :type "PrimitiveComponent Object Reference") (OtherActor :type "Actor Object Reference") (OtherComp :type "PrimitiveComponent Object Reference") (OtherBodyIndex :type Integer))
  ;[1 1 1] Faire en sorte que le dialogue ne se lance pas si on quitte la capsule collision
  (if (== OtherActor (`self.EthanRef`))
    (message `/Game/Blueprint/Interfaces/BPI_TalkToChara.Can'tTalk` OtherActor)
    (`SceneComponent.SetVisibility` (`self.E_perso`) false false)))

(event `ShowChoices`
  (bind _returnvalue (`GameplayStatics.GetPlayerController` 0))
  ;[1 1 1] Affiche les choix
  (if (`self.HasChoice`)
    (if (== (`self.ChoicesMade`) (`self.NumberOfChoices`))
      (`self.ChoiceEnd`)
      (else
        (`RichTextBlock.SetText` (`/Game/Blueprint/Widget/Dialogue/WB_DialogueTest.RichTextBlock_0` (`self.UI`)) (`self.Empty`))
        (bind _returnvalue_2 (`|CreateWidget` "/Game/Blueprint/Widget/Dialogue/WB_Choice.WB_Choice_C"))
        (bind _output_get (set `self.UIchoice` _returnvalue_2))
        (`UserWidget.AddToViewport` _output_get 0)
        (set `/Game/Blueprint/Widget/Dialogue/WB_Choice.CharaRef` self _output_get)
        (`self.SetLinesChoice` _output_get)
        (set `self.Letters` "")
        (set `self.willMakeAChoice` true)
        (set `PlayerController.bShowMouseCursor` true _returnvalue)
        (`WidgetBlueprintLibrary.SetInputMode_GameAndUIEx` _returnvalue null)
        (`self.ChooseName`)))
    (else
      ;[1 1 1] Met fin au dialogue. Reset certaines variables pour pouvoir répéter le dialogue.
      (set `/Game/Blueprint/MainCharacter/Blueprints/BP_Ethan.CantMove?` false (`self.EthanRef`))
      (`Widget.RemoveFromParent` (`self.UI`))
      (set `self.dialogueIndex` 0)
      (set `self.UI` null)
      (if (`self.isChoiceChara`)
        ;[0 0.2549 1] Variables à reset que pour le choix
        (set `PlayerController.bShowMouseCursor` false _returnvalue)
        (`WidgetBlueprintLibrary.SetInputMode_GameOnly` _returnvalue)
        (set `self.HasChoice` true)
        (set `self.ChoicesMade` 0)
        (set `self.isChoice1Made` false)
        (set `self.isChoice2Made` false)
        (set `self.isChoice3Made` false))
      (`KismetSystemLibrary.Delay` 0.0)
      (set `self.Dialogue` (`self.BaseDialogue`))
      (set `self.isNpcTalking` false)
      (set `/Game/Blueprint/MainCharacter/Blueprints/BP_Ethan.EPressed` false (`self.EthanRef`))
      (`SceneComponent.SetVisibility` (`self.PaperFlipbook`) true false)
      (`SceneComponent.SetVisibility` (`PaperCharacter.Sprite` (`self.EthanRef`)) true false)
      (`SceneComponent.SetVisibility` (`self.E_perso`) true false)
      (`/Game/Blueprint/MainCharacter/Blueprints/BP_Ethan.TimeToE` (`self.EthanRef`))
      (set `PlayerController.bShowMouseCursor` false (`GameplayStatics.GetPlayerController` 0))
      (`self.EndEvent`)
      (set `self.secondeTime?` true))))

(event `EndEvent`)

(event `/Game/Blueprint/Interfaces/BPI_DialogueChoice.Choice1`
  ;[0 0.2549 1] Si on appuie sur le premier choix
  (if (not (`self.isChoice1Made`))
    (`/Engine/EditorBlueprintResources/StandardMacros.IncrementInt` (`self.ChoicesMade`)
      (:`  `
        (set `self.isChoice1Made` true))))
  (set `self.justMadeAChoice` true)
  (set `self.willMakeAChoice` false)
  (`Widget.RemoveFromParent` (`self.UIchoice`))
  (set `self.Dialogue` (`self.DialogueChoice1`))
  (set `self.dialogueIndex` 0)
  (set `self.CharaIndex` 0)
  (`self.ChooseName`)
  (`self.StartDialogueAfterChoice`))

(event `/Game/Blueprint/Interfaces/BPI_DialogueChoice.Choice2`
  ;[0 0.2549 1] Si on appuie sur le deuxième choix
  (if (not (`self.isChoice2Made`))
    (`/Engine/EditorBlueprintResources/StandardMacros.IncrementInt` (`self.ChoicesMade`)
      (:`  `
        (set `self.isChoice2Made` true))))
  (set `self.justMadeAChoice` true)
  (set `self.willMakeAChoice` false)
  (`Widget.RemoveFromParent` (`self.UIchoice`))
  (set `self.Dialogue` (`self.DialogueChoice2`))
  (set `self.dialogueIndex` 0)
  (set `self.CharaIndex` 0)
  (`self.ChooseName`)
  (`self.StartDialogueAfterChoice`))

(event `/Game/Blueprint/Interfaces/BPI_DialogueChoice.Choice3`
  ;[0 0.2549 1] Si on appuie sur le troisième choix
  (if (not (`self.isChoice3Made`))
    (`/Engine/EditorBlueprintResources/StandardMacros.IncrementInt` (`self.ChoicesMade`)
      (:`  `
        (set `self.isChoice3Made` true))))
  (set `self.justMadeAChoice` true)
  (set `self.willMakeAChoice` false)
  (`Widget.RemoveFromParent` (`self.UIchoice`))
  (set `self.Dialogue` (`self.DialogueChoice3`))
  (set `self.dialogueIndex` 0)
  (set `self.CharaIndex` 0)
  (`self.ChooseName`)
  (`self.StartDialogueAfterChoice`))

(event `/Game/Blueprint/Interfaces/BPI_DialogueChoice.ChoiceEnd`
  ;[0 0.2549 1] Si on met fin au choix
  (set `self.justMadeAChoice` true)
  (set `self.willMakeAChoice` false)
  (`Widget.RemoveFromParent` (`self.UIchoice`))
  (set `self.Dialogue` (`self.DialogueChoiceEnd`))
  (set `self.dialogueIndex` 0)
  (set `self.CharaIndex` 0)
  (`self.ChooseName`)
  (`self.Talk`)
  (set `self.HasChoice` false)
  (set `self.ChoicesMade` 0)
  (`self.StartDialogueAfterChoice`))

(fn `ChooseName`
  ;[1 1 1] Faire apparaitre le nom haut à gauche de la box de dialogue
  (bind _ui (`self.UI`)
    (:`then`
      (if (`self.willMakeAChoice`)
        (`TextBlock.SetText` (`/Game/Blueprint/Widget/Dialogue/WB_DialogueTest.Name` _ui) "")
        (`self.LightOffTheOneWhoDontTalk` "")
        (else
          (`self.SetWhoAppears`)
          (bind _keys (`BlueprintMapLibrary.Map_Keys` (`self.Dialogue`)))
          (bind _value (`BlueprintMapLibrary.Map_Find` (`self.Dialogue`) (`|GetArrayItem` _keys (`self.dialogueIndex`))))
          (`TextBlock.SetText` (`/Game/Blueprint/Widget/Dialogue/WB_DialogueTest.Name` (`self.UI`)) (`KismetTextLibrary.Conv_StringToText` _value))
          (`self.LightOffTheOneWhoDontTalk` _value))))
    (:`else`)))

(fn `LightOffTheOneWhoDontTalk`
  (params (Name :type String))
  (bind _ui (`self.UI`))
  (bind _ethan (`/Game/Blueprint/Widget/Dialogue/WB_DialogueTest.Ethan` _ui))
  (bind _chara (`/Game/Blueprint/Widget/Dialogue/WB_DialogueTest.Chara` _ui))
  ;[1 1 1] Si c'est Ethan qui parle ou qui fait un choix, il apparait en clair et l'autre personne est grisé
  (if (or (`KismetStringLibrary.EqualEqual_StrStr` Name "Ethan") (`KismetStringLibrary.EqualEqual_StrStr` Name))
    (`Image.SetColorAndOpacity` _ethan (struct :`R` 1.0 :`G` 1.0 :`B` 1.0 :`A` 1.0))
    (`Image.SetColorAndOpacity` _chara (struct :`R` 0.1 :`G` 0.1 :`B` 0.1 :`A` 1.0))
    (else
      ;[1 1 1] Si c'est pas Ethan qui parle ou qui fait un choix, il est grisé et l'autre personne apparait en clair
      (if (`KismetStringLibrary.EqualEqual_StrStr` Name "Jean")
        (set `self.isJeanFR` true)
        (`Image.SetBrushFromTexture` (`/Game/Blueprint/Widget/Dialogue/WB_DialogueTest.Chara` (`self.UI`)) "/Game/Image/ImageDialogue/ImageFinale/IMG_JeanDialogue2.IMG_JeanDialogue2" false)
        (else
          (`self.SetWhoAppears`)))
      (`Image.SetColorAndOpacity` _ethan (struct :`R` 0.1 :`G` 0.1 :`B` 0.1 :`A` 1.0))
      (`Image.SetColorAndOpacity` _chara (struct :`R` 1.0 :`G` 1.0 :`B` 1.0 :`A` 1.0)))))

(fn `MakeTalkSounds`
  (`KismetSystemLibrary.PrintString` "Start")
  (bind _keys (`BlueprintMapLibrary.Map_Keys` (`self.Dialogue`)))
  (switch `string` (`BlueprintMapLibrary.Map_Find` (`self.Dialogue`) (`|GetArrayItem` _keys (`self.dialogueIndex`)))
    (:`Ethan`
      (`AudioComponent.SetSound` (`self.Voice`) "/Game/Sounds/Talk/SC_EthanTalk.SC_EthanTalk"))
    (:`Pierre`
      (`AudioComponent.SetSound` (`self.Voice`) "/Game/Sounds/Talk/SC_PierreTalk.SC_PierreTalk"))
    (:`Michel`
      (`AudioComponent.SetSound` (`self.Voice`) "/Game/Sounds/Talk/SC_MichelTalk.SC_MichelTalk"))
    (:`Marie`
      (`AudioComponent.SetSound` (`self.Voice`) "/Game/Sounds/Talk/SC_MarieTalk.SC_MarieTalk"))
    (:`Albert`
      (`AudioComponent.SetSound` (`self.Voice`) "/Game/Sounds/Talk/SC_AlbertTalk.SC_AlbertTalk"))
    (:`Laetricia`
      (`AudioComponent.SetSound` (`self.Voice`) "/Game/Sounds/Talk/SC_LaetriciaTalk.SC_LaetriciaTalk"))
    (:`Jean`
      (`AudioComponent.SetSound` (`self.Voice`) "/Game/Sounds/Talk/SC_JeanTalk.SC_JeanTalk"))
    (:`Serpent le serpent`
      (`AudioComponent.SetSound` (`self.Voice`) "/Game/Sounds/Serpent/SC_SerpentLeSon.SC_SerpentLeSon")))
  (`ActorComponent.Activate` (`self.Voice`) true))

(fn `SelectLine`
  (returns (Line :type Text))
  ;[1 1 1] Choisi la ligne de dialogue et la fait apparaitre letres par lettres
  (bind _keys (`BlueprintMapLibrary.Map_Keys` (`self.Dialogue`)))
  (bind _output_get (set `self.Letters` (`KismetStringLibrary.Concat_StrStr` (`self.Letters`) (`|GetArrayItem` (`KismetStringLibrary.GetCharacterArrayFromString` (`|GetArrayItem` _keys (`self.dialogueIndex`))) (`self.CharaIndex`)))))
  (return (`KismetTextLibrary.Conv_StringToText` _output_get)))

(fn `SetWhoAppears`
  (if (not (`self.isJeanFR`))
    ;[1 1 1] Vérifie qui parle et lui associe une image
    (`/Engine/EditorBlueprintResources/StandardMacros.DoOnce` false
      (:`Completed`
        _)))
  (switch `string` (`self.CharaName`)
    (:`Pierre`
      (`Image.SetBrushFromTexture` (`/Game/Blueprint/Widget/Dialogue/WB_DialogueTest.Chara` (`self.UI`)) "/Game/Image/ImageDialogue/ImageFinale/IMG_PierreDialogue.IMG_PierreDialogue" false))
    (:`Michel`
      (`Image.SetBrushFromTexture` (`/Game/Blueprint/Widget/Dialogue/WB_DialogueTest.Chara` (`self.UI`)) "/Game/Assets/Characters/Sprites/Sprite/Michel/Michel_Standing4.Michel_Standing4" false))
    (:`Marie`
      (`Image.SetBrushFromTexture` (`/Game/Blueprint/Widget/Dialogue/WB_DialogueTest.Chara` (`self.UI`)) "/Game/Image/ImageDialogue/ImageFinale/IMG_MarieDialogue.IMG_MarieDialogue" false))
    (:`Albert`
      (`Image.SetBrushFromTexture` (`/Game/Blueprint/Widget/Dialogue/WB_DialogueTest.Chara` (`self.UI`)) "/Game/Image/ImageDialogue/ImageFinale/IMG_AlbertDialogue2.IMG_AlbertDialogue2" false))
    (:`Laetricia`
      (`Image.SetBrushFromTexture` (`/Game/Blueprint/Widget/Dialogue/WB_DialogueTest.Chara` (`self.UI`)) "/Game/Image/ImageDialogue/ImageFinale/IMG_LaetriciaDialogue.IMG_LaetriciaDialogue" false))
    (:`Jean`
      (`Image.SetBrushFromTexture` (`/Game/Blueprint/Widget/Dialogue/WB_DialogueTest.Chara` (`self.UI`)) "/Game/Image/ImageDialogue/ImageFinale/IMG_JeanDialogue2.IMG_JeanDialogue2" false))
    (:`Jean-Francois`
      (`Image.SetBrushFromTexture` (`/Game/Blueprint/Widget/Dialogue/WB_DialogueTest.Chara` (`self.UI`)) "/Game/Assets/Characters/Sprites/Sprite/Jean-Francois/Jean-Francois.Jean-Francois" false))
    (:`Jeanne-Claude`
      (`Image.SetBrushFromTexture` (`/Game/Blueprint/Widget/Dialogue/WB_DialogueTest.Chara` (`self.UI`)) "/Game/Materials/Texture/Bouche_d_incendie-removebg-preview.Bouche_d_incendie-removebg-preview" false))
    (:`Jean-Driss`
      (`Image.SetBrushFromTexture` (`/Game/Blueprint/Widget/Dialogue/WB_DialogueTest.Chara` (`self.UI`)) "/Game/Image/PlaceHolderDialogue/IMG_PH_JeanDialogue.IMG_PH_JeanDialogue" false))
    (:`Emma`
      (`Image.SetBrushFromTexture` (`/Game/Blueprint/Widget/Dialogue/WB_DialogueTest.Chara` (`self.UI`)) "/Game/Image/PlaceHolderDialogue/IMG_PH_EmmaDialogue.IMG_PH_EmmaDialogue" false))
    (:`Croissandra`
      (`Image.SetBrushFromTexture` (`/Game/Blueprint/Widget/Dialogue/WB_DialogueTest.Chara` (`self.UI`)) "/Game/Image/PlaceHolderDialogue/IMG_PH_EmmaDialogue.IMG_PH_EmmaDialogue" false))
    (:`Serpent le serpent`
      (`Image.SetBrushFromTexture` (`/Game/Blueprint/Widget/Dialogue/WB_DialogueTest.Chara` (`self.UI`)) "/Game/Assets/Characters/Sprites/Sprite/Serpent/SerpentLeSerpent.SerpentLeSerpent" false))
    (:`Larry`
      (`Image.SetBrushFromTexture` (`/Game/Blueprint/Widget/Dialogue/WB_DialogueTest.Chara` (`self.UI`)) "/Game/Materials/Texture/LarryleTriste.LarryleTriste" false))
    (:`LarryLeMalicieux`
      (`Image.SetBrushFromTexture` (`/Game/Blueprint/Widget/Dialogue/WB_DialogueTest.Chara` (`self.UI`)) "/Game/Materials/Texture/LarryLeMalicieux.LarryLeMalicieux" false))
    (:`Nochara`
      (`Image.SetBrushFromTexture` (`/Game/Blueprint/Widget/Dialogue/WB_DialogueTest.Chara` (`self.UI`)) "/Game/Image/Non.Non" false))))

(fn `StartConversation`
  (`self.StartTalkingToChara`))

(fn `UserConstructionScript`)

(fn `VerifyEndOfLine`
  (returns (isLineEnded :type Boolean))
  ;[1 1 1] Vérifie si il reste des caractères dans le ligne de dialogue
  (bind _keys (`BlueprintMapLibrary.Map_Keys` (`self.Dialogue`)))
  (bind _result (`/Engine/EditorBlueprintResources/StandardMacros.IncrementInt` (`self.CharaIndex`))
    (:`  `
      (return (== _result (`KismetArrayLibrary.Array_Length` (`KismetStringLibrary.GetCharacterArrayFromString` (`|GetArrayItem` _keys (`self.dialogueIndex`)))))))))