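; BP_EthanChateauDeau is a child character Blueprint for Ethan, apparently placed at Château d'Eau, that offers dialogue during one game state.
; On BeginPlay it sets its normal dialogue, non-choice flag and placeholder name before calling the parent, then destroys itself unless GameState matches the first enumerator.
; ShowChoices runs the parent logic, then removes the actor after a short delay.
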(event `self.ReceiveBeginPlay`
  (set `self.BaseDialogue` (`self.DialogueNormal`))
  (set `self.isChoiceChara` false)
  (set `self.CharaName` "Nochara")
  (`parent.ReceiveBeginPlay`)
  (if (not (`|EnumEquality` (`/Game/Blueprint/GameSystem/GI_Havencrest.GameState` (`self.GameInstanceRef`)) "NewEnumerator0"))
    (`self.K2_DestroyActor`)))

(event `self.ShowChoices`
  (`parent.ShowChoices`)
  (`KismetSystemLibrary.Delay` 1.0)
  (`self.K2_DestroyActor`))

(fn `UserConstructionScript`
  (`parent.UserConstructionScript`))