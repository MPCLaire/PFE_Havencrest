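; Dialogue actor for the Serpent character, extending a parent dialogue Blueprint with its own name and dialogue sets.
; Ethan entering the capsule halts BP_Serpent and can flag a question as asked; leaving restores walking and calls Wait.
; Showing choices marks the serpent as already spoken to and hides the flipbook, and that flag selects the next dialogue.
; Tick keeps rotation locked at zero.
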(event `self.ReceiveBeginPlay`
  (bind _returnvalue (`GameplayStatics.GetActorOfClass` "/Game/Blueprint/Characters/BP_Serpent.BP_Serpent_C"))
  (set `self.SerpentRef` _returnvalue)
  (set `self.BaseDialogue` (`self.DialogueSnake`))
  (`parent.ReceiveBeginPlay`)
  (set `self.CharaName` "Serpent le serpent"))

(event `self.Capsule.OnComponentBeginOverlap`
  (params (OverlappedComponent :type "PrimitiveComponent Object Reference") (OtherActor :type "Actor Object Reference") (OtherComp :type "PrimitiveComponent Object Reference") (OtherBodyIndex :type Integer) (bFromSweep :type Boolean) (SweepResult :type "HitResult Structure (by ref)"))
  (bind _serpentref (`self.SerpentRef`))
  (if (== (`self.EthanRef`) OtherActor)
    (set `/Game/Blueprint/Characters/BP_Serpent.CanMove` false _serpentref)
    (`CharacterMovementComponent.DisableMovement` (`Character.CharacterMovement` _serpentref))
    (if (`self.CanShowQuestion`)
      (set `self.HasAsked?` true))))

(event `self.Capsule.OnComponentEndOverlap`
  (params (OverlappedComponent :type "PrimitiveComponent Object Reference") (OtherActor :type "Actor Object Reference") (OtherComp :type "PrimitiveComponent Object Reference") (OtherBodyIndex :type Integer))
  (bind _serpentref (`self.SerpentRef`))
  (if (== (`self.EthanRef`) OtherActor)
    (set `/Game/Blueprint/Characters/BP_Serpent.CanMove` true _serpentref)
    (`CharacterMovementComponent.SetMovementMode` (`Character.CharacterMovement` (`self.SerpentRef`)) "MOVE_Walking" 0)
    (`/Game/Blueprint/Characters/BP_Serpent.Wait` _serpentref)))

(event `self.ShowChoices`
  (`parent.ShowChoices`)
  (`|ExecutionSequence`
    (:`then_0`
      (`/Engine/EditorBlueprintResources/StandardMacros.DoOnce` false
        (:`Completed`
          (set `self.DejaParlé?` true))))
    (:`then_1`
      (`KismetSystemLibrary.Delay` 0.0)
      (`SceneComponent.SetVisibility` (`self.PaperFlipbook`) false false))))

(event `self.ReceiveTick`
  (params (DeltaSeconds :type "Float (single-precision)"))
  (`self.K2_SetActorRotation` (struct)))

(fn `ChangeToNextDialogue`
  (if (`self.DejaParlé?`)
    (set `self.Dialogue` (`self.DialogueSnake2`))
    (else
      (set `self.Dialogue` (`self.DialogueSnakeAll`))))
  (`KismetSystemLibrary.PrintString` "JECHANGKJACGEHNAJEHND"))

(fn `UserConstructionScript`
  (`parent.UserConstructionScript`))