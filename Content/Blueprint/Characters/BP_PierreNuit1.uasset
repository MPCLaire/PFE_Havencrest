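; Dialogue character Blueprint for Pierre on night 1, a child class that fills in the parent's dialogue, choice lines and character name at BeginPlay.
; Showing choices swaps in an extended second dialogue when the game instance says Ethan knows Pierre, and hides the end-choice button.
; Picking the second choice flags Pierre's lie about MM in the game instance and displays a garage photo in the dialogue UI before running parent logic.
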(event `self.ReceiveBeginPlay`
  (set `self.BaseDialogue` (`self.DialoguePierreNuit1`))
  (set `self.DialogueChoice1` (`self.DialogueChoice1PierreNuit1`))
  (set `self.DialogueChoice2` (`self.DialogueChoice2PierreNuit1`))
  (set `self.DialogueChoice3` (`self.DialogueChoice3PierreNuit1`))
  (set `self.DialogueChoiceEnd` (`self.DialogueChoiceEndPierreNuit1`))
  (set `self.LineChoice1` (`self.LineChoicePierreNuit1`))
  (set `self.LineChoice2` (`self.LineChoicePierreNuit2`))
  (set `self.LineChoice3` (`self.LineChoicePierreNuit3`))
  (set `self.CharaName` "Pierre")
  (`parent.ReceiveBeginPlay`))

(event `self.ShowChoices`
  (if (`/Game/Blueprint/GameSystem/GI_Havencrest.EthanKnowsPierre` (`self.GameInstanceRef`))
    (set `self.DialogueChoice2` (`self.DialogueChoice2PlusPierreNuit1`)))
  (`parent.ShowChoices`)
  (`Widget.SetVisibility` (`/Game/Blueprint/Widget/Dialogue/WB_Choice.BTN_ChoiceEnd` (`self.UIchoice`)) "Hidden"))

(event `/Game/Blueprint/Interfaces/BPI_DialogueChoice.Choice2`
  (bind _imagedialogue (`/Game/Blueprint/Widget/Dialogue/WB_DialogueTest.ImageDialogue` (`self.UI`)))
  (set `/Game/Blueprint/GameSystem/GI_Havencrest.PierreLiesAboutM&M` true (`self.GameInstanceRef`))
  (`Image.SetBrushFromTexture` _imagedialogue "/Game/Assets/DecorsAsset/Batiments/Garage/Garage_Photo.Garage_Photo" false)
  (`Widget.SetVisibility` _imagedialogue "Visible")
  (`parent.Choice2`))

(fn `UserConstructionScript`
  (`parent.UserConstructionScript`))