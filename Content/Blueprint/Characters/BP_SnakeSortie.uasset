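; Dialogue character acting as the exit of the Snake minigame, winning it when the overlapping BP_Snake holds a key.
; Without the key, it starts its inherited dialogue as "Serpent" and pauses the snake's movement.
; A looping timer then polls Ethan's E press, clears itself, removes the dialogue widget and restarts the snake through PlayerSnakeRef.
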(event `self.ReceiveBeginPlay`
  (set `self.BaseDialogue` (`self.MessageSnake`))
  (set `self.CharaName` "Snake")
  (`parent.ReceiveBeginPlay`))

(event `self.Capsule.OnComponentBeginOverlap`
  (params (OverlappedComponent :type "PrimitiveComponent Object Reference") (OtherActor :type "Actor Object Reference") (OtherComp :type "PrimitiveComponent Object Reference") (OtherBodyIndex :type Integer) (bFromSweep :type Boolean) (SweepResult :type "HitResult Structure (by ref)"))
  (bind _asbp_snake (cast `/Game/Blueprint/Mini_Jeux/Snake/BP_Snake` OtherActor))
  (set `self.SnakeRef` _asbp_snake)
  (if (`/Game/Blueprint/Mini_Jeux/Snake/BP_Snake.HasKey` _asbp_snake)
    (`/Game/Blueprint/Mini_Jeux/Snake/BP_Snake.SnakeWin` (`self.SnakeRef`))
    (else
      (set `self.CharaName` "Serpent")
      (`self.StartTalkingToChara`)
      (set `/Game/Blueprint/Mini_Jeux/Snake/BP_Snake.Snaking?` false (`self.SnakeRef`))
      (bind _returnvalue (`KismetSystemLibrary.K2_SetTimerDelegate` (delegate `CheckE`) 0.1 true)))))

(event `CheckE`
  (if (`/Game/Blueprint/MainCharacter/Blueprints/BP_Ethan.EPressed` (`self.EthanRef`))
    (`KismetSystemLibrary.K2_ClearAndInvalidateTimerHandle` (stale `self.Capsule.OnComponentBeginOverlap` _returnvalue))
    (bind _foundwidgets (`WidgetBlueprintLibrary.GetAllWidgetsOfClass` "/Game/Blueprint/Widget/Dialogue/WB_DialogueTest.WB_DialogueTest_C"))
    (`Widget.RemoveFromParent` (`|GetArrayItem` _foundwidgets))
    (`/Game/Blueprint/Mini_Jeux/Snake/BP_PlayerSnake.StartSnake` (`self.PlayerSnakeRef`))))

(fn `UserConstructionScript`
  (`parent.UserConstructionScript`))