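; BP_BoxStopChateau is a trigger box that activates the player's "stop chateau" state while BP_Ethan is inside it.
; On BeginPlay it destroys itself unless the GI_Havencrest game state matches the first enumerator.
; Box overlaps call Ethan's activate and deactivate functions and show or hide a shadowless widget.
; Tick slides that widget along world X to follow Ethan's capsule, keeping its Y and Z.
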(event `self.ReceiveBeginPlay`
  (bind _asbp_ethan (cast `/Game/Blueprint/MainCharacter/Blueprints/BP_Ethan` (`GameplayStatics.GetPlayerCharacter` 0)))
  (set `self.As BP Ethan` _asbp_ethan)
  (`PrimitiveComponent.SetCastShadow` (`self.Widget`) false)
  (bind _asgi_havencrest (cast `/Game/Blueprint/GameSystem/GI_Havencrest` (`GameplayStatics.GetGameInstance`)))
  (bind _output_get (set `self.As GI Havencrest` _asgi_havencrest))
  (if (not (`|EnumEquality` (`/Game/Blueprint/GameSystem/GI_Havencrest.GameState` _output_get) "NewEnumerator0"))
    (`self.K2_DestroyActor`)))

(event `self.Box.OnComponentBeginOverlap`
  (params (OverlappedComponent :type "PrimitiveComponent Object Reference") (OtherActor :type "Actor Object Reference") (OtherComp :type "PrimitiveComponent Object Reference") (OtherBodyIndex :type Integer) (bFromSweep :type Boolean) (SweepResult :type "HitResult Structure (by ref)"))
  (bind _as_bp_ethan (`self.As BP Ethan`))
  (if (== OtherActor _as_bp_ethan)
    (`/Game/Blueprint/MainCharacter/Blueprints/BP_Ethan.ActivateStopChateau` _as_bp_ethan)
    (`SceneComponent.SetVisibility` (`self.Widget`) true false)))

(event `self.Box.OnComponentEndOverlap`
  (params (OverlappedComponent :type "PrimitiveComponent Object Reference") (OtherActor :type "Actor Object Reference") (OtherComp :type "PrimitiveComponent Object Reference") (OtherBodyIndex :type Integer))
  (bind _as_bp_ethan (`self.As BP Ethan`))
  (if (== OtherActor _as_bp_ethan)
    (`/Game/Blueprint/MainCharacter/Blueprints/BP_Ethan.DeactivateStopChateau` _as_bp_ethan)
    (`SceneComponent.SetVisibility` (`self.Widget`) false false)))

(event `self.ReceiveTick`
  (params (DeltaSeconds :type "Float (single-precision)"))
  (bind _widget (`self.Widget`))
  (bind (_returnvalue_x _returnvalue_y _returnvalue_z) (`KismetMathLibrary.BreakVector` (`SceneComponent.K2_GetComponentLocation` _widget)))
  (bind _returnvalue_x_2 (`KismetMathLibrary.BreakVector` (`SceneComponent.K2_GetComponentLocation` (`Character.CapsuleComponent` (`self.As BP Ethan`)))))
  (`SceneComponent.K2_SetWorldLocation` _widget (`KismetMathLibrary.MakeVector` _returnvalue_x_2 _returnvalue_y _returnvalue_z) false false))

(fn `UserConstructionScript`)