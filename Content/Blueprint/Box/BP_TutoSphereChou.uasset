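; BP_TutoSphereChou is a trigger actor that shows an item tutorial widget when the player character, Ethan, enters its sphere.
; On BeginPlay it caches the player as BP_Ethan, then on sphere overlap checks that actor and an IsTutoTAB flag.
; It creates WB_TutoItem, adds it to the viewport, hands the reference to Ethan and clears the flag so it fires only once.
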(event `self.ReceiveBeginPlay`
  (bind _asbp_ethan (cast `/Game/Blueprint/MainCharacter/Blueprints/BP_Ethan` (`GameplayStatics.GetPlayerCharacter` 0)))
  (set `self.EthanRef` _asbp_ethan))

(event `self.Sphere.OnComponentBeginOverlap`
  (params (OverlappedComponent :type "PrimitiveComponent Object Reference") (OtherActor :type "Actor Object Reference") (OtherComp :type "PrimitiveComponent Object Reference") (OtherBodyIndex :type Integer) (bFromSweep :type Boolean) (SweepResult :type "HitResult Structure (by ref)"))
  (if (and (== OtherActor (`self.EthanRef`)) (`self.isTutoTAB`))
    (bind _returnvalue (`|CreateWidget` "/Game/Blueprint/Widget/Tutorial/WB_TutoItem.WB_TutoItem_C"))
    (`UserWidget.AddToViewport` _returnvalue 0)
    (set `/Game/Blueprint/MainCharacter/Blueprints/BP_Ethan.WB_TutoItemRef` _returnvalue (`self.EthanRef`))
    (set `self.isTutoTAB` false)))

(fn `UserConstructionScript`)