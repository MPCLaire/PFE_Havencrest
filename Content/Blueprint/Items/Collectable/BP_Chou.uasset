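; BP_Chou is a collectable item Blueprint that only remains in the level during certain story states.
; On BeginPlay it runs the parent logic, then reads GameState from the GI_Havencrest game instance.
; It destroys itself in each of the listed states, from Start and Snake through later story beats such as Sortie Pierre MJ.
; It adds no other logic of its own.
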(event `self.ReceiveBeginPlay`
  (`parent.ReceiveBeginPlay`)
  (bind _asgi_havencrest (cast `/Game/Blueprint/GameSystem/GI_Havencrest` (`GameplayStatics.GetGameInstance`)))
  (switch `/Game/Blueprint/GameSystem/E_Instance` (`/Game/Blueprint/GameSystem/GI_Havencrest.GameState` _asgi_havencrest)
    (:`NewEnumerator0`
      _)
    (:`NewEnumerator1`
      _)
    (:`NewEnumerator3`
      _)
    (:`NewEnumerator4`
      _)
    (:`NewEnumerator8`
      _)
    (:`NewEnumerator7`
      _)
    (:`NewEnumerator5`
      _)
    (:`NewEnumerator2`
      _))
  (`self.K2_DestroyActor`))

(fn `UserConstructionScript`
  (`parent.UserConstructionScript`))