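; Base Blueprint for collectable items that signals when one can be picked up.
; On BeginPlay it caches the BP_Snake actor and the GM_Ethan game mode.
; When the player character or snake enters or leaves the Box, it toggles the Widget's visibility and sends CanPickUp or CantPickUp messages with the item and its characteristics, always to the player character.
; Entering also prints the item's name.
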(event `self.ReceiveBeginPlay`
  (bind _returnvalue (`GameplayStatics.GetActorOfClass` "/Game/Blueprint/Mini_Jeux/Snake/BP_Snake.BP_Snake_C"))
  (set `self.SnakeRef` _returnvalue)
  (bind _asgm_ethan (cast `/Game/Blueprint/GameSystem/GM_Ethan` (`GameplayStatics.GetGameMode`)))
  (set `self.GMRef` _asgm_ethan))

(event `self.Box.OnComponentBeginOverlap`
  (params (OverlappedComponent :type "PrimitiveComponent Object Reference") (OtherActor :type "Actor Object Reference") (OtherComp :type "PrimitiveComponent Object Reference") (OtherBodyIndex :type Integer) (bFromSweep :type Boolean) (SweepResult :type "HitResult Structure (by ref)"))
  (bind _returnvalue (`GameplayStatics.GetPlayerCharacter` 0))
  (if (or (== OtherActor _returnvalue) (== OtherActor (`self.SnakeRef`)))
    (message `/Game/Blueprint/Interfaces/BPI_Items.CanPickUp` _returnvalue self (`self.ObjectCarac`))
    (`KismetSystemLibrary.PrintString` (`KismetSystemLibrary.GetDisplayName` self))
    (`SceneComponent.SetVisibility` (`self.Widget`) true false)))

(event `self.Box.OnComponentEndOverlap`
  (params (OverlappedComponent :type "PrimitiveComponent Object Reference") (OtherActor :type "Actor Object Reference") (OtherComp :type "PrimitiveComponent Object Reference") (OtherBodyIndex :type Integer))
  (bind _returnvalue (`GameplayStatics.GetPlayerCharacter` 0))
  (if (or (== OtherActor _returnvalue) (== OtherActor (`self.SnakeRef`)))
    (message `/Game/Blueprint/Interfaces/BPI_Items.CantPickUp` _returnvalue self (`self.ObjectCarac`))
    (`SceneComponent.SetVisibility` (`self.Widget`) false false)))

(fn `UserConstructionScript`)