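; BP_BrokenLadder is a broken ladder item that turns into a working ladder when possessed.
; Its Possess event spawns a BP_Ladder at the actor's location, then destroys the broken actor.
; Only the location is passed to the spawn, and all other graph events are disabled stubs.
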(event `self.Possess`
  (`|SpawnActorFromClass` "/Game/Blueprint/Items/BP_Ladder.BP_Ladder_C" (`KismetMathLibrary.MakeTransform` (`self.K2_GetActorLocation`)) "Undefined" "MultiplyWithRoot" null null)
  (`self.K2_DestroyActor`))

(fn `UserConstructionScript`
  (`parent.UserConstructionScript`))