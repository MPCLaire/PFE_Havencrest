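; Inventory component that holds the player's items in an array of slot structs and toggles the inventory screen with Tab when allowed.
; BeginPlay creates 16 slots and caches the BP_Ethan reference.
; AddToInventory increments a matching non-full stack, otherwise fills the first empty slot below index 15, then refreshes any open WB_inventory grid.
; Opening and closing the widget switches input mode and mouse cursor visibility.
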(event `self.ReceiveBeginPlay`
  ;[1 1 1] Créer les slots vide, le tableau comporte 16 struc vide, on les remplie une par une en ramassant des items
  (for _ (range 16)
    (`KismetArrayLibrary.Array_Add` (`self.Inventory2`))
    (bind _asbp_ethan (cast `/Game/Blueprint/MainCharacter/Blueprints/BP_Ethan` (`GameplayStatics.GetPlayerCharacter` 0)))
    (set `self.EthanRef` _asbp_ethan)))

(event `Key|Tab`
  (params (Key :type "Key Structure"))
  (:`Pressed`
    (if (`self.CanTab`)
      (bind _foundwidgets (`WidgetBlueprintLibrary.GetAllWidgetsOfClass` "/Game/Blueprint/Inventory/WB_inventory.WB_inventory_C"))
      (bind _output (`|GetArrayItem` _foundwidgets))
      (`/Engine/EditorBlueprintResources/StandardMacros.IsValid` _output
        (:`Is Valid`
          (`self.CloseInventory` _output))
        (:`Is Not Valid`
          (`self.OpenInventory`)
          (if (`/Game/Blueprint/MainCharacter/Blueprints/BP_Ethan.isTutoItem` (`self.EthanRef`))
            _))))))

(fn `AddToInventory`
  (params (Inventory :type "/Game/Blueprint/Inventory/ST_inventory2 Structure"))
  (returns (ItemAdded :type Boolean) (IndexRef1 :type Integer))
  (locals (InventoryRef :type "/Game/Blueprint/Inventory/ST_inventory Structure") (IndexRef :type Integer) (Found :type Boolean) (`Inventoryref 2` :type "/Game/Blueprint/Inventory/ST_inventory2 Structure"))
  (bind _indexref (`local.IndexRef`))
  (bind _indexref_2 (`local.IndexRef`))
  (bind _inventory2 (`self.Inventory2`))
  (bind _indexref_3 (`local.IndexRef`))
  (bind (_image _name _quantity _maxstack _namefusion _imagefusion _quantityfusion _maxstaxkfusion _itemclass _fusionitemclass _givable) (break `/Game/Blueprint/Inventory/ST_inventory2` (`|GetArrayItem` _inventory2 _indexref_3)))
  (set `local.Inventoryref 2` Inventory)
  (for (_array_element _array_index) (`self.Inventory2`)
    (set `local.IndexRef` _array_index)
    (if (and (`KismetTextLibrary.EqualEqual_TextText` (`.Name_7_C190B5B346B71737A982D69200F6DB2D` (break `/Game/Blueprint/Inventory/ST_inventory2` _array_element)) (`.Name_7_C190B5B346B71737A982D69200F6DB2D` (break `/Game/Blueprint/Inventory/ST_inventory2` (`local.Inventoryref 2`)))) (< (`.Quantity_10_AF96E3D6429E4CC20D8A7389A135EBDE` (break `/Game/Blueprint/Inventory/ST_inventory2` _array_element)) (`.MaxStack_12_4FD250F94E7B40059065E0BF4F091A52` (break `/Game/Blueprint/Inventory/ST_inventory2` _array_element))))
      (set `local.Found` true)
      (break)))
  (if (`local.Found`)
    (`KismetArrayLibrary.Array_Set` _inventory2 _indexref_3 (make `/Game/Blueprint/Inventory/ST_inventory2` _image _name (+ _quantity 1) _maxstack _namefusion _imagefusion _quantityfusion _maxstaxkfusion _itemclass _fusionitemclass _givable))
    (bind _foundwidgets (`WidgetBlueprintLibrary.GetAllWidgetsOfClass` "/Game/Blueprint/Inventory/WB_inventory.WB_inventory_C"))
    (bind _output (`|GetArrayItem` _foundwidgets))
    (`/Engine/EditorBlueprintResources/StandardMacros.IsValid` _output
      (:`Is Valid`
        (`/Game/Blueprint/Inventory/WB_inventory.SetGrid` _output))
      (:`Is Not Valid`
        _))
    (`KismetSystemLibrary.PrintString` (`KismetStringLibrary.Conv_IntToString` _indexref_2))
    (return true _indexref_2)
    (else
      (for (_array_element_2 _array_index_2) (`self.Inventory2`)
        (set `local.IndexRef` _array_index_2)
        (if (== (`.Quantity_10_AF96E3D6429E4CC20D8A7389A135EBDE` (break `/Game/Blueprint/Inventory/ST_inventory2` _array_element_2)) 0)
          (set `local.Found` true)
          (break)))
      (if (`local.Found`)
        (if (>= (`local.IndexRef`) 15)
          (`KismetSystemLibrary.PrintString` "InventairePlein")
          (else
            (`KismetArrayLibrary.Array_Set` (`self.Inventory2`) (`local.IndexRef`) (`local.Inventoryref 2`))
            (bind _foundwidgets_2 (`WidgetBlueprintLibrary.GetAllWidgetsOfClass` "/Game/Blueprint/Inventory/WB_inventory.WB_inventory_C"))
            (bind _output_2 (`|GetArrayItem` _foundwidgets_2))
            (`/Engine/EditorBlueprintResources/StandardMacros.IsValid` _output_2
              (:`Is Valid`
                (`/Game/Blueprint/Inventory/WB_inventory.SetGrid` _output_2))
              (:`Is Not Valid`
                _))
            (`KismetSystemLibrary.PrintString` (`KismetStringLibrary.Conv_IntToString` _indexref))
            (return true _indexref)))
        (else
          (return false 0))))))

(fn `CloseInventory`
  (params (WIdgetInventory :type "Widget Object Reference"))
  (bind _returnvalue (`GameplayStatics.GetPlayerController` 0))
  (`Widget.RemoveFromParent` WIdgetInventory)
  (`WidgetBlueprintLibrary.SetInputMode_GameOnly` _returnvalue)
  (set `PlayerController.bShowMouseCursor` false _returnvalue))

(fn `OpenInventory`
  (bind _returnvalue (`GameplayStatics.GetPlayerController` 0))
  (bind _returnvalue_2 (`|CreateWidget` "/Game/Blueprint/Inventory/WB_inventory.WB_inventory_C"))
  (`UserWidget.AddToViewport` _returnvalue_2 0)
  (`WidgetBlueprintLibrary.SetInputMode_GameAndUIEx` _returnvalue null)
  (set `PlayerController.bShowMouseCursor` true _returnvalue))