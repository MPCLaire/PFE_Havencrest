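; Obstacle for the Snake mini-game that moves at a constant per-frame offset along its direction, without delta-time scaling or sweep.
; When its Cube overlaps the BP_SnakeArena, it changes direction: two bounces flip only the Y component, then the third reverses the whole vector and resets the counter.
; Casts for bouncing off the snake and its tail exist but are disconnected, so only the arena triggers bounces.
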(event `self.ReceiveTick`
  (params (DeltaSeconds :type "Float (single-precision)"))
  (`self.K2_AddActorWorldOffset` (* (`self.MoveDirection`) (`self.MoveSpeed`))))

(event `self.ReceiveBeginPlay`
  (`parent.ReceiveBeginPlay`))

(event `ChangeDirection`
  (`/Engine/EditorBlueprintResources/StandardMacros.IncrementInt` (`self.RebondNumber`)
    (:`  `
      (if (== (`self.RebondNumber`) 3)
        (set `self.MoveDirection` (* (`self.MoveDirection`) -1.0))
        (set `self.RebondNumber` 0)
        (else
          (set `self.MoveDirection` (* (`self.MoveDirection`) (1.0 -1.0 0.0))))))))

(event `self.Cube.OnComponentBeginOverlap`
  (params (OverlappedComponent :type "PrimitiveComponent Object Reference") (OtherActor :type "Actor Object Reference") (OtherComp :type "PrimitiveComponent Object Reference") (OtherBodyIndex :type Integer) (bFromSweep :type Boolean) (SweepResult :type "HitResult Structure (by ref)"))
  (cast `/Game/Blueprint/Mini_Jeux/Snake/BP_SnakeArena` OtherActor)
  (`self.ChangeDirection`))

(fn `UserConstructionScript`
  (`parent.UserConstructionScript`))