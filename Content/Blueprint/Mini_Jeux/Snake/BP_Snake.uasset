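; BP_Snake is the player-piece actor of a Snake mini-game, with a head that can collect a key for BP_Ethan.
; AddTail recursively spawns up to six BP_SnakeTail segments behind the head.
; While Snaking, each Tick moves the head one mesh-width along MoveDirection and shifts every segment into its predecessor's previous location.
; Head overlap with BP_SnakeKey triggers Ethan's pickup and sets HasKey; SnakeDeath stops movement, while SnakeWin is empty.
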(event `self.ReceiveBeginPlay`
  (bind _returnvalue (`StaticMesh.GetBoundingBox` (`StaticMeshComponent.StaticMesh` (`self.Head`))))
  ;[1 1 1] Définis la taille d'une queue pour pas les faire spawn les unes sur les autres
  (set `self.StepSize` (- (.x (`.Max` (break `Box` _returnvalue))) (.x (break `Box` _returnvalue))))
  (bind _returnvalue_2 (`GameplayStatics.GetActorOfClass` "/Game/Blueprint/MainCharacter/Blueprints/BP_Ethan.BP_Ethan_C"))
  (set `self.EthanRef` _returnvalue_2))

(event `Add Tail`
  ;[1 1 1] Crée 6 queues et les ajoute à la liste
  (if (< (`self.TailsNumber`) 6)
    (bind _returnvalue (`|SpawnActorFromClass` "/Game/Blueprint/Mini_Jeux/Snake/BP_SnakeTail.BP_SnakeTail_C" (`KismetMathLibrary.MakeTransform` (- (`self.K2_GetActorLocation`) (* (`self.MoveDirection`) (`self.StepSize`)))) "AlwaysSpawn" "MultiplyWithRoot" null null))
    (`KismetArrayLibrary.Array_Add` (`self.Tails`) _returnvalue)
    (`/Engine/EditorBlueprintResources/StandardMacros.IncrementInt` (`self.TailsNumber`)
      (:`  `
        (`self.Add Tail`)))))

(event `self.ReceiveTick`
  (params (DeltaSeconds :type "Float (single-precision)"))
  ;[1 1 1] Déplacement du snake
  (if (`self.Snaking?`)
    (set `self.PreviousitemLocation` (`self.K2_GetActorLocation`))
    (`self.K2_AddActorWorldOffset` (* (`self.MoveDirection`) (`self.StepSize`)))
    (set `self.CurrentMoveDirection` (- (`self.K2_GetActorLocation`) (`self.PreviousitemLocation`)))
    (for _array_element (`self.Tails`)
      (bind _output_get (set `self.CurrentTailLocation` (`self.K2_GetActorLocation` _array_element)))
      (`self.K2_SetActorLocation` _array_element (`self.PreviousitemLocation`) false false)
      (set `self.PreviousitemLocation` _output_get))))

(event `self.Head.OnComponentBeginOverlap`
  (params (OverlappedComponent :type "PrimitiveComponent Object Reference") (OtherActor :type "Actor Object Reference") (OtherComp :type "PrimitiveComponent Object Reference") (OtherBodyIndex :type Integer) (bFromSweep :type Boolean) (SweepResult :type "HitResult Structure (by ref)"))
  (bind _ethanref (`self.EthanRef`))
  ;[1 1 1] ramasser la clef
  (bind _asbp_snake_key (cast `/Game/Blueprint/Items/Collectable/BP_SnakeKey` OtherActor))
  (`/Game/Blueprint/Interfaces/BPI_Items.CanPickUp` _ethanref _asbp_snake_key (`/Game/Blueprint/Items/Collectable/BP_ItemParent.ObjectCarac` _asbp_snake_key))
  (`/Game/Blueprint/MainCharacter/Blueprints/BP_Ethan.PickUpItem` _ethanref)
  (set `self.HasKey` true))

(fn `SnakeDeath`
  (set `self.Snaking?` false))

(fn `SnakeWin`)

(fn `UserConstructionScript`)