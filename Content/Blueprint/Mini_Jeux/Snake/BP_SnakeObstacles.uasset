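; BP_SnakeObstacles is an obstacle actor for the Snake minigame that kills the snake on contact.
; It finds the BP_Snake at BeginPlay and calls its SnakeDeath when the snake or a BP_SnakeTail overlaps its Cube.
; Obstacles flagged as walls give the head a brief timer-based grace period, killing it only if it still overlaps, and cancel the timer when it leaves.
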(event `self.ReceiveBeginPlay`
  (bind _returnvalue (`GameplayStatics.GetActorOfClass` "/Game/Blueprint/Mini_Jeux/Snake/BP_Snake.BP_Snake_C"))
  (set `self.snakeRef` _returnvalue))

(event `CheckIfOverlap`
  (if (`self.IsOverlaping?`)
    (`/Game/Blueprint/Mini_Jeux/Snake/BP_Snake.SnakeDeath` (`self.snakeRef`))))

(event `self.Cube.OnComponentBeginOverlap`
  (params (OverlappedComponent :type "PrimitiveComponent Object Reference") (OtherActor :type "Actor Object Reference") (OtherComp :type "PrimitiveComponent Object Reference") (OtherBodyIndex :type Integer) (bFromSweep :type Boolean) (SweepResult :type "HitResult Structure (by ref)"))
  (cast `/Game/Blueprint/Mini_Jeux/Snake/BP_Snake` OtherActor
    (:`then`
      (if (`self.IsWall?`)
        (set `self.IsOverlaping?` true)
        (bind _returnvalue (`KismetSystemLibrary.K2_SetTimerDelegate` (delegate `CheckIfOverlap`) 0.25))
        (else
          (`/Game/Blueprint/Mini_Jeux/Snake/BP_Snake.SnakeDeath` (`self.snakeRef`)))))
    (:`CastFailed`
      (cast `/Game/Blueprint/Mini_Jeux/Snake/BP_SnakeTail` OtherActor)
      (`/Game/Blueprint/Mini_Jeux/Snake/BP_Snake.SnakeDeath` (`self.snakeRef`)))))

(event `self.Cube.OnComponentEndOverlap`
  (params (OverlappedComponent :type "PrimitiveComponent Object Reference") (OtherActor :type "Actor Object Reference") (OtherComp :type "PrimitiveComponent Object Reference") (OtherBodyIndex :type Integer))
  (cast `/Game/Blueprint/Mini_Jeux/Snake/BP_Snake` OtherActor)
  (set `self.IsOverlaping?` false)
  (`KismetSystemLibrary.K2_ClearAndInvalidateTimerHandle` (stale `self.Cube.OnComponentBeginOverlap` _returnvalue)))

(fn `UserConstructionScript`)