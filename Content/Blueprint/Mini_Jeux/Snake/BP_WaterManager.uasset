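; Water manager for the Snake minigame that recycles two BP_WaterGreen actors, apparently to fake endless water.
; On BeginPlay it spawns a second actor offset along negative Y from the referenced one and records its location.
; A looping timer drives a FlipFlop that alternately teleports each actor to a fixed point beyond that recorded location.
; The box end-overlap only prints a debug string, and some older spawn logic is left disconnected.
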(event `self.ReceiveBeginPlay`
  (`self.SpawnNewWater`)
  (set `self.WaterInitialLoc` (`SceneComponent.K2_GetComponentLocation` (`/Game/Blueprint/Mini_Jeux/Snake/BP_WaterGreen.DefaultSceneRoot` (`self.WaterRef`))))
  (`KismetSystemLibrary.K2_SetTimerDelegate` (delegate `MoveWater`) 16.05 true))

(event `MoveWater`
  (bind (_secondwaterinitialloc_x _secondwaterinitialloc_y _secondwaterinitialloc_z) (`KismetMathLibrary.BreakVector` (`self.SecondWaterInitialLoc`)))
  (bind (_secondwaterinitialloc_x_2 _secondwaterinitialloc_y_2 _secondwaterinitialloc_z_2) (`KismetMathLibrary.BreakVector` (`self.SecondWaterInitialLoc`)))
  (`/Engine/EditorBlueprintResources/StandardMacros.FlipFlop`
    (:`A`
      (`SceneComponent.K2_SetWorldLocation` (`/Game/Blueprint/Mini_Jeux/Snake/BP_WaterGreen.DefaultSceneRoot` (`self.WaterRef`)) (`KismetMathLibrary.MakeVector` _secondwaterinitialloc_x (- _secondwaterinitialloc_y 1200.0) _secondwaterinitialloc_z) false true))
    (:`B`
      (`SceneComponent.K2_SetWorldLocation` (`/Game/Blueprint/Mini_Jeux/Snake/BP_WaterGreen.DefaultSceneRoot` (`self.SecondWaterRef`)) (`KismetMathLibrary.MakeVector` _secondwaterinitialloc_x_2 (- _secondwaterinitialloc_y_2 1200.0) _secondwaterinitialloc_z_2) false true))))

(event `SpawnNewWater`
  (bind _returnvalue (`self.GetTransform` (`self.WaterRef`)))
  (bind _returnvalue_2 (`|SpawnActorFromClass` "/Game/Blueprint/Mini_Jeux/Snake/BP_WaterGreen.BP_WaterGreen_C" (`KismetMathLibrary.MakeTransform` (`KismetMathLibrary.MakeVector` (.x (.location _returnvalue)) (- (.y (.location _returnvalue)) 1550.0) (.z (.location _returnvalue))) (.rotation _returnvalue) (`KismetMathLibrary.MakeVector` (.x (.scale _returnvalue)) (.y (.scale _returnvalue)) (.z (.scale _returnvalue)))) "AlwaysSpawn" "MultiplyWithRoot" null null))
  (bind _output_get (set `self.SecondWaterRef` _returnvalue_2))
  (set `self.SecondWaterInitialLoc` (`SceneComponent.K2_GetComponentLocation` (`/Game/Blueprint/Mini_Jeux/Snake/BP_WaterGreen.DefaultSceneRoot` _output_get))))

(event `self.Box.OnComponentEndOverlap`
  (params (OverlappedComponent :type "PrimitiveComponent Object Reference") (OtherActor :type "Actor Object Reference") (OtherComp :type "PrimitiveComponent Object Reference") (OtherBodyIndex :type Integer))
  (if (== OtherActor (`self.WaterRef`))
    (`KismetSystemLibrary.PrintString` "Hello")))

(fn `UserConstructionScript`)