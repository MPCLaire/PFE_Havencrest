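; BP_PlayerSnake is the player-controlled pawn for the Snake minigame, relaying keyboard input to the BP_Snake actor found at BeginPlay.
; Arrow keys set the snake's MoveDirection only when its current movement has no component on that axis, which blocks reversals.
; The first accepted press also calls AddTail through a shared DoOnce.
; StartSnake makes player controller 0 possess this pawn.
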(event `self.ReceiveBeginPlay`
  (bind _returnvalue (`GameplayStatics.GetActorOfClass` "/Game/Blueprint/Mini_Jeux/Snake/BP_Snake.BP_Snake_C"))
  (set `self.SnakeRef` _returnvalue))

(event `Key|Up`
  (params (Key :type "Key Structure"))
  (bind _currentmovedirection_x (`KismetMathLibrary.BreakVector` (`/Game/Blueprint/Mini_Jeux/Snake/BP_Snake.CurrentMoveDirection` (`self.SnakeRef`))))
  ;[1 1 1] Déplacements
  (:`Pressed`
    (if (== _currentmovedirection_x 0.0)
      (set `/Game/Blueprint/Mini_Jeux/Snake/BP_Snake.MoveDirection` (1.0 0.0 0.0) (`self.SnakeRef`))
      (`/Engine/EditorBlueprintResources/StandardMacros.DoOnce` false :!label _label
        (:`Completed`
          (`/Game/Blueprint/Mini_Jeux/Snake/BP_Snake.Add Tail` (`self.SnakeRef`)))))))

(event `Key|Down`
  (params (Key :type "Key Structure"))
  (bind _currentmovedirection_x (`KismetMathLibrary.BreakVector` (`/Game/Blueprint/Mini_Jeux/Snake/BP_Snake.CurrentMoveDirection` (`self.SnakeRef`))))
  ;[1 1 1] Déplacements
  (:`Pressed`
    (if (== _currentmovedirection_x 0.0)
      (set `/Game/Blueprint/Mini_Jeux/Snake/BP_Snake.MoveDirection` (-1.0 0.0 0.0) (`self.SnakeRef`))
      (goto _label))))

(event `Key|Left`
  (params (Key :type "Key Structure"))
  (bind (_currentmovedirection_x _currentmovedirection_y) (`KismetMathLibrary.BreakVector` (`/Game/Blueprint/Mini_Jeux/Snake/BP_Snake.CurrentMoveDirection` (`self.SnakeRef`))))
  ;[1 1 1] Déplacements
  (:`Pressed`
    (if (== _currentmovedirection_y 0.0)
      (set `/Game/Blueprint/Mini_Jeux/Snake/BP_Snake.MoveDirection` (0.0 -1.0 0.0) (`self.SnakeRef`))
      (goto _label))))

(event `Key|Right`
  (params (Key :type "Key Structure"))
  (bind (_currentmovedirection_x _currentmovedirection_y) (`KismetMathLibrary.BreakVector` (`/Game/Blueprint/Mini_Jeux/Snake/BP_Snake.CurrentMoveDirection` (`self.SnakeRef`))))
  ;[1 1 1] Déplacements
  (:`Pressed`
    (if (== _currentmovedirection_y 0.0)
      (set `/Game/Blueprint/Mini_Jeux/Snake/BP_Snake.MoveDirection` (0.0 1.0 0.0) (`self.SnakeRef`))
      (goto _label))))

(fn `StartSnake`
  (`Controller.Possess` (`GameplayStatics.GetPlayerController` 0) self))

(fn `UserConstructionScript`)