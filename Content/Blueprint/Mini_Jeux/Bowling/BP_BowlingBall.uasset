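; Bowling ball actor for the bowling minigame, with a spin animation for its Plane component during launch.
; RotateDuringLaunch plays a timeline that turns the Plane's relative pitch through a full circle, replaying while KeepRotating is true and setting world rotation when it stops.
; BeginPlay and the Plane's overlap event are empty; disconnected nodes hold unused logic to fetch the bowling garage and lift the Plane off its floor.
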(event `self.ReceiveBeginPlay`)

(event `RotateDuringLaunch`
  (bind (_relativerotation_roll _relativerotation_pitch _relativerotation_yaw) (`KismetMathLibrary.BreakRotator` (`SceneComponent.RelativeRotation` (`self.Plane`))))
  (bind (_direction _newtrack_0) (`Timeline|RotateTL` :!label _label)
    (:`Update`
      (bind _returnvalue (`KismetMathLibrary.MakeRotator` _relativerotation_roll (`KismetMathLibrary.Lerp` 0.0 360.0 _newtrack_0) _relativerotation_yaw))
      (`SceneComponent.K2_SetRelativeRotation` (`self.Plane`) _returnvalue false false))
    (:`Finished`
      (if (`self.KeepRotating?`)
        (goto _label :!via `PlayFromStart`)
        (else
          (`SceneComponent.K2_SetWorldRotation` (`self.Plane`) _returnvalue false false))))))

(event `self.Plane.OnComponentBeginOverlap`
  (params (OverlappedComponent :type "PrimitiveComponent Object Reference") (OtherActor :type "Actor Object Reference") (OtherComp :type "PrimitiveComponent Object Reference") (OtherBodyIndex :type Integer) (bFromSweep :type Boolean) (SweepResult :type "HitResult Structure (by ref)")))

(fn `UserConstructionScript`)