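; Bowling ball actor for a mini-game, handling the spin animation during a launch.
; RotateDuringLaunch plays a timeline that lerps the Plane component's relative pitch through a full turn, preserving roll and yaw.
; On finish it replays from the start while KeepRotating is true, otherwise it applies the final rotation in world space.
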(event `RotateDuringLaunch`
  (bind (_relativerotation_roll _relativerotation_pitch _relativerotation_yaw) (`KismetMathLibrary.BreakRotator` (`SceneComponent.RelativeRotation` (`self.Plane`))))
  (bind (_direction _newtrack_0) (`Timeline|RotateTL` :!label _label)
    (:`Update`
      (bind _returnvalue (`KismetMathLibrary.MakeRotator` _relativerotation_roll (`KismetMathLibrary.Lerp` 0.0 360.0 _newtrack_0) _relativerotation_yaw))
      (`SceneComponent.K2_SetRelativeRotation` (`self.Plane`) _returnvalue false false))
    (:`Finished`
      (if (`self.KeepRotating?`)
        (goto _label :!via `PlayFromStart`)
        (else
          (`SceneComponent.K2_SetWorldRotation` (`self.Plane`) _returnvalue false false))))))

(fn `UserConstructionScript`)