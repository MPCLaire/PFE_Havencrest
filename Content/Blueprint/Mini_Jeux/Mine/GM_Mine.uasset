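; Game mode for the mine minigame, where the player picks directions through a sequence of tunnels to reach the mine interior.
; A timeline slides a single reused tunnel actor by TurnDirection, then the player fades and the tunnel resets for the next step.
; CheckDirection compares input to the MineOnLeft sequence.
; A wrong turn resets progress and returns control to Ethan, while completing it moves Ethan to the interior start point.
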(event `self.ReceiveBeginPlay`
  (bind _asbp_ethan (cast `/Game/Blueprint/MainCharacter/Blueprints/BP_Ethan` (`GameplayStatics.GetPlayerPawn` 0)))
  (set `self.As BP Ethan` _asbp_ethan)
  (set `self.TunnelLoc` (`self.K2_GetActorLocation` (`self.TunnelRef`)))
  (bind _returnvalue (`GameplayStatics.GetActorOfClass` "/Game/Assets/DecorsAsset/Batiments/Mine/BP_MineInterieur.BP_MineInterieur_C"))
  (set `self.MineInterieurRef` _returnvalue))

(event `CallTimeline`
  (`|ExecutionSequence`
    (:`then_0`
      (`self.K2_SetActorLocation` (`self.TunnelRef`) (`self.TunnelLoc`) false false)
      (bind (_direction _movetrack _newtrack_1) (`Timeline|Timeline` :!via `PlayFromStart`)
        (:`Update`
          (bind _returnvalue (+ (+ _movetrack (`self.TunnelLoc`)) (* _newtrack_1 (`self.TurnDirection`))))
          (`self.K2_SetActorRelativeLocation` (`self.TunnelRef`) _returnvalue false false))
        (:`Finished`
          (`self.K2_SetActorLocation` (`self.TunnelRef`) _returnvalue false false))))
    (:`then_1`
      (`KismetSystemLibrary.Delay` 3.3)
      (`self.NextTunnel`))))

(event `NextTunnel`
  (`/Game/Blueprint/Mini_Jeux/Mine/BP_PlayerMine.FadeIn` (`self.PlayerMineRef`))
  (`KismetSystemLibrary.Delay` 1.0)
  (set `self.TurnDirection` 0)
  (`/Game/Blueprint/Widget/WB_Mine.ResetButtons` (`self.WidgetMineArrow`))
  (if (== (`self.levelMine`) (`KismetArrayLibrary.Array_Length` (`self.MineOnLeft`)))
    (`self.K2_SetActorLocation` (`self.As BP Ethan`) (`SceneComponent.K2_GetComponentLocation` (`/Game/Assets/DecorsAsset/Batiments/Mine/BP_MineInterieur.StartPoint` (`self.MineInterieurRef`))) false false)
    (`Widget.RemoveFromParent` (`self.WidgetMineArrow`))
    (`Controller.Possess` (`GameplayStatics.GetPlayerController` 0) (`self.As BP Ethan`))
    (elif (`self.TurnCorrectly?`)
      (`self.K2_SetActorLocation` (`self.TunnelRef`) (`self.TunnelLoc`) false false)
      (`KismetSystemLibrary.Delay` 0.5)
      (`self.CallTimeline`)
      (set `self.TurnCorrectly?` false)
      (else
        (`self.FromMineToEthan`)))))

(fn `CheckDirection`
  (params (PlayerInput :type Boolean))
  (if (== PlayerInput (`|GetArrayItem` (`self.MineOnLeft`) (`self.levelMine`)))
    (set `self.TurnCorrectly?` true)
    (`KismetSystemLibrary.PrintString` "Oui")
    (`/Engine/EditorBlueprintResources/StandardMacros.IncrementInt` (`self.levelMine`))
    (else
      (set `self.TurnCorrectly?` false)
      (`KismetSystemLibrary.PrintString` "Non"))))

(fn `FromMineToEthan`
  (bind _as_bp_ethan (`self.As BP Ethan`))
  (set `self.levelMine` 0)
  (`/Game/Blueprint/MainCharacter/Blueprints/BP_Ethan.PossessEthan` _as_bp_ethan)
  (`/Game/Blueprint/MainCharacter/Blueprints/BP_Ethan.SetNewCameraInBuilding` _as_bp_ethan (`/Game/Blueprint/MainCharacter/Blueprints/BP_Ethan.CameraBatimentRef` _as_bp_ethan))
  (`Widget.RemoveFromParent` (`self.WidgetMineArrow`)))

(fn `UserConstructionScript`)