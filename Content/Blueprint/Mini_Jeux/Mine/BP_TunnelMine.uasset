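; Tunnel actor for the mine mini-game that triggers the player's side move at a turn zone.
; On BeginPlay it caches the GM_Mine game mode and registers itself there as TunnelRef.
; When a BP_PlayerMine enters TurnBox, a DoOnce gate calls its MoveToSide, and the gate resets when the player's overlap ends.
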(event `self.ReceiveBeginPlay`
  (bind _asgm_mine (cast `/Game/Blueprint/Mini_Jeux/Mine/GM_Mine` (`GameplayStatics.GetGameMode`)))
  (set `self.GMMineRef` _asgm_mine)
  (set `/Game/Blueprint/Mini_Jeux/Mine/GM_Mine.TunnelRef` self _asgm_mine))

(event `self.TurnBox.OnComponentBeginOverlap`
  (params (OverlappedComponent :type "PrimitiveComponent Object Reference") (OtherActor :type "Actor Object Reference") (OtherComp :type "PrimitiveComponent Object Reference") (OtherBodyIndex :type Integer) (bFromSweep :type Boolean) (SweepResult :type "HitResult Structure (by ref)"))
  (bind _asbp_player_mine (cast `/Game/Blueprint/Mini_Jeux/Mine/BP_PlayerMine` OtherActor))
  (`/Engine/EditorBlueprintResources/StandardMacros.DoOnce` false :!label _label
    (:`Completed`
      (`/Game/Blueprint/Mini_Jeux/Mine/BP_PlayerMine.MoveToSide` _asbp_player_mine))))

(event `self.TurnBox.OnComponentEndOverlap`
  (params (OverlappedComponent :type "PrimitiveComponent Object Reference") (OtherActor :type "Actor Object Reference") (OtherComp :type "PrimitiveComponent Object Reference") (OtherBodyIndex :type Integer))
  (cast `/Game/Blueprint/Mini_Jeux/Mine/BP_PlayerMine` OtherActor)
  (goto _label :!via `Reset`))

(fn `UserConstructionScript`)