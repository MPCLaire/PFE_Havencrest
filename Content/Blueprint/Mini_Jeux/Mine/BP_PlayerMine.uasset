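; BP_PlayerMine is the possessable player for the Mine minigame, registering itself with GM_Mine on BeginPlay and caching the BP_Ethan player character.
; PossessMine hands player controller 0 to it, shows the mouse cursor, adds the WB_Mine widget to the viewport and calls the game mode's CallTimeline.
; FadeIn spawns an actor at the FadePlane transform, with no class specified.
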(event `self.ReceiveBeginPlay`
  (bind _asbp_ethan (cast `/Game/Blueprint/MainCharacter/Blueprints/BP_Ethan` (`GameplayStatics.GetPlayerCharacter` 0)))
  (set `self.As BP Ethan` _asbp_ethan)
  (bind _asgm_mine (cast `/Game/Blueprint/Mini_Jeux/Mine/GM_Mine` (`GameplayStatics.GetGameMode`)))
  (set `self.As GM Mine` _asgm_mine)
  (set `/Game/Blueprint/Mini_Jeux/Mine/GM_Mine.PlayerMineRef` self _asgm_mine))

(event `PossessMine`
  (bind _returnvalue (`GameplayStatics.GetPlayerController` 0))
  (bind _as_gm_mine (`self.As GM Mine`))
  (`Controller.Possess` _returnvalue self)
  (set `PlayerController.bShowMouseCursor` true _returnvalue)
  (bind _returnvalue_2 (`|CreateWidget` "/Game/Blueprint/Widget/WB_Mine.WB_Mine_C"))
  (bind _output_get (set `/Game/Blueprint/Mini_Jeux/Mine/GM_Mine.WidgetMineArrow` _returnvalue_2 _as_gm_mine))
  (`UserWidget.AddToViewport` _output_get 0)
  (`/Game/Blueprint/Mini_Jeux/Mine/GM_Mine.CallTimeline` _as_gm_mine))

(fn `FadeIn`
  (`|SpawnActorFromClass` "/Game/Blueprint/BP_FadePlane.BP_FadePlane_C" (`SceneComponent.K2_GetComponentToWorld` (`self.FadePlane`)) "Undefined" "MultiplyWithRoot" null null))

(fn `UserConstructionScript`)