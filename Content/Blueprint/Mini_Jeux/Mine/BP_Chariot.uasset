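; BP_Chariot is the cart actor of the Mine mini-game, marking when the player is within its trigger area.
; On BeginPlay it caches player 0's character as BP_Ethan.
; Its Box overlap events set that character's MineActivated flag to true on entry and false on exit, ignoring all other actors.
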(event `self.ReceiveBeginPlay`
  (bind _asbp_ethan (cast `/Game/Blueprint/MainCharacter/Blueprints/BP_Ethan` (`GameplayStatics.GetPlayerCharacter` 0)))
  (set `self.As BP Ethan` _asbp_ethan))

(event `self.Box.OnComponentBeginOverlap`
  (params (OverlappedComponent :type "PrimitiveComponent Object Reference") (OtherActor :type "Actor Object Reference") (OtherComp :type "PrimitiveComponent Object Reference") (OtherBodyIndex :type Integer) (bFromSweep :type Boolean) (SweepResult :type "HitResult Structure (by ref)"))
  (bind _as_bp_ethan (`self.As BP Ethan`))
  (if (== OtherActor _as_bp_ethan)
    (set `/Game/Blueprint/MainCharacter/Blueprints/BP_Ethan.mineActivated?` true _as_bp_ethan)))

(event `self.Box.OnComponentEndOverlap`
  (params (OverlappedComponent :type "PrimitiveComponent Object Reference") (OtherActor :type "Actor Object Reference") (OtherComp :type "PrimitiveComponent Object Reference") (OtherBodyIndex :type Integer))
  (bind _as_bp_ethan (`self.As BP Ethan`))
  (if (== OtherActor _as_bp_ethan)
    (set `/Game/Blueprint/MainCharacter/Blueprints/BP_Ethan.mineActivated?` false _as_bp_ethan)))

(fn `UserConstructionScript`)