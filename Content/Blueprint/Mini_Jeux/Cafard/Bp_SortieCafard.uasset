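; Exit trigger for the cockroach (Cafard) minigame, reacting when the BP_PlayerCafard found at BeginPlay enters its box.
; On entry it stops and disables the movement of the referenced rat, RatRef.
; It then calls Win on the player if they hold the necklace (HasCollier), otherwise Sort through a DoOnce gate.
; Any end overlap on the box resets that gate.
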(event `self.ReceiveBeginPlay`
  (bind _returnvalue (`GameplayStatics.GetActorOfClass` "/Game/Blueprint/Mini_Jeux/Cafard/BP_PlayerCafard.BP_PlayerCafard_C"))
  (set `self.CafardRef` _returnvalue))

(event `self.Box.OnComponentBeginOverlap`
  (params (OverlappedComponent :type "PrimitiveComponent Object Reference") (OtherActor :type "Actor Object Reference") (OtherComp :type "PrimitiveComponent Object Reference") (OtherBodyIndex :type Integer) (bFromSweep :type Boolean) (SweepResult :type "HitResult Structure (by ref)"))
  (bind _cafardref (`self.CafardRef`))
  (bind _charactermovement (`Character.CharacterMovement` (`self.RatRef`)))
  (if (== OtherActor _cafardref)
    (`NavMovementComponent.StopActiveMovement` _charactermovement)
    (`CharacterMovementComponent.DisableMovement` _charactermovement)
    (if (`/Game/Blueprint/Mini_Jeux/Cafard/BP_PlayerCafard.HasCollier` _cafardref)
      (`/Game/Blueprint/Mini_Jeux/Cafard/BP_PlayerCafard.Win` (`self.CafardRef`))
      (else
        (`/Engine/EditorBlueprintResources/StandardMacros.DoOnce` false :!label _label
          (:`Completed`
            (`/Game/Blueprint/Mini_Jeux/Cafard/BP_PlayerCafard.Sort` (`self.CafardRef`))))))))

(event `self.Box.OnComponentEndOverlap`
  (params (OverlappedComponent :type "PrimitiveComponent Object Reference") (OtherActor :type "Actor Object Reference") (OtherComp :type "PrimitiveComponent Object Reference") (OtherBodyIndex :type Integer))
  (goto _label :!via `Reset`))

(fn `UserConstructionScript`)