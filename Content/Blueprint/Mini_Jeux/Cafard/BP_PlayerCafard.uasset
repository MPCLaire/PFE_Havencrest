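; Player character for the cockroach (Cafard) mini-game, moving a Paper2D flipbook in four directions through Enhanced Input, with reference-counted walking sound.
; Overlapping BP_Collier hands it to EthanRef's pickup, while touching BP_CafardEnnemi triggers death and respawns any carried necklace.
; Death and Sort show widgets and set IsDead, letting E fade, return the player to start and reset enemies.
; Win freezes movement and shows the victory widget.
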(event `self.ReceiveBeginPlay`
  (set `self.StartLocation` (`self.K2_GetActorLocation`))
  ;[1 1 1] input mapping
  (bind _asplayer_controller (cast `PlayerController` (`self.GetController`)))
  (bind _returnvalue (pcsubsystem `EnhancedInputLocalPlayerSubsystem` _asplayer_controller))
  (`/Engine/EditorBlueprintResources/StandardMacros.IsValid` _returnvalue
    (:`Is Valid`
      (`EnhancedInputSubsystemInterface.AddMappingContext` _returnvalue "/Game/Blueprint/Mini_Jeux/Cafard/Inputs/IMC_Cafard.IMC_Cafard" 0 (struct)))))

(event `Key|E`
  (params (Key :type "Key Structure"))
  (:`Pressed`
    (if (`self.IsDead`)
      (set `self.IsDead` false)
      (`Widget.RemoveFromParent` (`self.WidgetRef`))
      (bind _returnvalue (`|SpawnActorFromClass` "/Game/Blueprint/BP_FadePlane.BP_FadePlane_C" (`SceneComponent.K2_GetComponentToWorld` (`self.FadePlane`)) "AlwaysSpawn" "MultiplyWithRoot" null null))
      (`self.K2_AttachToComponent` _returnvalue (`self.FadePlane`) "None" "KeepWorld" "KeepWorld" "KeepWorld" true)
      (`KismetSystemLibrary.Delay` 1.0)
      (`self.StartGame`))))

(event `EnhancedInput|/Game/Blueprint/Mini_Jeux/Cafard/Inputs/IA_MoveDownCafard`
  (params (ActionValue :type "Vector2D Structure") (ElapsedSeconds :type "Float (double-precision)") (TriggeredSeconds :type "Float (double-precision)") (InputAction :type "InputAction Object Reference" :default "/Game/Blueprint/Mini_Jeux/Cafard/Inputs/IA_MoveDownCafard.IA_MoveDownCafard"))
  (bind _paperflipbook (`self.PaperFlipbook`))
  (bind (_returnvalue_roll _returnvalue_pitch) (`KismetMathLibrary.BreakRotator` (`SceneComponent.K2_GetComponentRotation` _paperflipbook)))
  (bind (_returnvalue_x _returnvalue_y _returnvalue_z) (`KismetMathLibrary.BreakVector` (`SceneComponent.GetForwardVector` (`self.Cube`))))
  ;[1 1 1] déplacements
  (:`Triggered`
    (if (`self.CanMove`)
      (`PaperFlipbookComponent.Play` (`self.PaperFlipbook`))
      (`self.AddMovementInput` (`KismetMathLibrary.MakeVector` (* _returnvalue_x -1.0) _returnvalue_y _returnvalue_z) (`self.speed`))
      (`SceneComponent.K2_SetWorldRotation` _paperflipbook (`KismetMathLibrary.MakeRotator` _returnvalue_roll _returnvalue_pitch -90.0) false false)))
  (:`Started`
    (`self.CreateSoundWalk` :!label _label))
  (:`Completed`
    (`self.EnleveSonCafardMarche` :!label _label_2)))

(event `EnhancedInput|/Game/Blueprint/Mini_Jeux/Cafard/Inputs/IA_MoveUpCafard`
  (params (ActionValue :type "Vector2D Structure") (ElapsedSeconds :type "Float (double-precision)") (TriggeredSeconds :type "Float (double-precision)") (InputAction :type "InputAction Object Reference" :default "/Game/Blueprint/Mini_Jeux/Cafard/Inputs/IA_MoveUpCafard.IA_MoveUpCafard"))
  (bind _paperflipbook (`self.PaperFlipbook`))
  (bind (_returnvalue_roll _returnvalue_pitch) (`KismetMathLibrary.BreakRotator` (`SceneComponent.K2_GetComponentRotation` _paperflipbook)))
  ;[1 1 1] déplacements
  (:`Triggered`
    (if (`self.CanMove`)
      (`PaperFlipbookComponent.Play` (`self.PaperFlipbook`))
      (`self.AddMovementInput` (`SceneComponent.GetForwardVector` (`self.Cube`)) (`self.speed`))
      (`SceneComponent.K2_SetWorldRotation` _paperflipbook (`KismetMathLibrary.MakeRotator` _returnvalue_roll _returnvalue_pitch 90.0) false false)))
  (:`Started`
    (goto _label))
  (:`Completed`
    (goto _label_2)))

(event `self.CapsuleComponent.OnComponentBeginOverlap`
  (params (OverlappedComponent :type "PrimitiveComponent Object Reference") (OtherActor :type "Actor Object Reference") (OtherComp :type "PrimitiveComponent Object Reference") (OtherBodyIndex :type Integer) (bFromSweep :type Boolean) (SweepResult :type "HitResult Structure (by ref)"))
  (bind _ethanref (`self.EthanRef`))
  (bind _asbp_collier (cast `/Game/Blueprint/Items/Collectable/BP_Collier` OtherActor)
    (:`then`
      (bind _output_get (set `self.CollierRef` _asbp_collier))
      (set `self.CollierTransfo` (`self.GetTransform` _output_get))
      (`/Game/Blueprint/Interfaces/BPI_Items.CanPickUp` _ethanref _asbp_collier (`/Game/Blueprint/Items/Collectable/BP_ItemParent.ObjectCarac` _asbp_collier))
      (`/Game/Blueprint/MainCharacter/Blueprints/BP_Ethan.PickUpItem` _ethanref)
      (set `self.HasCollier` true))
    (:`CastFailed`
      (cast `/Game/Blueprint/Mini_Jeux/Cafard/BP_CafardEnnemi` OtherActor)
      (`self.Death`))))

(event `EnhancedInput|/Game/Blueprint/Mini_Jeux/Cafard/Inputs/IA_MoveLeftCafard`
  (params (ActionValue :type "Vector2D Structure") (ElapsedSeconds :type "Float (double-precision)") (TriggeredSeconds :type "Float (double-precision)") (InputAction :type "InputAction Object Reference" :default "/Game/Blueprint/Mini_Jeux/Cafard/Inputs/IA_MoveLeftCafard.IA_MoveLeftCafard"))
  (bind _paperflipbook (`self.PaperFlipbook`))
  (bind (_returnvalue_x _returnvalue_y _returnvalue_z) (`KismetMathLibrary.BreakVector` (`SceneComponent.GetRightVector` (`self.Cube`))))
  (bind (_returnvalue_roll _returnvalue_pitch) (`KismetMathLibrary.BreakRotator` (`SceneComponent.K2_GetComponentRotation` _paperflipbook)))
  ;[1 1 1] déplacements
  (:`Triggered`
    (if (`self.CanMove`)
      (`PaperFlipbookComponent.Play` (`self.PaperFlipbook`))
      (`self.AddMovementInput` (`KismetMathLibrary.MakeVector` _returnvalue_x (* _returnvalue_y -1.0) _returnvalue_z) (`self.speed`))
      (`SceneComponent.K2_SetWorldRotation` _paperflipbook (`KismetMathLibrary.MakeRotator` _returnvalue_roll _returnvalue_pitch) false false)))
  (:`Started`
    (goto _label))
  (:`Completed`
    (goto _label_2)))

(event `EnhancedInput|/Game/Blueprint/Mini_Jeux/Cafard/Inputs/IA_MoveRightCafard`
  (params (ActionValue :type "Vector2D Structure") (ElapsedSeconds :type "Float (double-precision)") (TriggeredSeconds :type "Float (double-precision)") (InputAction :type "InputAction Object Reference" :default "/Game/Blueprint/Mini_Jeux/Cafard/Inputs/IA_MoveRightCafard.IA_MoveRightCafard"))
  (bind _paperflipbook (`self.PaperFlipbook`))
  (bind (_returnvalue_roll _returnvalue_pitch) (`KismetMathLibrary.BreakRotator` (`SceneComponent.K2_GetComponentRotation` _paperflipbook)))
  ;[1 1 1] déplacements
  (:`Triggered`
    (if (`self.CanMove`)
      (`PaperFlipbookComponent.Play` (`self.PaperFlipbook`))
      (`self.AddMovementInput` (`SceneComponent.GetRightVector` (`self.Cube`)) (`self.speed`))
      (`SceneComponent.K2_SetWorldRotation` _paperflipbook (`KismetMathLibrary.MakeRotator` _returnvalue_roll _returnvalue_pitch 180.0) false false)))
  (:`Started`
    (goto _label))
  (:`Completed`
    (goto _label_2)))

(event `self.ReceiveTick`
  (params (DeltaSeconds :type "Float (single-precision)"))
  (`KismetSystemLibrary.PrintString` (`KismetStringLibrary.Conv_IntToString` (`self.sonCafard?`)))
  (if (== (`SceneComponent.GetComponentVelocity` (`self.CapsuleComponent`)) (0.0 0.0 0.0))
    (`/Engine/EditorBlueprintResources/StandardMacros.DoOnce` false :!label _label_3
      (:`Completed`
        (`PaperFlipbookComponent.Stop` (`self.PaperFlipbook`))))
    (else
      (goto _label_3 :!via `Reset`))))

(fn `Death`
  (if (`self.HasCollier`)
    (set `self.HasCollier` false)
    (`|SpawnActorFromClass` "/Game/Blueprint/Items/Collectable/BP_Collier.BP_Collier_C" (`self.CollierTransfo`) "Undefined" "MultiplyWithRoot" null null))
  (set `self.CanMove` false)
  (bind _returnvalue (`|CreateWidget` "/Game/Blueprint/Widget/Dialogue/WB_MortCafard.WB_MortCafard_C"))
  (set `self.WidgetRef` _returnvalue)
  (`UserWidget.AddToViewport` _returnvalue 0)
  (set `self.IsDead` true))

(fn `Sort`
  (bind _returnvalue (`|CreateWidget` "/Game/Blueprint/Widget/Dialogue/WB_SortieCafard.WB_SortieCafard_C"))
  (set `self.WidgetRef` _returnvalue)
  (`UserWidget.AddToViewport` _returnvalue 0)
  (set `self.CanMove` false)
  (set `self.IsDead` true))

(fn `StartGame`
  (`SceneComponent.K2_SetWorldLocation` (`self.CapsuleComponent`) (`self.StartLocation`) false false)
  (set `self.CanMove` true)
  (bind _outactors (`GameplayStatics.GetAllActorsOfClass` "/Game/Blueprint/Mini_Jeux/Cafard/BP_CafardEnnemi.BP_CafardEnnemi_C"))
  (for _array_element _outactors
    (`/Game/Blueprint/Mini_Jeux/Cafard/BP_CafardEnnemi.Resetennemi` _array_element)))

(fn `UserConstructionScript`)

(fn `Win`
  (set `self.CanMove` false)
  (bind _returnvalue (`|CreateWidget` "/Game/Blueprint/Widget/Dialogue/WB_WinCafard.WB_WinCafard_C"))
  (`UserWidget.AddToViewport` _returnvalue 0))