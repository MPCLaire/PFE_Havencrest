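; PC_Cafard, likely the player controller for the Cafard (cockroach) minigame, lets the player return to the Havencrest level once the minigame is won.
; It caches the GI_Havencrest game instance on BeginPlay.
; Pressing E checks that instance's WonCafard flag, then sets GameState and opens Havencrest, or only prints a debug string if the game is not won.
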(event `self.ReceiveBeginPlay`
  (bind _asgi_havencrest (cast `/Game/Blueprint/GameSystem/GI_Havencrest` (`GameplayStatics.GetGameInstance`)))
  (set `self.As GI Havencrest` _asgi_havencrest))

(event `Key|E`
  (params (Key :type "Key Structure"))
  (:`Pressed`
    (`KismetSystemLibrary.PrintString` "oui ee")
    (if (`/Game/Blueprint/GameSystem/GI_Havencrest.wonCafard` (`self.As GI Havencrest`))
      (set `/Game/Blueprint/GameSystem/GI_Havencrest.GameState` "NewEnumerator2" (`self.As GI Havencrest`))
      (`GameplayStatics.OpenLevelBySoftObjectPtr` "/Game/Maps/Havencrest.Havencrest")
      (else
        (`KismetSystemLibrary.PrintString` "paswion")))))

(fn `UserConstructionScript`)