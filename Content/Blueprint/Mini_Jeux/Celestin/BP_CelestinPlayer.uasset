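; Player pawn for Celestin's bug-shooting minigame, possessed on StartGame with cursor input and the journal hidden.
; Each tick the gun child actor turns toward the cursor hit, while shooting plays sound, flipbook and score-scaled camera shake.
; Lose decrements lives; running out or winning stops live bugs and shows WB_LoseCelestin, retitled for wins.
; E then fades out to ExplosionCameraRef and re-enables Ethan's movement, resetting state only after defeat.
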(event `self.ReceiveBeginPlay`
  (set `self.PlayerControllerRef` (`GameplayStatics.GetPlayerController` 0))
  (bind _asbp_gun (cast `/Game/Blueprint/Mini_Jeux/Celestin/BP_Gun` (`ChildActorComponent.ChildActor` (`self.Gun`))))
  (set `self.GunRef` _asbp_gun)
  (bind _asbp_ethan (cast `/Game/Blueprint/MainCharacter/Blueprints/BP_Ethan` (`GameplayStatics.GetPlayerCharacter` 0)))
  (set `self.As BP Ethan` _asbp_ethan))

(event `self.ReceiveTick`
  (params (DeltaSeconds :type "Float (single-precision)"))
  (if (`self.isMinigameActivated`)
    (`self.FollowMouseCursor`)))

(event `/Game/Blueprint/Interfaces/BPI_Celestin.StartGame`
  (bind _returnvalue (`GameplayStatics.GetPlayerController` 0))
  (bind _cafardbruit (`self.CafardBruit`))
  (bind (_screencenter_x _screencenter_y) (`KismetMathLibrary.BreakVector2D` (`self.ScreenCenter`)))
  (if (`self.canPlay`)
    (`/Game/Assets/DecorsAsset/Batiments/BP_Batiments_Parent.ExitBuildingCelestin` (`self.CelestinRef`))
    (`KismetSystemLibrary.Delay` 1.0)
    (bind _foundwidgets (`WidgetBlueprintLibrary.GetAllWidgetsOfClass` "/Game/Blueprint/Widget/WB_Journal.WB_Journal_C"))
    (bind _output_get (set `self.JournalRef` (`|GetArrayItem` _foundwidgets)))
    (`/Game/Blueprint/Widget/WB_Journal.InvisibleWidget` _output_get)
    (`Controller.Possess` _returnvalue self)
    (bind _output_get_2 (set `PlayerController.bShowMouseCursor` true _returnvalue))
    (set `PlayerController.bEnableClickEvents` _output_get_2 _returnvalue)
    (`WidgetBlueprintLibrary.SetInputMode_GameAndUIEx` _returnvalue null "DoNotLock" false)
    (`PlayerController.SetMouseLocation` (`self.PlayerControllerRef`) (`KismetMathLibrary.FTrunc` _screencenter_x) (`KismetMathLibrary.FTrunc` _screencenter_y))
    (set `self.isMinigameActivated` true)
    (`ActorComponent.Activate` _cafardbruit false)
    (`KismetSystemLibrary.Delay` 3.0)
    (`AudioComponent.AdjustVolume` _cafardbruit 0.0 0.15 "Linear")))

(event `EnhancedInput|/Game/Blueprint/MainCharacter/Input/Actions/IA_Shoot`
  (params (ActionValue :type Boolean) (ElapsedSeconds :type "Float (double-precision)") (TriggeredSeconds :type "Float (double-precision)") (InputAction :type "InputAction Object Reference" :default "/Game/Blueprint/MainCharacter/Input/Actions/IA_Shoot.IA_Shoot"))
  (bind _scorebugs (`self.ScoreBugs`))
  (:`Triggered`
    (if (< (`self.Life`) 1)
      _
      (elif (not (`self.hasWon`))
        (`PlayerController.ClientStartCameraShake` :`self` (`GameplayStatics.GetPlayerController` 0) :`Shake` "/Game/Blueprint/Mini_Jeux/Celestin/BP_CameraShakeCelestin.BP_CameraShakeCelestin_C" :`Scale` (`self.CameraShakeScale`))
        (`GameplayStatics.SpawnSound2D` "/Game/Sounds/CelestinSounds/SC_Shot.SC_Shot" 0.7 1.0 0.0 null)
        (`self.Shot` (`/Game/Blueprint/Mini_Jeux/Celestin/BP_Gun.PaperFlipbook` (`self.GunRef`)))
        (if (== _scorebugs 10)
          (set `self.CameraShakeScale` 0.7)
          (elif (== _scorebugs 20)
            (set `self.CameraShakeScale` 1.0)
            (elif (== _scorebugs 40)
              (set `self.CameraShakeScale` 1.2))))))))

(event `Key|E`
  (params (Key :type "Key Structure"))
  (:`Pressed`
    (if (< (`self.Life`) 1)
      (`|ExecutionSequence`
        (:`then_0`
          (`Widget.RemoveFromParent` (`self.WidgetLoseRef`) :!label _label)
          (`self.Fade`)
          (bind _returnvalue (`|CreateWidget` "/Game/Image/UI/WB_Curseur.WB_Curseur_C"))
          (`PlayerController.SetMouseCursorWidget` (`GameplayStatics.GetPlayerController` 0) "Default" _returnvalue)
          (set `self.hasWon` false)
          (set `self.canPlay` false))
        (:`then_1`
          (`self.ResetEverything`)))
      (elif (`self.hasWon`)
        (goto _label)))))

(fn `FollowMouseCursor`
  (bind _gun (`self.Gun`))
  (bind (_returnvalue_roll _returnvalue_pitch _returnvalue_yaw) (`KismetMathLibrary.BreakRotator` (`KismetMathLibrary.FindLookAtRotation` (`SceneComponent.K2_GetComponentLocation` _gun) (`.Location` (`GameplayStatics.BreakHitResult` (`PlayerController.GetHitResultUnderCursorByChannel` (`self.PlayerControllerRef`) "TraceTypeQuery1" true))))))
  (`SceneComponent.K2_SetWorldRotation` _gun (`KismetMathLibrary.MakeRotator` 0.0 _returnvalue_pitch _returnvalue_yaw) false false))

(fn `Lose`
  (bind _result (`/Engine/EditorBlueprintResources/StandardMacros.DecrementInt` (`self.Life`))
    (:`  `
      (if (< _result 1)
        (set `self.isMinigameActivated` false)
        (bind _returnvalue (`|CreateWidget` "/Game/Blueprint/Widget/Dialogue/WB_LoseCelestin.WB_LoseCelestin_C"))
        (bind _output_get (set `self.WidgetLoseRef` _returnvalue))
        (`UserWidget.AddToViewport` _output_get 0)
        (for _array_element (`self.BP_AliveBugs`)
          (`/Game/Blueprint/Mini_Jeux/Celestin/BP_CelestinBugs.StopThem` _array_element)
          (`KismetSystemLibrary.PrintString` "Perdu")
          (set `self.hasLost` true)
          (`ActorComponent.Deactivate` (`self.CafardBruit`))
          (`GameplayStatics.PlaySound2D` "/Game/Sounds/MiniGame/FailSoundEffect.FailSoundEffect" 0.2 1.0 0.0 null null))
        (else
          (`KismetSystemLibrary.PrintString` (`KismetTextLibrary.Conv_TextToString` (`|FormatText` "Tu as perdu une vie. Il t'en reste {vie}." _result))))))))

(fn `ResetEverything`
  (set `self.ScoreBugs` 0)
  (set `self.Life` 3)
  (set `self.hasLost` false)
  (for _array_element (`self.BP_AliveBugs`)
    (`self.K2_DestroyActor` _array_element))
  (`KismetArrayLibrary.Array_Clear` (`self.BP_AliveBugs`)))

(fn `UserConstructionScript`)

(fn `WinCelestin`
  (set `self.isMinigameActivated` false)
  (bind _returnvalue (`|CreateWidget` "/Game/Blueprint/Widget/Dialogue/WB_LoseCelestin.WB_LoseCelestin_C"))
  (bind _output_get (set `self.WidgetLoseRef` _returnvalue))
  (`TextBlock.SetText` (`/Game/Blueprint/Widget/Dialogue/WB_LoseCelestin.TalkText` _output_get) "Oh oh !")
  (`UserWidget.AddToViewport` _output_get 0)
  (for _array_element (`self.BP_AliveBugs`)
    (`/Game/Blueprint/Mini_Jeux/Celestin/BP_CelestinBugs.StopThem` _array_element)
    (set `self.hasWon` true)
    (`ActorComponent.Deactivate` (`self.CafardBruit`))
    (`GameplayStatics.PlaySound2D` "/Game/Sounds/MiniGame/SuccessSoundEffect.SuccessSoundEffect" 0.1 1.0 0.0 null null)))