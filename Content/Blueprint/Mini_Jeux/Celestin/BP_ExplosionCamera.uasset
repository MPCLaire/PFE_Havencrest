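; Camera pawn that plays the explosion cutscene of Celestin's mini-game in Havencrest.
; On possession it moves Ethan to Celestin's inside point and runs a delay-timed sequence: camera shake, sound, flipbook, Niagara burst and a timeline-driven launch of Ethan.
; It then possesses Ethan, advances the journal objective, swaps or reveals destruction props and saves the state in the GameInstance.
; BeginPlay reapplies the destroyed props when that GameState is post-explosion.
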(event `LaunchEthan`
  (bind (_ethaninitlocation_x _ethaninitlocation_y _ethaninitlocation_z) (`KismetMathLibrary.BreakVector` (`self.EthanInitLocation`)))
  (set `self.EthanInitLocation` (`self.K2_GetActorLocation` (`self.EthanRef`)))
  (bind (_direction _newtrack_0 _newtrack_1) (`Timeline|LaunchTL` :!via `PlayFromStart`)
    (:`Update`
      (`self.K2_SetActorLocation` (`self.EthanRef`) (`KismetMathLibrary.MakeVector` _ethaninitlocation_x (+ (`KismetMathLibrary.Lerp` 0.0 2000.0 _newtrack_1) _ethaninitlocation_y) (+ (`KismetMathLibrary.Lerp` 0.0 800.0 _newtrack_0) _ethaninitlocation_z)) false false))))

(event `self.ReceiveBeginPlay`
  (bind _asgi_havencrest (cast `/Game/Blueprint/GameSystem/GI_Havencrest` (`GameplayStatics.GetGameInstance`)))
  (bind _output_get (set `self.As GI Havencrest` _asgi_havencrest))
  (switch `/Game/Blueprint/GameSystem/E_Instance` (`/Game/Blueprint/GameSystem/GI_Havencrest.GameState` _output_get)
    (:`NewEnumerator5`
      _)
    (:`NewEnumerator6`
      _)
    (:`NewEnumerator2`
      _))
  (`self.PropsDestruction`))

(event `self.ReceivePossessed`
  (params (NewController :type "Controller Object Reference"))
  (bind (_returnvalue_x _returnvalue_y _returnvalue_z) (`KismetMathLibrary.BreakVector` (`SceneComponent.K2_GetComponentLocation` (`/Game/Assets/DecorsAsset/Batiments/BP_Batiments_Parent.InsidePoint` (`self.CelestinRef`)))))
  (bind _foundwidgets (`WidgetBlueprintLibrary.GetAllWidgetsOfClass` "/Game/Blueprint/Widget/WB_Journal.WB_Journal_C"))
  (set `self.JournalRef` (`|GetArrayItem` _foundwidgets))
  (`self.Explosion`)
  (`self.K2_SetActorLocation` (`self.EthanRef`) (`KismetMathLibrary.MakeVector` _returnvalue_x _returnvalue_y (+ _returnvalue_z 100.0)) false false))

(event `Explosion`
  (bind _niagara (`self.Niagara`))
  (bind _journalref (`self.JournalRef`))
  (bind _paperflipbook (`self.PaperFlipbook`))
  (`PlayerController.ClientStartCameraShake` :`self` (`GameplayStatics.GetPlayerController` 0) :`Shake` "/Game/Blueprint/Mini_Jeux/Celestin/BP_CameraShakeExplosion.BP_CameraShakeExplosion_C")
  (`KismetSystemLibrary.Delay` 7.0)
  (`GameplayStatics.PlaySound2D` "/Game/Sounds/MicrowaveSounds/ExplosionMicrowave.ExplosionMicrowave" 1.0 1.0 0.0 null null)
  (`KismetSystemLibrary.Delay` 0.5)
  (`PaperFlipbookComponent.SetFlipbook` _paperflipbook "/Game/FX/Explosion/FB_Explosion.FB_Explosion")
  (`PaperFlipbookComponent.SetLooping` _paperflipbook false)
  (`self.LaunchEthan`)
  (`NiagaraComponent.ResetSystem` _niagara)
  (`SceneComponent.SetVisibility` _niagara true false)
  (`KismetSystemLibrary.Delay` 1.0)
  (`PaperFlipbookComponent.SetFlipbook` (`self.PaperFlipbook`) null)
  (`KismetSystemLibrary.Delay` 0.5)
  (`Controller.Possess` (`GameplayStatics.GetPlayerController` 0) (`self.EthanRef`))
  (`/Game/Blueprint/Widget/WB_Journal.SetVisibilityBack` _journalref)
  (`/Game/Blueprint/Widget/WB_Journal.NextObjectif` _journalref 12)
  (`self.PropsDestruction`)
  (set `/Game/Blueprint/GameSystem/GI_Havencrest.GameState` "NewEnumerator5" (`self.As GI Havencrest`)))

(event `PropsDestruction`
  (`/Game/Assets/DecorsAsset/Batiments/Celestin/BP_MaisonCelestin.ChangeFacade` (`self.CelestinRef`))
  (`/Game/Assets/DecorsAsset/DecorsVille/BP_BarrierreMine.ChangeGrille` (`self.GrilleRef`))
  (`self.K2_DestroyActor` (`self.BoxGrillage`))
  (for _array_element (`self.BoisDehors`)
    (bind _planche (`/Game/Assets/DecorsAsset/Batiments/Celestin/BP_Planches.Planche` _array_element))
    (`SceneComponent.SetVisibility` _planche true false)
    (`SceneComponent.SetVisibility` (`/Game/Assets/DecorsAsset/Batiments/Celestin/BP_Planches.Planche1` _array_element) true false)
    (`SceneComponent.SetVisibility` (`/Game/Assets/DecorsAsset/Batiments/Celestin/BP_Planches.Planche2` _array_element) true false)
    (`PrimitiveComponent.SetCollisionEnabled` _planche "QueryAndPhysics")
    (`PrimitiveComponent.SetCollisionEnabled` (`/Game/Assets/DecorsAsset/Batiments/Celestin/BP_Planches.Planche1` _array_element) "QueryAndPhysics")
    (`PrimitiveComponent.SetCollisionEnabled` (`/Game/Assets/DecorsAsset/Batiments/Celestin/BP_Planches.Planche2` _array_element) "QueryAndPhysics"))
  (for _array_element_2 (`self.Rocher`)
    (`SceneComponent.SetVisibility` (`StaticMeshActor.StaticMeshComponent` _array_element_2) true false)))

(fn `UserConstructionScript`)