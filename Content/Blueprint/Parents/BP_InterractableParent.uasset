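; Parent Blueprint for interactable objects that respond to an item given from the player's inventory.
; GiveItem stores the item name, checks it against the accepted list, then fires Possess or the empty Don'tPosess event as a hook for children.
; Either way it messages the player character to remove the inventory, and an accepted item flagged Givable is also removed from it.
; Possess only prints a debug string here.
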(event `/Game/Blueprint/Interfaces/BPI_Interraction.GiveItem`
  (params (ItemName :type "/Game/Blueprint/Inventory/ST_inventory Structure") (Index :type Integer) (ItemName2 :type "/Game/Blueprint/Inventory/ST_inventory2 Structure"))
  (bind (_image _name _quantity _maxstack _namefusion _imagefusion _quantityfusion _maxstaxkfusion _itemclass _fusionitemclass _givable) (break `/Game/Blueprint/Inventory/ST_inventory2` ItemName2))
  (bind _returnvalue (`GameplayStatics.GetPlayerCharacter` 0))
  (`KismetSystemLibrary.PrintString` "GIVE ITem7")
  (set `self.Item` _name)
  (if (`KismetArrayLibrary.Array_Contains` (`self.ItemWhichInteract`) _name)
    (`self.Possess`)
    (message `/Game/Blueprint/Interfaces/BPI_Player.RemoveInventory` _returnvalue)
    (if _givable
      (message `/Game/Blueprint/Interfaces/BPI_Player.RemoveItemInInventory` _returnvalue false Index ItemName2))
    (else
      (`self.Don'tPosess`)
      (message `/Game/Blueprint/Interfaces/BPI_Player.RemoveInventory` _returnvalue))))

(event `Possess`
  (`KismetSystemLibrary.PrintString` "Interract"))

(event `Don'tPosess`)

(fn `UserConstructionScript`)