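; Parent Blueprint for collectable items that signals the player when one can be picked up.
; A Box overlap by the player character sends CanPickUpMessage with the item's Inventory data and a self reference, and leaving sends CantPickUpMessage.
; SetStructure lets that Inventory data be assigned from outside.
; An unreachable, obsolete chain that added directly to Comp_Inventory and refreshed WB_inventory is kept for reference.
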(event `self.Box.OnComponentBeginOverlap`
  (params (OverlappedComponent :type "PrimitiveComponent Object Reference") (OtherActor :type "Actor Object Reference") (OtherComp :type "PrimitiveComponent Object Reference") (OtherBodyIndex :type Integer) (bFromSweep :type Boolean) (SweepResult :type "HitResult Structure (by ref)"))
  (if (== OtherActor (`GameplayStatics.GetPlayerCharacter` 0))
    (message `/Game/Blueprint/Interfaces/BPI_Items.CanPickUp` OtherActor (`self.Inventory`) self)))

(event `/Game/Blueprint/Interfaces/BPI_Items.SetStructure`
  (params (Inventory :type "/Game/Blueprint/Inventory/ST_inventory Structure"))
  (set `self.Inventory` Inventory))

(event `self.Box.OnComponentEndOverlap`
  (params (OverlappedComponent :type "PrimitiveComponent Object Reference") (OtherActor :type "Actor Object Reference") (OtherComp :type "PrimitiveComponent Object Reference") (OtherBodyIndex :type Integer))
  (if (== OtherActor (`GameplayStatics.GetPlayerCharacter` 0))
    (message `/Game/Blueprint/Interfaces/BPI_Items.Can'tPickUp` OtherActor)))

(fn `UserConstructionScript`)