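; BP_CollectableParent is a base collectable pickup that adds its item to the player's inventory when BP_Ethan overlaps its box.
; The overlap passes its Inventory variable to the Comp_Inventory component on BP_Ethan.
; On success it finds the top-level WB_inventory widget, rebuilds it through SetGrid and destroys itself.
; On failure the actor stays in the world and prints a debug message that the inventory is full.
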(event `self.Box.OnComponentBeginOverlap`
  (params (OverlappedComponent :type "PrimitiveComponent Object Reference") (OtherActor :type "Actor Object Reference") (OtherComp :type "PrimitiveComponent Object Reference") (OtherBodyIndex :type Integer) (bFromSweep :type Boolean) (SweepResult :type "HitResult Structure (by ref)"))
  (bind _asbp_ethan (cast `/Game/Blueprint/MainCharacter/Blueprints/BP_Ethan` OtherActor))
  (bind _itemadded (`/Game/Blueprint/NewInventaire/Comp_Inventory.AddToInventory` (`self.GetComponentByClass` _asbp_ethan "/Game/Blueprint/NewInventaire/Comp_Inventory.Comp_Inventory_C") (`self.Inventory`)))
  (if _itemadded
    (bind _foundwidgets (`WidgetBlueprintLibrary.GetAllWidgetsOfClass` "/Game/Blueprint/NewInventaire/WB_inventory.WB_inventory_C"))
    (bind _output (`|GetArrayItem` _foundwidgets))
    (`/Engine/EditorBlueprintResources/StandardMacros.IsValid` _output
      (:`Is Valid`
        (`/Game/Blueprint/NewInventaire/WB_inventory.SetGrid` _output))
      (:`Is Not Valid`
        _))
    (`self.K2_DestroyActor`)
    (`KismetSystemLibrary.PrintString` "ItemCollected")
    (else
      (`KismetSystemLibrary.PrintString` "inventoryFull"))))

(fn `UserConstructionScript`)