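; Inventory component that holds a fixed array of item slots and toggles the WB_inventory screen with Tab.
; BeginPlay fills the slots, and Tab adds or removes the widget while switching input mode and cursor visibility.
; AddToInventory increments a matching non-full stack or takes the first zero-quantity slot, treating the last index as full.
; Successful additions refresh any open inventory widget through SetGrid and return true.
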(event `self.ReceiveBeginPlay`
  (for _ (range 16)
    (`KismetArrayLibrary.Array_Add` (`self.Inventory`))))

(event `Key|Tab`
  (params (Key :type "Key Structure"))
  (bind _returnvalue (`GameplayStatics.GetPlayerController` 0))
  (bind _returnvalue_2 (`GameplayStatics.GetPlayerController` 0))
  (:`Pressed`
    (bind _foundwidgets (`WidgetBlueprintLibrary.GetAllWidgetsOfClass` "/Game/Blueprint/NewInventaire/WB_inventory.WB_inventory_C"))
    (bind _output (`|GetArrayItem` _foundwidgets))
    (`/Engine/EditorBlueprintResources/StandardMacros.IsValid` _output
      (:`Is Valid`
        (`Widget.RemoveFromParent` _output)
        (`WidgetBlueprintLibrary.SetInputMode_GameOnly` _returnvalue_2)
        (set `PlayerController.bShowMouseCursor` false _returnvalue_2))
      (:`Is Not Valid`
        (bind _returnvalue_3 (`|CreateWidget` "/Game/Blueprint/NewInventaire/WB_inventory.WB_inventory_C"))
        (`UserWidget.AddToViewport` _returnvalue_3 0)
        (`WidgetBlueprintLibrary.SetInputMode_GameAndUIEx` _returnvalue null)
        (set `PlayerController.bShowMouseCursor` true _returnvalue)))))

(fn `AddToInventory`
  (params (Inventory :type "/Game/Blueprint/NewInventaire/ST_inventory Structure"))
  (returns (ItemAdded :type Boolean))
  (locals (InventoryRef :type "/Game/Blueprint/NewInventaire/ST_inventory Structure") (IndexRef :type Integer) (Found :type Boolean))
  (bind (_inventoryref_image _inventoryref_name) (break `/Game/Blueprint/NewInventaire/ST_inventory` (`local.InventoryRef`)))
  (bind _inventory (`self.Inventory`))
  (bind _indexref (`local.IndexRef`))
  (bind (_output_image _output_name _output_quantity _output_maxstack) (break `/Game/Blueprint/NewInventaire/ST_inventory` (`|GetArrayItem` _inventory _indexref)))
  (set `local.InventoryRef` Inventory)
  (for (_array_element _array_index) (`self.Inventory`)
    (set `local.IndexRef` _array_index)
    (if (and (`KismetTextLibrary.EqualEqual_TextText` (`.Name_7_C190B5B346B71737A982D69200F6DB2D` (break `/Game/Blueprint/NewInventaire/ST_inventory` _array_element)) _inventoryref_name) (< (`.Quantity_10_AF96E3D6429E4CC20D8A7389A135EBDE` (break `/Game/Blueprint/NewInventaire/ST_inventory` _array_element)) (`.MaxStack_12_4FD250F94E7B40059065E0BF4F091A52` (break `/Game/Blueprint/NewInventaire/ST_inventory` _array_element))))
      (set `local.Found` true)
      (break)))
  (if (`local.Found`)
    (`KismetArrayLibrary.Array_Set` _inventory _indexref (make `/Game/Blueprint/NewInventaire/ST_inventory` _output_image _output_name (+ _output_quantity 1) _output_maxstack "" null))
    (bind _foundwidgets (`WidgetBlueprintLibrary.GetAllWidgetsOfClass` "/Game/Blueprint/NewInventaire/WB_inventory.WB_inventory_C"))
    (bind _output (`|GetArrayItem` _foundwidgets))
    (`/Engine/EditorBlueprintResources/StandardMacros.IsValid` _output
      (:`Is Valid`
        (`/Game/Blueprint/NewInventaire/WB_inventory.SetGrid` _output))
      (:`Is Not Valid`
        _))
    (`KismetSystemLibrary.PrintString` (`KismetStringLibrary.Conv_IntToString` (`local.IndexRef`)))
    (return true)
    (else
      (for (_array_element_2 _array_index_2) (`self.Inventory`)
        (set `local.IndexRef` _array_index_2)
        (if (== (`.Quantity_10_AF96E3D6429E4CC20D8A7389A135EBDE` (break `/Game/Blueprint/NewInventaire/ST_inventory` _array_element_2)) 0)
          (set `local.Found` true)
          (break)))
      (if (`local.Found`)
        (if (>= (`local.IndexRef`) 15)
          (`KismetSystemLibrary.PrintString` "InventairePlein")
          (else
            (`KismetArrayLibrary.Array_Set` (`self.Inventory`) (`local.IndexRef`) (`local.InventoryRef`))
            (bind _foundwidgets_2 (`WidgetBlueprintLibrary.GetAllWidgetsOfClass` "/Game/Blueprint/NewInventaire/WB_inventory.WB_inventory_C"))
            (bind _output_2 (`|GetArrayItem` _foundwidgets_2))
            (`/Engine/EditorBlueprintResources/StandardMacros.IsValid` _output_2
              (:`Is Valid`
                (`/Game/Blueprint/NewInventaire/WB_inventory.SetGrid` _output_2))
              (:`Is Not Valid`
                _))
            (`KismetSystemLibrary.PrintString` (`KismetStringLibrary.Conv_IntToString` (`local.IndexRef`)))
            (return true)))
        (else
          (return false))))))