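; BP_FadePlane is a self-destroying plane actor that plays a material-driven fade when play begins.
; It applies M_FadeIn to the plane, then a timeline drives the material's InnerRadius scalar parameter on each update.
; When the timeline finishes, the plane switches to M_Transparent and the actor destroys itself.
; A DoOnce-gated delay fires when the track value is zero, but nothing follows it.
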(event `self.ReceiveBeginPlay`
  (bind _plane (`self.Plane`))
  (`PrimitiveComponent.SetMaterial` _plane 0 "/Game/Materials/Materials/M_FadeIn.M_FadeIn")
  (bind (_direction _newtrack_0) (`Timeline|Timeline` :!via `PlayFromStart`)
    (:`Update`
      (`MeshComponent.SetScalarParameterValueOnMaterials` (`self.Plane`) "InnerRadius" _newtrack_0)
      (`|ExecutionSequence`
        (:`then_0`
          (`/Engine/EditorBlueprintResources/StandardMacros.DoOnce` false))
        (:`then_1`
          (if (== _newtrack_0 0.0)
            (`/Engine/EditorBlueprintResources/StandardMacros.DoOnce` false :!label _label
              (:`Completed`
                (`KismetSystemLibrary.Delay` 0.7)))))))
    (:`Finished`
      (`PrimitiveComponent.SetMaterial` _plane 0 "/Game/Materials/Materials/M_Transparent.M_Transparent")
      (`self.K2_DestroyActor`)
      (goto _label :!via `Reset`))))

(fn `UserConstructionScript`)